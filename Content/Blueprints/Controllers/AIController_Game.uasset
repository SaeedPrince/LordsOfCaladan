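; Server-side AI controller for a person (civilian or soldier), tracking its job, carried items and residence, work or garrison building.
; Construction picks and runs a behavior tree and blackboard by person type from SpawnData.
; Assigned jobs drive walk, run or attack on the character; arrival completes once both move and turn finish, updating presence, buildings and UI.
; Soldier conversion swaps residence for garrison and sets the military tree variable without rerunning it.
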(event `ServerPersonPositionChanged`
  (bind _player (`/Game/Assets/BP_Meshes/Architecture/BP_House.Player` (`/Game/Blueprints/Libraries/LibAIController.ResidenceByType` self)))
  ;[0 1 0] Updates bottom widget
  (if (`/Game/Blueprints/Controllers/PlayerController_Game.BottomWidget` _player)
    (`/Game/Blueprints/Controllers/PlayerController_Game.ShowBottomData` _player)))

(event `ServerPickupItem`
  (params (Item :type "/Game/Assets/BP_Meshes/Item/BP_Item Object Reference") (Building :type "/Game/Assets/BP_Meshes/Architecture/BP_House Object Reference"))
  ;[1 1 0] Career item pickup or drop
  (`KismetArrayLibrary.Array_Add` (`self.Inventory`) Item)
  (`self.K2_AttachToActor` Item (`self.CharacterRef`) "hand_rSocket" "SnapToTarget" "SnapToTarget" "SnapToTarget" false)
  (`/Game/Assets/BP_Meshes/Architecture/BP_House.ServerItemSent` Building Item))

(event `ServerDropItem`
  (params (Item :type "/Game/Assets/BP_Meshes/Item/BP_Item Object Reference") (Building :type "/Game/Assets/BP_Meshes/Architecture/BP_House Object Reference"))
  ;[1 1 0] Career item pickup or drop
  (`self.MacRemoveItem` Item)
  (`/Game/Assets/BP_Meshes/Architecture/BP_House.ServerItemReceived` Building Item))

(event `ServerWasteItem`
  (params (Item :type "/Game/Assets/BP_Meshes/Item/BP_Item Object Reference"))
  ;[1 1 0] Career item pickup or drop
  (`|ExecutionSequence`
    (:`then_0`
      (`self.MacRemoveItem` Item))
    (:`then_1`
      (`self.K2_DestroyActor` Item))))

(event `ServerAssignJob`
  (params (Job :type "/Game/Blueprints/Structures/Game/StructJob Structure"))
  ;[1 1 0] Assign job or carry to person
  (set `self.ProviousJob` (`self.CurrentJob`))
  (set `self.CurrentJob` Job)
  (`self.MacProcessJob`))

(event `ServerAssignCarry`
  (params (Carry :type "/Game/Blueprints/Structures/Game/StructCarry Structure"))
  ;[1 1 0] Assign job or carry to person
  (set `self.Carry` Carry))

(event `ServerAssignCivilResidenceAndPlacement`
  (params (Residence :type "/Game/Assets/BP_Meshes/Architecture/BP_House Object Reference") (Placement :type "Vector Structure") (ResidenceIndex :type Integer))
  ;[1 1 0] Assign residence and placement
  (set `self.BuildingResidence` Residence)
  (set `self.ResidentPlacement` Placement)
  (set `self.IndexInResidence` ResidenceIndex))

(event `ServerTurnToSoldier`
  (params (Garrison :type "/Game/Assets/BP_Meshes/Architecture/BP_House Object Reference"))
  (bind _indexingarrison (`self.IndexInGarrison`))
  (bind ((`SoldierType_34_5278AB3A4FD1EAD828BDAFB3CA3D87C5` _soldiertype) (`IndexInGarrison_30_8CA9B9BD460FE569641DD78051C27F78` _indexingarrison_2)) (break `/Game/Blueprints/Structures/Game/StructJob` (`self.CurrentJob`)))
  ;[1 1 0] Change civil to soldier
  (set `self.SoldierType` _soldiertype)
  (set `self.IndexInGarrison` _indexingarrison_2)
  (`/Game/Assets/BP_Meshes/Architecture/BP_House.ServerReleaseCivilResident` (`self.BuildingResidence`) self)
  (set `self.BuildingGarrison` Garrison)
  (set `self.SoldierPlacement` (`SceneComponent.K2_GetComponentLocation` (`|GetArrayItem` (`/Game/Assets/BP_Meshes/Architecture/BP_House.MilitPlacements` (`self.BuildingGarrison`)) _indexingarrison)))
  (`/Game/Assets/BP_Meshes/Architecture/BP_House.ServerAddGarrisonPerson` Garrison self _indexingarrison)
  (set `self.CurrentBehaviorTree` "/Game/Blueprints/AI/BehaviorTree/BT_Miltary.BT_Miltary")
  (`BlackboardComponent.SetValueAsVector` (`AIBlueprintHelperLibrary.GetBlackboard` self) (`self.HomeLocation`) (`self.SoldierPlacement`))
  (`KismetSystemLibrary.PrintString` "Soldier created successfully." true true (struct :`G` 1.0 :`A` 1.0) 10.0)
  (`/Game/Blueprints/Characters/HumanBP.MulticastSoldierApperance` (`self.CharacterRef`) (`self.SoldierType`)))

(event `ServerReleasePersonFromBuildingResidence`
  (params (Building :type "/Game/Assets/BP_Meshes/Architecture/BP_House Object Reference"))
  ;[1 1 0] Release person from residence
  (`/Game/Assets/BP_Meshes/Architecture/BP_House.ServerReleaseCivilResidence` Building (`self.IndexInResidence`))
  (set `self.IndexInResidence` -1)
  (set `self.ResidentPlacement` (0.0 0.0 0.0)))

(event `ServerReleasePersonFromBuildingGarrison`
  (params (Building :type "/Game/Assets/BP_Meshes/Architecture/BP_House Object Reference"))
  ;[1 1 0] Release person from residence
  (`/Game/Assets/BP_Meshes/Architecture/BP_House.ServerReleaseMilitaryGarrison` Building (`self.IndexInGarrison`))
  (set `self.IndexInGarrison` -1)
  (set `self.SoldierPlacement` (0.0 0.0 0.0)))

(event `ServerAddPersonToBuildingAsResident`
  (params (Building :type "/Game/Assets/BP_Meshes/Architecture/BP_House Object Reference") (IndexInResidence :type Integer))
  ;[1 1 0] Add person to building as resident / worker / soldier
  (set `self.BuildingResidence` Building)
  (set `self.ResidentPlacement` (`SceneComponent.K2_GetComponentLocation` (`|GetArrayItem` (`/Game/Assets/BP_Meshes/Architecture/BP_House.CivilPlacements` Building) IndexInResidence)))
  (set `self.IndexInResidence` IndexInResidence)
  (`/Game/Assets/BP_Meshes/Architecture/BP_House.ServerAddResidentPerson` Building self IndexInResidence))

(event `ServerAddPersonToBuildingAsWorker`
  (params (Building :type "/Game/Assets/BP_Meshes/Architecture/BP_House Object Reference") (IndexInWork :type Integer))
  ;[1 1 0] Add person to building as resident / worker / soldier
  (set `self.BuildingWork` Building)
  (set `self.WorkPlacement` (`SceneComponent.K2_GetComponentLocation` (`|GetArrayItem` (`/Game/Assets/BP_Meshes/Architecture/BP_House.CivilPlacements` Building) IndexInWork)))
  (set `self.IndexInWorker` IndexInWork)
  (`/Game/Assets/BP_Meshes/Architecture/BP_House.ServerAddResidentPerson` Building self IndexInWork))

(event `ServerAddPersonToBuildingAsSoldier`
  (params (Building :type "/Game/Assets/BP_Meshes/Architecture/BP_House Object Reference") (IndexInGarrison :type Integer))
  ;[1 1 0] Add person to building as resident / worker / soldier
  (set `self.BuildingGarrison` Building)
  (set `self.SoldierPlacement` (`SceneComponent.K2_GetComponentLocation` (`|GetArrayItem` (`/Game/Assets/BP_Meshes/Architecture/BP_House.MilitPlacements` Building) IndexInGarrison)))
  (set `self.IndexInGarrison` IndexInGarrison)
  (`/Game/Assets/BP_Meshes/Architecture/BP_House.ServerAddGarrisonPerson` Building self IndexInGarrison))

(event `ServerReleasePersonFromBuildingWorker`
  (params (Building :type "/Game/Assets/BP_Meshes/Architecture/BP_House Object Reference"))
  ;[1 1 0] Release person from work
  (`/Game/Assets/BP_Meshes/Architecture/BP_House.ServerReleaseCivilWork` Building (`self.IndexInWorker`))
  (set `self.IndexInWorker` -1)
  (set `self.WorkPlacement` (0.0 0.0 0.0)))

(event `ServerMoveDone`
  ;[1 1 0] Process move done and turn done
  (set `self.MoveDone` true)
  (if (`self.TurnDone`)
    (`self.MacProcessEndJob` :!label _label)))

(event `ServerTurnDone`
  ;[1 1 0] Process move done and turn done
  (set `self.TurnDone` true)
  (if (`self.MoveDone`)
    (goto _label)))

(event `ServerPersonIsAtWork`
  (bind _buildingwork (`self.BuildingWork`))
  ;[1 1 0] Building start to work or garrison or stop
  (set `self.IsAtWork` true)
  (`/Engine/EditorBlueprintResources/StandardMacros.IsValid` _buildingwork
    (:`Is Valid`
      (`/Game/Assets/BP_Meshes/Architecture/BP_House.ServerPersonArrivedBuilding` _buildingwork (`self.PersonType`) (`self.IndexInWorker`)))))

(event `ServerPersonLeftWork`
  (bind _buildingwork (`self.BuildingWork`))
  ;[1 1 0] Building start to work or garrison or stop
  (set `self.IsAtWork` false)
  (`/Engine/EditorBlueprintResources/StandardMacros.IsValid` _buildingwork
    (:`Is Valid`
      (`/Game/Assets/BP_Meshes/Architecture/BP_House.ServerPersonLeftBuilding` _buildingwork (`self.PersonType`) (`self.IndexInWorker`)))))

(event `ServerPersonLeftHome`
  ;[1 1 0] Building start to work or garrison or stop
  (set `self.IsAtHome` false))

(event `ServerPersonIsAtHome`
  ;[1 1 0] Building start to work or garrison or stop
  (set `self.IsAtHome` true))

(event `ServerPersonIsAtGarrison`
  (bind _buildinggarrison (`self.BuildingGarrison`))
  ;[1 1 0] Building start to work or garrison or stop
  (set `self.IsAtGarrison` true)
  (`/Engine/EditorBlueprintResources/StandardMacros.IsValid` _buildinggarrison
    (:`Is Valid`
      (`/Game/Assets/BP_Meshes/Architecture/BP_House.ServerPersonArrivedBuilding` _buildinggarrison (`self.PersonType`) (`self.IndexInGarrison`)))))

(event `ServerPersonLeftGarrison`
  (bind _buildinggarrison (`self.BuildingGarrison`))
  ;[1 1 0] Building start to work or garrison or stop
  (set `self.IsAtGarrison` false)
  (`/Engine/EditorBlueprintResources/StandardMacros.IsValid` _buildinggarrison
    (:`Is Valid`
      (`/Game/Assets/BP_Meshes/Architecture/BP_House.ServerPersonLeftBuilding` _buildinggarrison (`self.PersonType`) (`self.IndexInGarrison`)))))

(fn `UserConstructionScript`
  (bind (_persontype _soldiertype _playerindex) (break `/Game/Blueprints/Structures/Object/StructAIController` (`self.SpawnData`)))
  (bind _returnvalue (`AIBlueprintHelperLibrary.GetBlackboard` self))
  (bind (_behaviortree _blackboard) (`/Game/Blueprints/Libraries/LibAIController.GetBehaviorTreeByPersonType` _persontype))
  (set `self.PersonType` _persontype)
  (set `self.CurrentBehaviorTree` _behaviortree)
  (set `self.CurrentBlackBoard` _blackboard)
  (set `self.SoldierType` _soldiertype)
  (set `self.PlayerIndex` _playerindex)
  (`self.UseBlackboard` (`self.CurrentBlackBoard`))
  (`self.RunBehaviorTree` (`self.CurrentBehaviorTree`))
  (`BlackboardComponent.SetValueAsVector` _returnvalue (`self.HomeLocation`) (`/Game/Blueprints/Libraries/LibAIController.LocationByType` self))
  (`BlackboardComponent.SetValueAsObject` _returnvalue "SelfActor" (`self.K2_GetPawn`)))