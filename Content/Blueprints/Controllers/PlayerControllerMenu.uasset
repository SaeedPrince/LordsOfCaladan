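; Player controller for the main menu, linking the menu widget to multiplayer session management.
; On BeginPlay it caches GameInstanceMain and adds a Widget_MenuMain to the viewport, through separate but equivalent authority and remote branches.
; Server-prefixed events forward create, find, join and destroy session requests to the game instance, passing itself along.
; ClientShowSearchResult hands search results back to the menu widget.
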(event `self.ReceiveBeginPlay`
  ;[1 1 0] Begin play
  (bind _asgame_instance_main (cast `/Game/Blueprints/Instances/GameInstanceMain` (`GameplayStatics.GetGameInstance`))
    (:`then`
      (set `self.GameInstanceRef` _asgame_instance_main)
      (`/Engine/EditorBlueprintResources/ActorMacros.Switch Has Authority`
        (:`Authority`
          (`self.CreateMenu`))
        (:`Remote`
          (bind _returnvalue (`|CreateWidget` "/Game/Blueprints/Widgets/Widget_MenuMain.Widget_MenuMain_C" self))
          (bind _output_get (set `self.WidgetMenuMain` _returnvalue))
          (`UserWidget.AddToViewport` _output_get 0))))
    (:`CastFailed`
      (`KismetSystemLibrary.PrintString` "Cast to game instance failed" true true (struct :`R` 1.0 :`A` 1.0) 10.0))))

(event `CreateMenu`
  ;[1 1 0] Begin play
  (bind _returnvalue (`|CreateWidget` "/Game/Blueprints/Widgets/Widget_MenuMain.Widget_MenuMain_C" self))
  (bind _output_get (set `self.WidgetMenuMain` _returnvalue))
  (`UserWidget.AddToViewport` _output_get 0))

(event `ServerCreateHost`
  (params (UseLan :type Boolean))
  ;[1 1 0] Server commands on game instance
  (`/Game/Blueprints/Instances/GameInstanceMain.CreateGame` (`self.GameInstanceRef`) self UseLan))

(event `ServerSearchForGame`
  (params (UseLan :type Boolean))
  ;[1 1 0] Server commands on game instance
  (`/Game/Blueprints/Instances/GameInstanceMain.FindGame` (`self.GameInstanceRef`) self UseLan))

(event `ServerJoinGame`
  (params (Session :type "BlueprintSessionResult Structure"))
  ;[1 1 0] Server commands on game instance
  (`/Game/Blueprints/Instances/GameInstanceMain.JoinGame` (`self.GameInstanceRef`) self Session))

(event `ServerDestroySession`
  ;[1 1 0] Server commands on game instance
  (`/Game/Blueprints/Instances/GameInstanceMain.DestroyGame` (`self.GameInstanceRef`) self))

(event `ClientShowSearchResult`
  (params (Result :type "Array of BlueprintSessionResult Structure"))
  ;[1 1 0] Show search result
  (`/Game/Blueprints/Widgets/Widget_MenuMain.ShowSearchResult` (`self.WidgetMenuMain`) Result))

(fn `UserConstructionScript`)