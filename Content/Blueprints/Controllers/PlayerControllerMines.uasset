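; Player controller for a Mines game that handles a player's request to join.
; The ServerRequestJoinNewPlayer event casts the game mode to GameModeBaseMines, gets a spawn place by order and a random color, and stores them with the game mode reference.
; It then asks the game mode to create the new player from this controller, color and place.
; BeginPlay, Tick and construction only call their parents.
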(event `self.ReceiveBeginPlay`
  ;[1 1 0] Parent call
  (`parent.ReceiveBeginPlay`))

(event `self.ReceiveTick`
  (params (DeltaSeconds :type "Float (single-precision)"))
  ;[1 1 0] Parent call
  (`parent.ReceiveTick` DeltaSeconds))

(event `self.ServerRequestJoinNewPlayer`
  (params (Username :type Text) (BypassLobby :type Boolean))
  ;[1 1 0] Join player
  (bind _asgame_mode_base_mines (cast `/Game/Blueprints/GameModes/GameModeBaseMines` (`GameplayStatics.GetGameMode`)))
  (set `self.GameModeRef` _asgame_mode_base_mines)
  (bind _spawnplace (`/Game/Blueprints/GameModes/GameModeBaseGame.GetSpawnPlaceByOrder` _asgame_mode_base_mines))
  (set `self.PlayerIndex` _spawnplace)
  (bind _rndcolor (`/Game/Blueprints/GameModes/GameModeBaseGame.GetRandomPlayerColor` _asgame_mode_base_mines))
  (set `self.PlayerColor` _rndcolor)
  (`/Game/Blueprints/GameModes/GameModeBaseMines.CreateNewPlayerMines` _asgame_mode_base_mines self (`self.PlayerColor`) (`self.PlayerIndex`)))

(fn `UserConstructionScript`
  (`parent.UserConstructionScript`))