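; Player controller Blueprint that handles a new player's request to join a game run by GameModeBaseMechanic.
; ServerRequestJoinNewPlayer caches the game mode, gets a random player color and an ordered spawn place from it, and stores both.
; It then asks the game mode to create the player's mechanic at that place.
; BeginPlay, Tick and construction only call the parent.
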(event `self.ReceiveBeginPlay`
  ;[1 1 0] Parent call
  (`parent.ReceiveBeginPlay`))

(event `self.ReceiveTick`
  (params (DeltaSeconds :type "Float (single-precision)"))
  ;[1 1 0] Parent call
  (`parent.ReceiveTick` DeltaSeconds))

(event `self.ServerRequestJoinNewPlayer`
  (params (Username :type Text) (BypassLobby :type Boolean))
  ;[1 1 0] Join player
  (bind _asgame_mode_base_mechanic (cast `/Game/Blueprints/GameModes/GameModeBaseMechanic` (`GameplayStatics.GetGameMode`)))
  (set `self.GameModeRef` _asgame_mode_base_mechanic)
  (bind _rndcolor (`/Game/Blueprints/GameModes/GameModeBaseGame.GetRandomPlayerColor` _asgame_mode_base_mechanic))
  (set `self.PlayerColor` _rndcolor)
  (bind _spawnplace (`/Game/Blueprints/GameModes/GameModeBaseGame.GetSpawnPlaceByOrder` _asgame_mode_base_mechanic))
  (set `self.Index` _spawnplace)
  (`/Game/Blueprints/GameModes/GameModeBaseMechanic.CreateNewPlayerMechanic` _asgame_mode_base_mechanic self (`self.Index`)))

(fn `UserConstructionScript`
  (`parent.UserConstructionScript`))