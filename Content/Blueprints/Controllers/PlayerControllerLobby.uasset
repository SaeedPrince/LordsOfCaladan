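; Player controller for the lobby that shows the lobby menu and relays the request to travel out of the lobby.
; On BeginPlay it caches the main game instance, then creates and displays the lobby widget on both authority and remote sides through separate branches.
; Server- and Client-named events hand travel to the lobby game mode's ServerTravel and remove the menu from the viewport.
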(event `self.ReceiveBeginPlay`
  ;[1 1 0] Begin play
  (bind _asgame_instance_main (cast `/Game/Blueprints/Instances/GameInstanceMain` (`GameplayStatics.GetGameInstance`))
    (:`then`
      (set `self.GameInstanceRef` _asgame_instance_main)
      (`/Engine/EditorBlueprintResources/ActorMacros.Switch Has Authority`
        (:`Authority`
          (`self.CreateMenu`))
        (:`Remote`
          (bind _returnvalue (`|CreateWidget` "/Game/Blueprints/Widgets/Widget_MenuLobby.Widget_MenuLobby_C" self))
          (bind _output_get (set `self.WidgetMenuLobby` _returnvalue))
          (`UserWidget.AddToViewport` _output_get 0))))
    (:`CastFailed`
      (`KismetSystemLibrary.PrintString` "Cast to game instance failed" true true (struct :`R` 1.0 :`A` 1.0) 10.0))))

(event `CreateMenu`
  ;[1 1 0] Begin play
  (bind _returnvalue (`|CreateWidget` "/Game/Blueprints/Widgets/Widget_MenuLobby.Widget_MenuLobby_C" self))
  (bind _output_get (set `self.WidgetMenuLobby` _returnvalue))
  (`UserWidget.AddToViewport` _output_get 0))

(event `ServerSeamlessTravel`
  ;[1 1 0] Seamless travel
  (bind _asgame_mode_base_lobby (cast `/Game/Blueprints/GameModes/GameModeBaseLobby` (`GameplayStatics.GetGameMode`)))
  (`/Game/Blueprints/GameModes/GameModeBaseLobby.ServerTravel` _asgame_mode_base_lobby))

(event `ClientRemoveMenuLobby`
  (bind _widgetmenulobby (`self.WidgetMenuLobby`))
  ;[1 1 0] Remove widget
  (if (`Widget.IsInViewport` _widgetmenulobby)
    (`Widget.RemoveFromParent` _widgetmenulobby)))

(fn `UserConstructionScript`)