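; Game HUD that draws a drag-selection box to select HumanAI actors with the mouse.
; StartDrawRectangle stores the mouse start point and turns on ShowHUD, letting DrawHUD outline the box to the current cursor with four lines.
; Each drawn frame gathers the actors inside the box with GetActorsInSelectionRectangle.
; StopDrawRectangle hides the HUD, hands the selection to PlayerController_Game and resets its state.
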(event `self.ReceiveBeginPlay`
  (bind _asplayer_controller_game (cast `/Game/Blueprints/Controllers/PlayerController_Game` (`self.GetOwningPlayerController`))
    (:`then`
      (set `self.ControllerRef` _asplayer_controller_game))
    (:`CastFailed`
      (`KismetSystemLibrary.PrintString` "Cast to player controller failed." true true (struct :`R` 1.0 :`A` 1.0) 10.0))))

(event `StartDrawRectangle`
  (bind (_locationx _locationy) (`PlayerController.GetMousePosition` (`self.ControllerRef`)))
  (set `self.bShowHUD` true)
  (set `self.StartX` _locationx)
  (set `self.StartY` _locationy))

(event `ShowHudSet`
  (params (NewValue :type Boolean))
  (set `self.bShowHUD` NewValue))

(event `StopDrawRectangle`
  (set `self.bShowHUD` false)
  (`/Game/Blueprints/Controllers/PlayerController_Game.PersonSelectedArraySet` (`self.ControllerRef`) (`self.SelectedActors`))
  (set `self.StartX` 0.0)
  (set `self.StartY` 0.0)
  (set `self.LocationX` 0.0)
  (set `self.LocationY` 0.0)
  (`KismetArrayLibrary.Array_Clear` (`self.SelectedActors`)))

(event `self.ReceiveDrawHUD`
  (params (SizeX :type Integer) (SizeY :type Integer))
  (bind _startx (`self.StartX`))
  (bind _starty (`self.StartY`))
  (bind _locationx (`self.LocationX`))
  (bind _locationy (`self.LocationY`))
  (bind _controllerref (`self.ControllerRef`))
  (bind (_locationx_2 _locationy_2) (`PlayerController.GetMousePosition` _controllerref))
  (`/Engine/EditorBlueprintResources/StandardMacros.IsValid` _controllerref
    (:`Is Valid`
      (set `self.LocationX` _locationx_2)
      (set `self.LocationY` _locationy_2)
      (`self.DrawEmptyRect` _startx _starty _locationx _locationy 2.0)
      (set `self.SelectedActors` (`self.GetActorsInSelectionRectangle` "/Game/Blueprints/Characters/HumanAI.HumanAI_C" (`KismetMathLibrary.MakeVector2D` _startx _starty) (`KismetMathLibrary.MakeVector2D` _locationx _locationy) false)))))

(fn `DrawEmptyRect`
  (params (X1 :type "Float (double-precision)") (Y1 :type "Float (double-precision)") (X2 :type "Float (double-precision)") (Y2 :type "Float (double-precision)") (Thickness :type "Float (double-precision)"))
  (locals (LineColor :type "LinearColor Structure" :default (struct :`R` 1.0 :`A` 0.25)))
  (bind _linecolor (`local.LineColor`))
  (`self.DrawLine` X1 Y1 X2 Y1 _linecolor Thickness)
  (`self.DrawLine` X2 Y1 X2 Y2 _linecolor Thickness)
  (`self.DrawLine` X2 Y2 X1 Y2 _linecolor Thickness)
  (`self.DrawLine` X1 Y2 X1 Y1 _linecolor Thickness))

(fn `UserConstructionScript`)