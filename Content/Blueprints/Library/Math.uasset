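; Math helper library with functions for balanced random integer arrays and 2D square corners.
; RandomArray draws random entries from a shrinking candidate list, retiring each once it reaches an equal share of Total, yielding a shuffled, evenly distributed result.
; Box2DVertices returns four corners around an origin in winding order at zero Z, treating Side as the half-extent.
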(fn `Box2DVertices`
  (params (Origin :type "Vector Structure") (Side :type "Float (double-precision)"))
  (returns (ReturnValue :type "Array of Vector Structure"))
  (locals (Point1 :type "Vector Structure") (Point2 :type "Vector Structure") (Point3 :type "Vector Structure") (Point4 :type "Vector Structure"))
  (bind _x (.x Origin))
  (bind _y (.y Origin))
  (bind _returnvalue (- _x Side))
  (bind _returnvalue_2 (- _y Side))
  (bind _returnvalue_3 (+ _y Side))
  (bind _returnvalue_4 (+ _x Side))
  (set `local.Point1` (`KismetMathLibrary.MakeVector` _returnvalue _returnvalue_2))
  (set `local.Point2` (`KismetMathLibrary.MakeVector` _returnvalue_4 _returnvalue_2))
  (set `local.Point3` (`KismetMathLibrary.MakeVector` _returnvalue_4 _returnvalue_3))
  (set `local.Point4` (`KismetMathLibrary.MakeVector` _returnvalue _returnvalue_3))
  (return (`|MakeArray` (`local.Point1`) (`local.Point2`) (`local.Point3`) (`local.Point4`))))

(fn `RandomArray`
  (params (Total :type Integer) (OccurnessArray :type "Array of Integer"))
  (returns (ReturnValue :type "Array of Integer"))
  (locals (SelectionArray :type "Array of Integer") (OccurnessCount :type Integer) (Occurness :type "Array of Integer") (OutInteger :type "Array of Integer") (OccurenessIndex :type Integer))
  (bind _occurness (`local.Occurness`))
  (bind _selectionarray (`local.SelectionArray`))
  (set `local.SelectionArray` OccurnessArray)
  (set `local.OccurnessCount` (/ Total (`KismetArrayLibrary.Array_Length` OccurnessArray)))
  (for _ (range (`KismetArrayLibrary.Array_Length` _selectionarray))
    (`KismetArrayLibrary.Array_Add` _occurness))
  (while (> (`KismetArrayLibrary.Array_Length` _selectionarray) 0)
    (bind _output_get (set `local.OccurenessIndex` (`KismetMathLibrary.RandomIntegerInRange` 0 (- (`KismetArrayLibrary.Array_Length` _selectionarray) 1))))
    (`KismetArrayLibrary.Array_Add` (`local.OutInteger`) (`|GetArrayItem` _selectionarray _output_get))
    (bind _result (`/Engine/EditorBlueprintResources/StandardMacros.IncrementInt` (`|GetArrayItem` _occurness _output_get))
      (:`  `
        (if (>= _result (`local.OccurnessCount`))
          (`KismetArrayLibrary.Array_Remove` _selectionarray _output_get)
          (`KismetArrayLibrary.Array_Remove` _occurness _output_get)))))
  (return (`local.OutInteger`)))