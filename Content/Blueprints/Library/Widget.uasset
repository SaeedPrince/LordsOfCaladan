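; Widget helper function library that supplies text for session search results and a checkbox state check.
; SearchHeader gives the column titles, and SessionToText builds a matching row from a session's server name (truncated), current and max players, and ping.
; AllUnchecked loops over a checkbox array, setting its result false and stopping at the first checked box, with no explicit true assignment.
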(fn `AllUnchecked`
  (params (CheckboxArray :type "Array of CheckBox Object Reference"))
  (returns (ReturnValue :type Boolean))
  (locals (OutBool :type Boolean :default true))
  (for _array_element CheckboxArray
    (if (`|EnumEquality` (`CheckBox.GetCheckedState` _array_element) "Checked")
      (set `local.OutBool` false)
      (break)))
  (return (`local.OutBool`)))

(fn `SearchHeader`
  (returns (ReturnValue :type "Array of Text"))
  (return (`|MakeArray` "Server Name" "Current Players" "Max Players" "Ping" :!type "Text")))

(fn `SessionToText`
  (params (Session :type "BlueprintSessionResult Structure"))
  (returns (ReturnValue :type "Array of Text"))
  (locals (OutText :type "Array of Text"))
  (return (`|MakeArray` (`KismetTextLibrary.Conv_StringToText` (`KismetStringLibrary.Left` (`FindSessionsCallbackProxy.GetServerName` Session) 15)) (`KismetTextLibrary.Conv_IntToText` (`FindSessionsCallbackProxy.GetCurrentPlayers` Session)) (`KismetTextLibrary.Conv_IntToText` (`FindSessionsCallbackProxy.GetMaxPlayers` Session)) (`KismetTextLibrary.Conv_IntToText` (`FindSessionsCallbackProxy.GetPingInMs` Session)))))