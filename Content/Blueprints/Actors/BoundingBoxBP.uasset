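; BoundingBoxBP is an actor whose box component is sized from movement bounds and a vertical trace range.
; Its construction script sets the box half-extents from the bounds length, bounds width and the span between the minimum and maximum trace Z offsets.
; It then places the box at world X and Y zero, with its height centered on that Z range, regardless of the actor's location.
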(fn `UserConstructionScript`
  (bind _box (`self.Box`))
  (bind _offsettracezmin (`self.OffsetTraceZMin`))
  (bind _returnvalue (/ (- (`self.OffsetTraceZMax`) _offsettracezmin) 2.0))
  (`BoxComponent.SetBoxExtent` _box (`KismetMathLibrary.MakeVector` (/ (`self.MovementBoundsLength`) 2.0) (/ (`self.MovementBoundsWidth`) 2.0) _returnvalue) true)
  (`SceneComponent.K2_SetWorldLocation` _box (`KismetMathLibrary.MakeVector` 0.0 0.0 (+ _returnvalue _offsettracezmin)) false false))