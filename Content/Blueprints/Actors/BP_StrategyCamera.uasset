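; Strategy camera actor that pans, rotates and zooms a spring arm target within box bounds via keyboard, gamepad, mouse drag, screen-edge scroll and touch gestures.
; Inputs set clamped target values, with height from a downward line trace, and Tick lerps toward them.
; Pan speed scales with zoom distance.
; MoveCamera teleports or glides to a point, locking input until a glide nears its destination.
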(event `CameraMoveForward`
  (params (AxisValue :type "Float (double-precision)"))
  ;[1 1 1] Keyboard/gamepad movement control
  (if (`self.IsInputEnabled`)
    (`self.AddMovementX` AxisValue)))

(event `CameraZoomIn`
  ;[1 1 1] Zoom control
  (if (`self.IsInputEnabled`)
    (set `self.TargetDistance` (`KismetMathLibrary.FClamp` (- (`self.TargetDistance`) (`self.ZoomSpeed`)) (`self.MinDistance`) (`self.MaxDistance`)))
    (`self.SetAdjustedMovementSpeed` :!label _label)))

(event `InputTouch`
  (params (Location :type "Vector Structure") (FingerIndex :type "ETouchIndex Enum"))
  (bind _returnvalue (`|EnumEquality` FingerIndex "Touch2"))
  (bind _returnvalue_2 (`|EnumEquality` FingerIndex "Touch1"))
  (bind _returnvalue_3 (`KismetMathLibrary.MakeVector2D` (.x Location) (.y Location)))
  ;[1 1 1] Touch controls
  (:`Pressed`
    (if (`self.IsInputEnabled`)
      (`|ExecutionSequence`
        (:`then_0`
          (if _returnvalue_2
            (set `self.IsTouch1` true)
            (set `self.TouchLocation1` _returnvalue_3)))
        (:`then_1`
          (if _returnvalue
            (set `self.IsTouch2` true)
            (set `self.TouchLocation2` _returnvalue_3))))))
  (:`Released`
    (`|ExecutionSequence`
      (:`then_0`
        (if _returnvalue_2
          (set `self.IsTouch1` false)))
      (:`then_1`
        (if _returnvalue
          (set `self.IsTouch2` false))))))

(event `CameraMoveRight`
  (params (AxisValue :type "Float (double-precision)"))
  ;[1 1 1] Keyboard/gamepad movement control
  (if (`self.IsInputEnabled`)
    (`self.AddMovementY` AxisValue)))

(event `CameraZoomOut`
  ;[1 1 1] Zoom control
  (if (`self.IsInputEnabled`)
    (set `self.TargetDistance` (`KismetMathLibrary.FClamp` (+ (`self.TargetDistance`) (`self.ZoomSpeed`)) (`self.MinDistance`) (`self.MaxDistance`)))
    (goto _label)))

(event `CameraRotate`
  (params (AxisValue :type "Float (double-precision)"))
  ;[1 1 1] Keyboard/gamepad rotation control
  (if (`self.IsInputEnabled`)
    (`self.AddRotation` AxisValue)))

(event `CameraResetRotation`
  ;[1 1 1] Home
  (set `self.TargetRotation` 0.0))

(event `self.ReceiveTick`
  (params (DeltaSeconds :type "Float (single-precision)"))
  (`|ExecutionSequence`
    (:`then_0`
      (`self.UpdateMovement` ; Update camera movement
        (:`Out`
          (`self.UpdateRotation` ; Update camera rotation
            (:`Out`
              (`self.UpdateZoom`) ; Update camera zoom
            )))))
    (:`then_1`
      (`self.ProcessMouseWindowBorderScroll`) ; Process mouse window border scroll - disable this if you are going to use touch controls
    )
    (:`then_2`
      ;[1 1 1] Mouse movement control and update
      (if (`self.IsInputEnabled`)
        (`/Engine/EditorBlueprintResources/StandardMacros.Gate` true :!label _label_2
          (:`Exit`
            (`self.AddMovementX` (`self.GetInputAxisKeyValue`)
              (:`Out`
                (`self.AddMovementY` (`self.GetInputAxisKeyValue`))))))))
    (:`then_3`
      ;[1 1 1] Mouse rotation control and update
      (if (`self.IsInputEnabled`)
        (`/Engine/EditorBlueprintResources/StandardMacros.Gate` true :!label _label_3
          (:`Exit`
            (`self.AddRotation` (`self.GetInputAxisKeyValue`))))))
    (:`then_4`
      (`self.ProcessTouch`) ; Process touch (pan/rotate/zoom)
    )))

(event `Key|LeftMouseButton`
  (params (Key :type "Key Structure"))
  ;[1 1 1] Mouse movement control and update
  (:`Pressed`
    (goto _label_2 :!via `Open`))
  (:`Released`
    (goto _label_2 :!via `Close`)))

(event `Key|RightMouseButton`
  (params (Key :type "Key Structure"))
  ;[1 1 1] Mouse rotation control and update
  (:`Pressed`
    (goto _label_3 :!via `Open`))
  (:`Released`
    (goto _label_3 :!via `Close`)))

(fn `IsCameraMoving`
  (returns (IsMoving :type Boolean))
  (return (`self.IsMoving`)))

(fn `MoveCamera`
  (params (X :type "Float (double-precision)") (Y :type "Float (double-precision)") (SetRotation :type Boolean) (Rotation :type "Float (double-precision)") (SetDistance :type Boolean) (Distance :type "Float (double-precision)") (Teleport :type Boolean))
  (bind _returnvalue (`KismetMathLibrary.FClamp` Distance (`self.MinDistance`) (`self.MaxDistance`)))
  (`|ExecutionSequence`
    (:`then_0`
      ;[1 1 1] Location
      (set `self.TargetX` (`KismetMathLibrary.FClamp` X (`self.MinX`) (`self.MaxX`)))
      (set `self.TargetY` (`KismetMathLibrary.FClamp` Y (`self.MinY`) (`self.MaxY`)))
      (`self.SetTargetZ`
        (:`Out`
          (if Teleport
            (`SceneComponent.K2_SetWorldLocation` (`self.Target`) (`KismetMathLibrary.MakeVector` (`self.TargetX`) (`self.TargetY`) (`self.TargetZ`)) false false)
            (else
              (set `self.IsMoving` true)
              (set `self.WasInputEnabled` (`self.IsInputEnabled`))
              (set `self.IsInputEnabled` false))))))
    (:`then_1`
      ;[1 1 1] Rotation
      (if SetRotation
        (if Teleport
          (bind _output_get (set `self.CurrentRotation` Rotation))
          (bind _output_get_2 (set `self.TargetRotation` _output_get))
          (`SceneComponent.K2_SetRelativeRotation` (`self.Target`) (`KismetMathLibrary.MakeRotator` 0.0 0.0 _output_get_2) false false)
          (else
            (set `self.TargetRotation` Rotation)))))
    (:`then_2`
      ;[1 1 1] Zoom
      (if SetDistance
        (if Teleport
          (set `SpringArmComponent.TargetArmLength` _returnvalue (`self.SpringArm`)))
        (set `self.TargetDistance` _returnvalue)
        (`self.SetAdjustedMovementSpeed`)))))

(fn `SetInputEnabled`
  (params (InputEnabled :type Boolean))
  (set `self.IsInputEnabled` InputEnabled))

(fn `UserConstructionScript`
  (bind _offsettracezmin (`self.OffsetTraceZmin`))
  (bind _initialrotation (`self.InitialRotation`))
  (bind _boundingbox (`self.BoundingBox`))
  (bind _movementspeed (`self.MovementSpeed`))
  (bind _returnvalue (/ (`self.MovementBoundsWidth`) 2.0))
  (bind _x (.x (`self.K2_GetActorLocation`)))
  (bind _y (.y (`self.K2_GetActorLocation`)))
  (bind _z (.z (`self.K2_GetActorLocation`)))
  (bind _returnvalue_2 (/ (`self.MovementBoundsLength`) 2.0))
  (bind _returnvalue_3 (/ (- (`self.OffsetTraceZmax`) _offsettracezmin) 2.0))
  (`|ExecutionSequence`
    (:`then_0`
      ;[1 1 1] Set bounding box helper extents and relative location
      (`BoxComponent.SetBoxExtent` _boundingbox (`KismetMathLibrary.MakeVector` (/ (`self.MovementBoundsLength`) 2.0) (/ (`self.MovementBoundsWidth`) 2.0) _returnvalue_3) true)
      (`SceneComponent.K2_SetRelativeLocation` _boundingbox (`KismetMathLibrary.MakeVector` 0.0 0.0 (+ _returnvalue_3 _offsettracezmin)) false false)
      ;[1 1 1] Set camera movement world X/Y boundaries and camera offset trace start/end
      (set `self.MinX` (- _x _returnvalue_2))
      (set `self.MaxX` (+ _x _returnvalue_2))
      (set `self.MinY` (- _y _returnvalue))
      (set `self.MaxY` (+ _y _returnvalue))
      (set `self.TraceStartZ` (+ _z (`self.OffsetTraceZmax`)))
      (set `self.TraceEndZ` (+ _z (`self.OffsetTraceZmin`))))
    (:`then_1`
      ;[1 1 1] Set initial TargetX/TargetY/TargetZ and adjust camera target location
      (set `self.TargetX` (`KismetMathLibrary.FClamp` (+ (.x (`self.K2_GetActorLocation`)) (`self.InitialX`)) (`self.MinX`) (`self.MaxX`)))
      (set `self.TargetY` (`KismetMathLibrary.FClamp` (+ (.y (`self.K2_GetActorLocation`)) (`self.InitialY`)) (`self.MinY`) (`self.MaxY`)))
      (set `self.TargetZ` (`self.TraceEndZ`))
      (`self.SetTargetZ`
        (:`Out`
          (`SceneComponent.K2_SetWorldLocation` (`self.Target`) (`KismetMathLibrary.MakeVector` (`self.TargetX`) (`self.TargetY`) (`self.TargetZ`)) false false)
          ;[1 1 1] Set initial CurrentRotation/TargetRotation and adjust camera target rotation
          (bind _output_get (set `self.TargetRotation` _initialrotation))
          (set `self.CurrentRotation` _initialrotation)
          (`SceneComponent.K2_SetRelativeRotation` (`self.Target`) (`KismetMathLibrary.MakeRotator` 0.0 0.0 _output_get) false false)
          ;[1 1 1] Setup camera spring arm - set camera angle and initial distance
          (`SceneComponent.K2_SetRelativeRotation` (`self.SpringArm`) (`KismetMathLibrary.MakeRotator` 0.0 (- 0.0 (`self.Angle`))) false false)
          (bind _output_get_2 (set `self.TargetDistance` (`KismetMathLibrary.FClamp` (`self.InitialDistance`) (`self.MinDistance`) (`self.MaxDistance`))))
          (set `SpringArmComponent.TargetArmLength` _output_get_2 (`self.SpringArm`))
          ;[1 1 1] Setup adaptive movement speed range and set AdjustedMovementSpeed
          (set `self.MovementSpeedRange` (- (* (`self.MaxMovementSpeedMultiplier`) _movementspeed) _movementspeed))
          (`self.SetAdjustedMovementSpeed`))))))