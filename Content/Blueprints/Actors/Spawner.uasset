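; Spawner actor that queues and spawns a building's civilian and military AI humans for a player.
; ServerActiveSpawner fills JobQueue from the building's generation counts, then starts a looping timer on SpawnerJob, which is not defined here.
; Capsule overlaps flag the spawner as occupied.
; SpawnerJobBackup, on authority, waits until clear, spawns a random-bodied human and possesses it with a new controller from the first job, without dequeuing it.
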(event `self.Capsule.OnComponentBeginOverlap`
  (params (OverlappedComponent :type "PrimitiveComponent Object Reference") (OtherActor :type "Actor Object Reference") (OtherComp :type "PrimitiveComponent Object Reference") (OtherBodyIndex :type Integer) (bFromSweep :type Boolean) (SweepResult :type "HitResult Structure (by ref)"))
  ;[1 1 0] If spawner occupied by anything don't spawn
  (set `self.SpawnerOccupied` true))

(event `self.Capsule.OnComponentEndOverlap`
  (params (OverlappedComponent :type "PrimitiveComponent Object Reference") (OtherActor :type "Actor Object Reference") (OtherComp :type "PrimitiveComponent Object Reference") (OtherBodyIndex :type Integer))
  ;[1 1 0] If spawner occupied by anything don't spawn
  (set `self.SpawnerOccupied` false))

(event `ServerActiveSpawner`
  (params (Building :type "/Game/Assets/BP_Meshes/Architecture/BP_House Object Reference") (PlayerIndex :type Integer))
  ;[1 1 0] Activater
  (`self.MacAssignJobToSpawner` Building (`/Game/Assets/BP_Meshes/Architecture/BP_House.CivilGenerationCount` Building) (`/Game/Assets/BP_Meshes/Architecture/BP_House.CivilPlacements` Building) 0 PlayerIndex)
  (`self.MacAssignJobToSpawner` Building (`/Game/Assets/BP_Meshes/Architecture/BP_House.MilitGenerationCount` Building) (`/Game/Assets/BP_Meshes/Architecture/BP_House.MilitPlacements` Building) 1 PlayerIndex)
  (bind _returnvalue (`KismetSystemLibrary.K2_SetTimer` self "SpawnerJob" (`self.SpawnCheckPeriod`) true))
  (set `self.TimerSpawnerJob` _returnvalue))

(fn `SpawnerJobBackup`
  (locals (Body :type "/Game/Blueprints/Structures/Game/StructBody Structure"))
  (bind _returnvalue (`self.K2_GetActorLocation`))
  (bind _returnvalue_2 (`self.K2_GetActorRotation`))
  (bind _jobqueue (`self.JobQueue`))
  (bind (_persontype _soldiertype _playerindex) (break `/Game/Blueprints/Structures/Object/StructAIController` (`|GetArrayItem` _jobqueue)))
  (`/Engine/EditorBlueprintResources/ActorMacros.Switch Has Authority`
    (:`Authority`
      (if (> (`KismetArrayLibrary.Array_Length` _jobqueue) 0)
        (if (not (`self.SpawnerOccupied`))
          (bind _returnvalue_3 (`AIBlueprintHelperLibrary.SpawnAIFromClass` "/Game/Blueprints/Characters/HumanAI.HumanAI_C" "/Game/Blueprints/AI/BehaviorTree/BT_Civilian.BT_Civilian" _returnvalue _returnvalue_2))
          (`/Engine/EditorBlueprintResources/StandardMacros.IsValid` _returnvalue_3
            (:`Is Valid`
              (`KismetSystemLibrary.PrintString` "AI spawned" true true (struct :`G` 1.0 :`A` 1.0) 8.0)
              (set `Pawn.AIControllerClass` "/Game/Blueprints/Controllers/AIController_Game.AIController_Game_C" _returnvalue_3)
              (bind _ashuman_bp (cast `/Game/Blueprints/Characters/HumanBP` _returnvalue_3))
              (bind _output_get (set `local.Body` (`/Game/Blueprints/Libraries/LibHuman.RandomBody`)))
              (`/Game/Blueprints/Characters/HumanBP.SetOrgans` _ashuman_bp _output_get)
              (`/Game/Blueprints/Characters/HumanBP.MulticastSetOrgans` _ashuman_bp _output_get)
              (set `/Game/Blueprints/Characters/HumanBP.PlayerIndex` 0 _ashuman_bp)
              (bind _returnvalue_4 (`|SpawnActorFromClass` "/Game/Blueprints/Controllers/AIController_Game.AIController_Game_C" (`KismetMathLibrary.MakeTransform` _returnvalue _returnvalue_2) "Undefined" "OverrideRootScale" null (make `/Game/Blueprints/Structures/Object/StructAIController` _persontype 0 _playerindex) null))
              (`/Engine/EditorBlueprintResources/StandardMacros.IsValid` _returnvalue_4
                (:`Is Valid`
                  (`Controller.Possess` _returnvalue_4 _ashuman_bp)
                  (set `/Game/Blueprints/Characters/HumanBP.AIControllerRef` _returnvalue_4 _ashuman_bp))))
            (:`Is Not Valid`
              (`KismetSystemLibrary.PrintString` "AI didn't spawned" true true (struct :`R` 1.0 :`A` 1.0) 8.0)))
          (else
            (`KismetSystemLibrary.PrintString` (`KismetStringLibrary.Concat_StrStr` (`KismetSystemLibrary.GetObjectName` self) " is waiting") true true (struct :`R` 1.0 :`G` 1.0 :`A` 1.0) 8.0)))
        (else
          (`KismetSystemLibrary.K2_ClearAndInvalidateTimerHandle` (`self.TimerSpawnerJob`)))))))

(fn `UserConstructionScript`)