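; Game instance that manages multiplayer sessions, with events to create, find, join and destroy them.
; Creation and search each come in standard and Advanced Sessions variants, with selectable LAN use; advanced creation adds a server name and a dedicated-server option.
; Successful creation opens the Lobby level as a listen server, and successful searches pass their results to PlayerControllerMenu for display.
; Outcomes are mostly reported with debug prints.
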(event `CreateSessionNormal`
  (params (Player :type "PlayerController Object Reference") (UseLan :type Boolean))
  ;[1 1 0] Create session normal
  (`CreateSessionCallbackProxy.CreateSession` Player 6 UseLan
    (:`OnSuccess`
      (`KismetSystemLibrary.PrintString` "Session created." true true (struct :`G` 1.0 :`A` 1.0) 8.0)
      (`GameplayStatics.OpenLevel` "Lobby" true "listen"))
    (:`OnFailure`
      (`KismetSystemLibrary.PrintString` "Session creation failed." true true (struct :`R` 1.0 :`A` 1.0) 8.0))))

(event `CreateSessionAdvanced`
  (params (Host :type "PlayerController Object Reference") (UseLan :type Boolean) (UseDedicated :type Boolean))
  ;[1 1 0] Create session advanced
  (`CreateSessionCallbackProxyAdvanced.CreateAdvancedSession` (`|MakeArray` (`AdvancedSessionsLibrary.MakeLiteralSessionPropertyString` "ServerName" "Saeed")) Host 6 6 UseLan true UseDedicated false false
    (:`OnSuccess`
      (`KismetSystemLibrary.PrintString` "Session created." true true (struct :`G` 1.0 :`A` 1.0) 8.0)
      (`GameplayStatics.OpenLevel` "Lobby" true "listen"))
    (:`OnFailure`
      (`KismetSystemLibrary.PrintString` "Session creation failed." true true (struct :`R` 1.0 :`A` 1.0) 8.0))))

(event `FindAdvancedSession`
  (params (Searcher :type "PlayerController Object Reference") (UseLan :type Boolean))
  ;[1 1 0] Find advanced session
  (bind _results (`FindSessionsCallbackProxyAdvanced.FindSessionsAdvanced` Searcher 10 UseLan "AllServers")
    (:`OnSuccess`
      (bind _asplayer_controller_menu (cast `/Game/Blueprints/Controllers/PlayerControllerMenu` Searcher))
      (`/Game/Blueprints/Controllers/PlayerControllerMenu.ClientShowSearchResult` _asplayer_controller_menu _results))
    (:`OnFailure`
      (`KismetSystemLibrary.PrintString` "Session search failed." true true (struct :`R` 1.0 :`A` 1.0) 8.0))))

(event `FindSessionNormal`
  (params (Player :type "PlayerController Object Reference") (UseLan :type Boolean))
  ;[1 1 0] Find session normal
  (bind _results (`FindSessionsCallbackProxy.FindSessions` Player 6 UseLan)
    (:`OnSuccess`
      (bind _asplayer_controller_menu (cast `/Game/Blueprints/Controllers/PlayerControllerMenu` Player))
      (`/Game/Blueprints/Controllers/PlayerControllerMenu.ClientShowSearchResult` _asplayer_controller_menu _results))
    (:`OnFailure`
      (`KismetSystemLibrary.PrintString` "Session search failed." true true (struct :`R` 1.0 :`A` 1.0) 8.0))))

(event `JoinGame`
  (params (Joiner :type "PlayerController Object Reference") (Session :type "BlueprintSessionResult Structure"))
  ;[1 1 0] Session join
  (`JoinSessionCallbackProxy.JoinSession` Joiner Session
    (:`OnSuccess`
      (`KismetSystemLibrary.PrintString` "Session joined." true true (struct :`G` 1.0 :`A` 1.0) 8.0))
    (:`OnFailure`
      (`KismetSystemLibrary.PrintString` "Session join failed." true true (struct :`R` 1.0 :`A` 1.0) 8.0))))

(event `SessionDestroy`
  (params (Controller :type "PlayerController Object Reference"))
  ;[1 1 0] Session destroy
  (`DestroySessionCallbackProxy.DestroySession` Controller
    (:`OnSuccess`
      (`KismetSystemLibrary.PrintString` "Session destroyed." true true (struct :`G` 1.0 :`A` 1.0) 8.0))
    (:`OnFailure`
      (`KismetSystemLibrary.PrintString` "Session destroy failed." true true (struct :`R` 1.0 :`A` 1.0) 8.0))))