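; Game mode that sets up the server match for a settlement-style game with two player places, Hilltop and Lowland.
; Server initialization spawns both fortresses from map data and starts server time.
; CreateNewPlayerStart possesses a new HumanPlayer with a random body, assigns a fortress and border, seeds population and items, and refreshes player colors.
; Spawn helpers fill free building slots with AI and item stacks, alternating between two soldier types.
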(event `InitializeServerStart`
  (params (PlStart :type "Array of PlayerStart Object Reference"))
  ;[1 1 0] Initialize server
  (set `self.PlayerStarts` PlStart)
  (`self.MacSpawnMapObjects`)
  (`self.StartServerTime`))

(event `SpawnSoldier`
  (params (SoldierCount :type Integer) (Building :type "/Game/Assets/BP_Meshes/Architecture/BP_House Object Reference"))
  ;[1 1 0] Spawn soldier
  (for _ (range SoldierCount)
    (if (`|EnumEquality` (`self.SoldierType`) "NewEnumerator1")
      (set `self.SoldierType` "NewEnumerator0")
      (else
        (set `self.SoldierType` "NewEnumerator1")))
    (`self.MacSpawnSoldier` Building (`self.SoldierType`))
    (`KismetSystemLibrary.Delay` 1.0)))

(event `SpawnPopulation`
  (params (Count :type Integer) (Building :type "/Game/Assets/BP_Meshes/Architecture/BP_House Object Reference") (PersonType :type "/Game/Blueprints/Enums/EnumPersonType Enum" :default "NewEnumerator0"))
  ;[1 1 0] SpawnPopulation
  (for _ (range Count)
    (if (`|EnumEquality` PersonType "NewEnumerator1")
      (if (`|EnumEquality` (`self.SoldierType`) "NewEnumerator1")
        (set `self.SoldierType` "NewEnumerator0")
        (else
          (set `self.SoldierType` "NewEnumerator1"))))
    (`self.MacSpawnPopulation` Building PersonType)))

(fn `CreateNewPlayerStart`
  (params (Player :type "/Game/Blueprints/Controllers/PlayerControllerStart Object Reference") (Color :type "LinearColor Structure") (Place :type Integer))
  (locals (Body :type "/Game/Blueprints/Structures/Game/StructBody Structure") (CustomStarts :type "Array of Vector Structure"))
  (bind _body (`local.Body`))
  (bind _output (`|GetArrayItem` (`self.PlayerStarts`) Place))
  (bind _returnvalue (`|SpawnActorFromClass` "/Game/Blueprints/Characters/HumanPlayer.HumanPlayer_C" (`KismetMathLibrary.MakeTransform` (`self.K2_GetActorLocation` _output) (`self.K2_GetActorRotation` _output)) "Undefined" "OverrideRootScale" null (make `/Game/Blueprints/Structures/Object/StructHuman` :`PlayerIndex` Place) null))
  (`Controller.Possess` Player _returnvalue)
  (set `/Game/Blueprints/Controllers/PlayerController_Game.CharacterRef` _returnvalue Player)
  (set `/Game/Blueprints/Characters/HumanBP.ControllerRef` Player _returnvalue)
  (set `local.Body` (`/Game/Blueprints/Libraries/LibHuman.RandomBody`))
  (`/Game/Blueprints/Characters/HumanBP.MulticastSetOrgans` _returnvalue _body)
  (`/Game/Blueprints/Characters/HumanBP.SetOrgans` _returnvalue _body)
  (bind (_fortress _border) (`self.PlayerFortress` Place Player Color))
  (if (!= _fortress null)
    (`KismetArrayLibrary.Array_Add` (`/Game/Blueprints/Controllers/PlayerController_Game.Buildings` Player) _fortress)
    (set `/Game/Assets/BP_Meshes/Architecture/BP_House.Player` Player _fortress)
    (set `/Game/Blueprints/Controllers/PlayerController_Game.BorderStructRef` _border Player)
    (`self.SpawnPopulation` 4 _fortress "NewEnumerator0")
    (`self.SpawnPopulation` 4 _fortress "NewEnumerator1"))
  (bind _outactors (`GameplayStatics.GetAllActorsOfClass` "/Game/Blueprints/Characters/HumanPlayer.HumanPlayer_C"))
  (for _array_element _outactors
    (bind _controllerref (`/Game/Blueprints/Characters/HumanBP.ControllerRef` _array_element))
    (`/Engine/EditorBlueprintResources/StandardMacros.IsValid` _controllerref
      (:`Is Valid`
        (`/Game/Blueprints/Characters/HumanBP.MulticastSetPlayerColor` _array_element (`/Game/Blueprints/Controllers/PlayerController_Game.PlayerColor` _controllerref))
        (`/Game/Blueprints/Characters/HumanBP.ClientSetPlayerColor` _array_element (make `LinearColor` 1.0 1.0 1.0 1.0)))))
  (`self.MacSpawnItem` 18 _fortress "NewEnumerator2")
  (`self.MacSpawnItem` 16 _fortress "NewEnumerator1"))

(fn `PlayerFortress`
  (params (Place :type Integer) (Player :type "/Game/Blueprints/Controllers/PlayerController_Game Object Reference") (Color :type "LinearColor Structure"))
  (returns (Fortress :type "/Game/Assets/BP_Meshes/Architecture/BP_Fortress Object Reference") (Border :type "Array of /Game/Blueprints/Structures/Object/StructBox Structure"))
  (locals (OutRef :type "/Game/Assets/BP_Meshes/Architecture/BP_Fortress Object Reference") (OutCastle :type "Vector Structure") (OutBorder :type "Array of /Game/Blueprints/Structures/Object/StructBox Structure") (OutVertices :type "Array of Vector Structure") (OutWarrior :type "Vector Structure") (OutArcher :type "Vector Structure"))
  (bind _hilltopvertices (`self.HilltopVertices`))
  (bind _lowlandvertices (`self.LowlandVertices`))
  (bind _hilltop (`self.Hilltop`))
  (bind _lowland (`self.Lowland`))
  (switch `int` Place
    (:`0`
      (set `local.OutRef` _hilltop)
      (`self.SetOwner` _hilltop Player)
      (bind _returnvalue (`self.SpawnBorder` _hilltopvertices Color))
      (set `local.OutBorder` (`|MakeArray` (make `/Game/Blueprints/Structures/Object/StructBox` _hilltopvertices _returnvalue _hilltop)))
      (set `local.OutCastle` (14542.706055 -25247.171875 -510.001007))
      (set `local.OutVertices` (`|MakeArray` (-5457.293945 -45247.171875 0.0) (34542.707031 -45247.171875 0.0) (34542.707031 -5247.171875 0.0) (-5457.293945 -5247.171875 0.0) :!type "Vector Structure"))
      (set `local.OutWarrior` (13945.0 -21935.0 132.0))
      (set `local.OutArcher` (13945.0 -21735.0 132.0)))
    (:`1`
      (set `local.OutRef` _lowland)
      (`self.SetOwner` _lowland Player)
      (bind _returnvalue_2 (`self.SpawnBorder` _lowlandvertices Color))
      (set `local.OutBorder` (`|MakeArray` (make `/Game/Blueprints/Structures/Object/StructBox` _lowlandvertices _returnvalue_2 _lowland)))
      (set `local.OutCastle` (-19558.716797 20465.865234 -510.0))
      (set `local.OutVertices` (`|MakeArray` (-39558.71875 465.86499 0.0) (441.28299 465.86499 0.0) (441.28299 40465.867188 0.0) (-39558.71875 40465.867188 0.0) :!type "Vector Structure"))
      (set `local.OutWarrior` (13245.0 -21935.0 132.0))
      (set `local.OutArcher` (13245.0 -21735.0 132.0)))
    (:`2`
      _)
    (:`3`
      _)
    (:`4`
      _)
    (:`5`
      _))
  (return (`local.OutRef`) (`local.OutBorder`)))

(fn `UserConstructionScript`
  (`parent.UserConstructionScript`))