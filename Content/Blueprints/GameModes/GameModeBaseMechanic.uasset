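; Game mode base that sets up the map and players for a two-fortress match.
; InitializeServer stores player starts and arrow references, then spawns the Hilltop and Lowland fortresses.
; CreateNewPlayerMechanic spawns and possesses a HumanPlayer with a multicast random body, assigns the fortress for its slot and refreshes all player colors.
; A macro garrisons that fortress with an AI soldier in a free military placement; only the first two slots map to fortresses.
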(event `InitializeServer`
  (params (PlStart :type "Array of PlayerStart Object Reference") (SpawnArrow :type "StaticMeshActor Object Reference") (SpawnDestin :type "StaticMeshActor Object Reference"))
  ;[1 1 0] Initialize server
  (set `self.PlayerStarts` PlStart)
  (`self.MacSpawnMapObjects`)
  (set `self.SpawnArrow` SpawnArrow)
  (set `self.SpawnDestin` SpawnDestin))

(fn `CreateNewPlayerMechanic`
  (params (Player :type "/Game/Blueprints/Controllers/PlayerControllerMechanic Object Reference") (Place :type Integer))
  (locals (Body :type "/Game/Blueprints/Structures/Game/StructBody Structure"))
  (bind _output (`|GetArrayItem` (`self.PlayerStarts`) Place))
  (bind _returnvalue (`|SpawnActorFromClass` "/Game/Blueprints/Characters/HumanPlayer.HumanPlayer_C" (`KismetMathLibrary.MakeTransform` (`self.K2_GetActorLocation` _output) (`self.K2_GetActorRotation` _output)) "Undefined" "OverrideRootScale" null null))
  (set `/Game/Blueprints/Controllers/PlayerController_Game.Index` Place Player)
  (`Controller.Possess` Player _returnvalue)
  (set `/Game/Blueprints/Controllers/PlayerController_Game.CharacterRef` _returnvalue Player)
  (set `/Game/Blueprints/Characters/HumanBP.ControllerRef` Player _returnvalue)
  (bind _output_get (set `local.Body` (`/Game/Blueprints/Libraries/LibHuman.RandomBody`)))
  (`/Game/Blueprints/Characters/HumanBP.MulticastSetOrgans` _returnvalue _output_get)
  (`/Game/Blueprints/Characters/HumanBP.SetOrgans` _returnvalue _output_get)
  (bind _fortress (`self.PlayerFortress` Place Player))
  (if (!= _fortress null)
    (`KismetArrayLibrary.Array_Add` (`/Game/Blueprints/Controllers/PlayerController_Game.Buildings` Player))
    (set `/Game/Assets/BP_Meshes/Architecture/BP_House.Player` Player _fortress)
    (`self.MacSpawnSoldier` _fortress "NewEnumerator1"))
  (set `/Game/Blueprints/Controllers/PlayerController_Game.ArrowSpawn` (`self.SpawnArrow`) Player)
  (set `/Game/Blueprints/Controllers/PlayerController_Game.ArrowDestin` (`self.SpawnDestin`) Player)
  (bind _outactors (`GameplayStatics.GetAllActorsOfClass` "/Game/Blueprints/Characters/HumanPlayer.HumanPlayer_C"))
  (for _array_element _outactors
    (bind _controllerref (`/Game/Blueprints/Characters/HumanBP.ControllerRef` _array_element))
    (`/Engine/EditorBlueprintResources/StandardMacros.IsValid` _controllerref
      (:`Is Valid`
        (`/Game/Blueprints/Characters/HumanBP.SetPlayerColorForEveryone` _array_element (`/Game/Blueprints/Controllers/PlayerController_Game.PlayerColor` _controllerref))))))

(fn `PlayerFortress`
  (params (Place :type Integer) (Player :type "/Game/Blueprints/Controllers/PlayerController_Game Object Reference"))
  (returns (Fortress :type "/Game/Assets/BP_Meshes/Architecture/BP_House Object Reference"))
  (locals (OutRef :type "/Game/Assets/BP_Meshes/Architecture/BP_House Object Reference"))
  (switch `int` Place
    (:`0`
      (bind _output_get (set `local.OutRef` (`self.Hilltop`)))
      (`self.SetOwner` _output_get Player))
    (:`1`
      (bind _output_get_2 (set `local.OutRef` (`self.Lowland`)))
      (`self.SetOwner` _output_get_2 Player))
    (:`2`
      _)
    (:`3`
      _)
    (:`4`
      _)
    (:`5`
      _))
  (return (`local.OutRef`)))

(fn `UserConstructionScript`
  (`parent.UserConstructionScript`))