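; Character helper function library for movement vectors, facing and turn direction, distance-band checks, target validation and ranged aiming.
; Facing checks compare the capsule's direction to the target with a 2D angle, using the cross product's Z sign for turn direction.
; Hit collider names map to arrow attachment sockets.
; RangeVelocity line-traces to hip, then head (which returns no component), and solves a ballistic quadratic, placing the root in the returned vector's Z.
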(fn `CharacterNeedMove`
  (params (TargetLocation :type "Vector Structure") (CharacterLocation :type "Vector Structure") (MinDistance :type "Float (double-precision)") (MaxDistance :type "Float (double-precision)"))
  (returns (ReturnValue :type Boolean) (Direction :type "Vector Structure"))
  (bind _returnvalue (`/Game/Blueprints/Libraries/LibMath.VectorLenghth2D` TargetLocation CharacterLocation))
  (return (or (< _returnvalue MinDistance) (> _returnvalue MaxDistance)) (- TargetLocation CharacterLocation)))

(fn `CharacterNeedRotation`
  (params (Character :type "Character Object Reference") (TargetLocation :type "Vector Structure") (AcceptableAngle :type "Float (double-precision)"))
  (returns (ReturnValue :type Boolean) (VectorA :type "Vector Structure") (VectorB :type "Vector Structure"))
  (bind _returnvalue (- TargetLocation (`Actor.K2_GetActorLocation` Character)))
  (bind _direction (`/Game/Blueprints/Libraries/LibMath.GetDirectionFromSceneComponent` (`Character.CapsuleComponent` Character)))
  (return (> (`/Game/Blueprints/Libraries/LibMath.AngleBetweenVectors2D` _returnvalue _direction) AcceptableAngle) _returnvalue _direction))

(fn `GetMovementVector`
  (params (InputRotator :type "Rotator Structure") (Direction :type String) (MovementMode :type "EMovementMode Enum" :default "MOVE_None"))
  (returns (ReturnValue :type "Vector Structure"))
  (locals (OutVector :type "Vector Structure"))
  (switch `string` Direction
    (:`Forward`
      (if (`|EnumEquality` MovementMode "MOVE_Flying")
        (set `local.OutVector` (`KismetMathLibrary.GetUpVector` InputRotator))
        (else
          (set `local.OutVector` (`KismetMathLibrary.GetForwardVector` InputRotator)))))
    (:`Right`
      (set `local.OutVector` (`KismetMathLibrary.GetRightVector` InputRotator))))
  (return (`local.OutVector`)))

(fn `IsLookingAtPoint`
  (params (Character :type "Character Object Reference") (TargetLocation :type "Vector Structure") (AcceptableAngle :type "Float (double-precision)"))
  (returns (Yes :type Boolean) (ClockWise :type "Float (double-precision)"))
  (locals (Clock :type "Float (double-precision)"))
  (bind _returnvalue (- TargetLocation (`Actor.K2_GetActorLocation` Character)))
  (bind _direction (`/Game/Blueprints/Libraries/LibMath.GetDirectionFromSceneComponent` (`Character.CapsuleComponent` Character)))
  (if (> (.z (`KismetMathLibrary.Cross_VectorVector` _returnvalue _direction)) 0.0)
    (set `local.Clock` -1.0)
    (else
      (set `local.Clock` 1.0)))
  (return (<= (`/Game/Blueprints/Libraries/LibMath.AngleBetweenVectors2D` _returnvalue _direction) AcceptableAngle) (`local.Clock`)))

(fn `MakeRotatorByZ`
  (params (InputRotator :type "Rotator Structure"))
  (returns (ReturnValue :type "Rotator Structure"))
  (return (`KismetMathLibrary.MakeRotator` 0.0 0.0 (.yaw InputRotator))))

(fn `RangeVelocity`
  (params (Start :type "Vector Structure") (TargetCharacter :type "/Game/Blueprints/Characters/HumanBP Object Reference") (PowerForce :type "Float (double-precision)"))
  (returns (RaycastOkay :type Boolean) (Velocity :type "Vector Structure"))
  (locals (OutBool :type Boolean) (Height :type "Float (double-precision)") (Destination :type "Float (double-precision)") (Range :type "Float (double-precision)") (GravityScale :type "Float (double-precision)") (Speed :type "Float (double-precision)"))
  (bind (_selected _component) (`self.SelectBodyPart` Start TargetCharacter))
  (bind (_height _destination _range) (`/Game/Blueprints/Libraries/LibProjectile.HeightAndDestination` Start (`SceneComponent.K2_GetComponentLocation` _component)))
  (if _selected
    (set `local.OutBool` true)
    (set `local.Height` _height)
    (set `local.Destination` _destination)
    (set `local.Range` _range)
    (set `local.Speed` (* PowerForce 100.0))
    (bind (_a _b _c) (`/Game/Blueprints/Libraries/LibProjectile.CreateQuadraticEquationFactors` (`local.Height`) (`local.Destination`) (`local.GravityScale`) (`local.Speed`)))
    (bind (_hasvalue _x1 _x2) (`/Game/Blueprints/Libraries/LibMath.QuadraticEquation` _a _b _c))
    (if (not _hasvalue)
      (`KismetSystemLibrary.PrintString` null "No Value" true true (struct :`R` 1.0 :`A` 1.0) 6.0 :!label _label))
    (else
      (goto _label)))
  (return (`local.OutBool`) (`KismetMathLibrary.MakeVector` 0.0 1.0 _x2)))

(fn `RaycastOkay`
  (params (Start :type "Vector Structure") (End :type "Vector Structure") (TargetCharacter :type "/Game/Blueprints/Characters/HumanBP Object Reference"))
  (returns (ReturnValue :type Boolean))
  (locals (OutBool :type Boolean))
  (bind (_outhit _returnvalue) (`KismetSystemLibrary.LineTraceSingleForObjects` :`Start` Start :`End` End :`ObjectTypes` (`|MakeArray` "ObjectTypeQuery1" "ObjectTypeQuery3" :!type "EObjectTypeQuery Enum") :`DrawDebugType` "ForDuration" :`DrawTime` 2.0))
  (if _returnvalue
    (if (== (`.HitActor` (`GameplayStatics.BreakHitResult` _outhit)) TargetCharacter)
      (set `local.OutBool` true)))
  (return (`local.OutBool`)))

(fn `SelectBodyPart`
  (params (Start :type "Vector Structure") (TargetCharacter :type "/Game/Blueprints/Characters/HumanBP Object Reference"))
  (returns (Selected :type Boolean) (Component :type "PrimitiveComponent Object Reference"))
  (locals (OutBool :type Boolean) (OutComponent :type "PrimitiveComponent Object Reference"))
  (bind _hipcoll (`/Game/Blueprints/Characters/HumanBP.HipColl` TargetCharacter))
  (if (`self.RaycastOkay` Start (`SceneComponent.K2_GetComponentLocation` _hipcoll) TargetCharacter)
    (set `local.OutBool` true)
    (set `local.OutComponent` _hipcoll)
    (elif (`self.RaycastOkay` Start (`SceneComponent.K2_GetComponentLocation` (`/Game/Blueprints/Characters/HumanBP.HeadColl` TargetCharacter)) TargetCharacter)
      (set `local.OutBool` true)
      (set `local.OutComponent` null)))
  (return (`local.OutBool`) (`local.OutComponent`)))

(fn `SetClockwise`
  (params (VectorA :type "Vector Structure") (VectorB :type "Vector Structure"))
  (returns (ReturnValue :type "Float (double-precision)"))
  (locals (OutFloat :type "Float (double-precision)"))
  (if (> (.z (`KismetMathLibrary.Cross_VectorVector` VectorA VectorB)) 0.0)
    (set `local.OutFloat` -1.0)
    (else
      (set `local.OutFloat` 1.0)))
  (return (`local.OutFloat`)))

(fn `SetRotationValue`
  (params (Character :type "Character Object Reference") (TargetLocation :type "Vector Structure") (AcceptableAngle :type "Float (double-precision)"))
  (returns (ReturnValue :type "Float (double-precision)"))
  (locals (OutFloat :type "Float (double-precision)"))
  (bind (_returnvalue _vectora _vectorb) (`self.CharacterNeedRotation` Character TargetLocation AcceptableAngle))
  (if _returnvalue
    (if (> (.z (`KismetMathLibrary.Cross_VectorVector` _vectora _vectorb)) 0.0)
      (set `local.OutFloat` -1.0)
      (else
        (set `local.OutFloat` 1.0))))
  (return (`local.OutFloat`)))

(fn `SocketByOverlappedComponent`
  (params (Component :type "PrimitiveComponent Object Reference"))
  (returns (CanAttach :type Boolean) (SocketName :type Name))
  (locals (OutSocket :type Name) (OutBool :type Boolean))
  (switch `string` (`KismetSystemLibrary.GetObjectName` Component)
    (:`SwordColl`
      (set `local.OutBool` false)
      (set `local.OutSocket` "None"))
    (:`ShieldColl`
      (set `local.OutBool` false)
      (set `local.OutSocket` "None"))
    (:`LeftArmColl`
      (set `local.OutBool` true)
      (set `local.OutSocket` "ArrowLeftArm"))
    (:`LeftHandColl`
      (set `local.OutBool` false)
      (set `local.OutSocket` "None"))
    (:`RightArmColl`
      (set `local.OutBool` true)
      (set `local.OutSocket` "ArrowArmRight"))
    (:`RightHandColl`
      (set `local.OutBool` true)
      (set `local.OutSocket` "ArrowHandRight"))
    (:`LeftLegColl`
      (set `local.OutBool` true)
      (set `local.OutSocket` "ArrowFootLeft"))
    (:`RightLegColl`
      (set `local.OutBool` true)
      (set `local.OutSocket` "ArrowFootRight"))
    (:`HipColl`
      (set `local.OutBool` true)
      (set `local.OutSocket` "ArrowHip"))
    (:`HeadColl`
      (set `local.OutBool` true)
      (set `local.OutSocket` "ArrowHead")))
  (return (`local.OutBool`) (`local.OutSocket`)))

(fn `TargetCharacterValidation`
  (params (Character :type "/Game/Blueprints/Characters/HumanBP Object Reference"))
  (returns (ReturnValue :type Boolean))
  (locals (OutBool :type Boolean))
  (`/Engine/EditorBlueprintResources/StandardMacros.IsValid` Character
    (:`Is Valid`
      (set `local.OutBool` (not (`/Game/Blueprints/Characters/HumanBP.IsDead` Character))))
    (:`Is Not Valid`
      _))
  (return (`local.OutBool`)))