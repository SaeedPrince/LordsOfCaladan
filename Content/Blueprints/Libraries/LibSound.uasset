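; LibSound is a Blueprint function library of helpers for movement sounds.
; SoundByMovement picks a walk or run cue by person type, Civilian or Soldier, through nested switches, assigning none for No Move.
; PlayRateByMoveSpeed appears unfinished: it derives a rate from move speed against walk speed, but RunSpeed is unused, faster speeds are unhandled and its return node is never reached.
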(fn `PlayRateByMoveSpeed`
  (params (MoveSpeed :type "Float (double-precision)") (WalkSpeed :type "Float (double-precision)") (RunSpeed :type "Float (double-precision)"))
  (returns (ReturnValue :type "Float (double-precision)"))
  (locals (OutRate :type "Float (double-precision)"))
  (if (< MoveSpeed WalkSpeed)
    (set `local.OutRate` 1.0)
    (elif (== MoveSpeed WalkSpeed)
      (set `local.OutRate` (/ MoveSpeed WalkSpeed)))))

(fn `SoundByMovement`
  (params (PersonType :type "/Game/Blueprints/Enums/EnumPersonType Enum" :default "NewEnumerator0") (MovementType :type "/Game/Blueprints/Enums/EnumMovementType Enum" :default "NewEnumerator0"))
  (returns (RetuenValue :type "SoundCue Object Reference"))
  (locals (OutCue :type "SoundCue Object Reference"))
  (switch `/Game/Blueprints/Enums/EnumPersonType` PersonType
    (:`NewEnumerator0`
      (switch `/Game/Blueprints/Enums/EnumMovementType` MovementType
        (:`NewEnumerator0`
          _)
        (:`NewEnumerator1`
          (set `local.OutCue` "/Game/Assets/Audio/SFX/Civilian/Cues/Civil_Walk.Civil_Walk"))
        (:`NewEnumerator2`
          (set `local.OutCue` "/Game/Assets/Audio/SFX/Civilian/Cues/Civil_Run.Civil_Run"))))
    (:`NewEnumerator1`
      (switch `/Game/Blueprints/Enums/EnumMovementType` MovementType
        (:`NewEnumerator0`
          _)
        (:`NewEnumerator1`
          (set `local.OutCue` "/Game/Assets/Audio/SFX/Soldier/Cues/Soldier_Walk.Soldier_Walk"))
        (:`NewEnumerator2`
          (set `local.OutCue` "/Game/Assets/Audio/SFX/Soldier/Cues/Soldier_Run_Fast.Soldier_Run_Fast")))))
  (return (`local.OutCue`)))