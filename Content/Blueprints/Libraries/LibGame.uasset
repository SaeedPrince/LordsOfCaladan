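; LibGame is a library of small, unrelated gameplay helpers.
; It creates player-owned widgets with their controller reference set, and returns the highest true index in a bool array.
; It also searches person arrays by residence or worker index, chosen by the array name, and maps mined products (ores, coal, sulfur) to their mine flag meshes.
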(fn `BoolMax`
  (params (BoolArray :type "Array of Boolean"))
  (returns (ReturnValue :type Integer))
  (locals (OutMax :type Integer :default -1))
  (for (_array_element _array_index) BoolArray
    (if _array_element
      (set `local.OutMax` _array_index)))
  (return (`local.OutMax`)))

(fn `CreateGameWidget`
  (params (Class :type "/Game/Blueprints/Widgets/Widget_ParentGame Class Reference") (Player :type "/Game/Blueprints/Controllers/PlayerController_Game Object Reference"))
  (returns (ReturnValue :type "/Game/Blueprints/Widgets/Widget_ParentGame Object Reference"))
  (bind _returnvalue (`|CreateWidget` Class Player))
  (set `/Game/Blueprints/Widgets/Widget_ParentGame.ControllerRef` Player _returnvalue)
  (return _returnvalue))

(fn `FindPersonInPersonArray`
  (params (Index :type Integer) (PersonArray :type "Array of /Game/Blueprints/Controllers/AIController_Game Object Reference") (ArrayName :type String))
  (returns (Found :type Boolean) (Person :type "/Game/Blueprints/Controllers/AIController_Game Object Reference"))
  (locals (OutBool :type Boolean) (OutIndex :type "/Game/Blueprints/Controllers/AIController_Game Object Reference"))
  (for _array_element PersonArray
    (switch `string` ArrayName
      (:`Residence`
        (if (== (`/Game/Blueprints/Libraries/LibAIController.GetIndexInResidenceByType` _array_element) Index)
          (set `local.OutBool` true :!label _label)
          (set `local.OutIndex` _array_element)
          (break)))
      (:`Work`
        (if (== Index (`/Game/Blueprints/Controllers/AIController_Game.IndexInWorker` _array_element))
          (goto _label)))))
  (return (`local.OutBool`) (`local.OutIndex`)))

(fn `FlagMesh`
  (params (ProductID :type "/Game/Blueprints/Enums/EnumItem Enum" :default "NewEnumerator0"))
  (returns (ReturnValue :type "SkeletalMesh Object Reference"))
  (locals (OutMesh :type "SkeletalMesh Object Reference"))
  (switch `/Game/Blueprints/Enums/EnumItem` ProductID
    (:`NewEnumerator19`
      (set `local.OutMesh` "/Game/Assets/SkeletalMeshes/A_Flag_IronMine.A_Flag_IronMine"))
    (:`NewEnumerator34`
      (set `local.OutMesh` "/Game/Assets/SkeletalMeshes/A_Flag_GoldMine.A_Flag_GoldMine"))
    (:`NewEnumerator35`
      (set `local.OutMesh` "/Game/Assets/SkeletalMeshes/A_Flag_CopperMine.A_Flag_CopperMine"))
    (:`NewEnumerator20`
      (set `local.OutMesh` "/Game/Assets/SkeletalMeshes/A_Flag_CoalMine.A_Flag_CoalMine"))
    (:`NewEnumerator21`
      (set `local.OutMesh` "/Game/Assets/SkeletalMeshes/A_Flag_SulfurMine.A_Flag_SulfurMine")))
  (return (`local.OutMesh`)))