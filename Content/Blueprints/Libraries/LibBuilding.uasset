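; Blueprint function library of query helpers for buildings: items, stack storage, civilian and military slots, and closest-building lookup.
; A hard-coded item-index map to weapon, material and food categories feeds per-category inventory counts for a widget struct.
; Military placement picks a random free slot on the least occupied flag, assuming six slots per flag.
; Ladder end offsets are hard-coded per building and ladder index; GetItemArrayIndexFromBuilding is an empty stub.
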(fn `BuildingDestinationToLocation`
  (params (Location :type "Vector Structure") (Building :type "/Game/Assets/BP_Meshes/Architecture/BP_House Object Reference"))
  (returns (Destination :type "Float (double-precision)"))
  (return (`KismetMathLibrary.VSize` (- Location (`SceneComponent.K2_GetComponentLocation` (`/Game/Assets/BP_Meshes/Architecture/BP_House.ItemPlace` Building))))))

(fn `BuildingInventory`
  (params (BuildingRef :type "/Game/Assets/BP_Meshes/Architecture/BP_House Object Reference"))
  (returns (ReturnValue :type "/Game/Blueprints/Structures/Game/StructWidgetInventory Structure"))
  (locals (NumWeapon :type "Array of Integer") (NumMaterial :type "Array of Integer") (NumFood :type "Array of Integer") (BoolWeapon :type Boolean) (BoolMatreial :type Boolean) (BoolFood :type Boolean))
  (for _array_element (`/Game/Assets/BP_Meshes/Architecture/BP_House.AvailableItems` BuildingRef)
    (bind (_weapon _material _food) (`self.ItemIndexInCategory` (`/Game/Assets/BP_Meshes/Item/BP_Item.Index` _array_element)))
    (if (!= _weapon -1)
      (`/Engine/EditorBlueprintResources/StandardMacros.IncrementInt` (`|GetArrayItem` (`local.NumWeapon`) _weapon)
        (:`  `
          (set `local.BoolWeapon` true)))
      (elif (!= _material -1)
        (`/Engine/EditorBlueprintResources/StandardMacros.IncrementInt` (`|GetArrayItem` (`local.NumMaterial`) _material)
          (:`  `
            (set `local.BoolMatreial` true)))
        (elif (!= _food -1)
          (`/Engine/EditorBlueprintResources/StandardMacros.IncrementInt` (`|GetArrayItem` (`local.NumFood`) _food)
            (:`  `
              (set `local.BoolFood` true)))
          (else
            (`KismetSystemLibrary.PrintString` null "Error in building inventory" true true (struct :`R` 1.0 :`A` 1.0) 10.0))))))
  (return (make `/Game/Blueprints/Structures/Game/StructWidgetInventory` (`local.BoolWeapon`) (`local.BoolMatreial`) (`local.BoolFood`) (`local.NumWeapon`) (`local.NumMaterial`) (`local.NumFood`))))

(fn `FlagOccupiedCount`
  (params (FlagNumber :type Integer) (Building :type "/Game/Assets/BP_Meshes/Architecture/BP_House Object Reference"))
  (returns (ReturnValue :type Integer))
  (locals (OutInteger :type Integer))
  (bind _returnvalue (`self.OccupiedArrayByFlagNumber` FlagNumber Building))
  (for _array_element _returnvalue
    (if _array_element
      (set `local.OutInteger` (+ (`local.OutInteger`) 1))))
  (return (`local.OutInteger`)))

(fn `FreeIndexes`
  (params (IndexArray :type "Array of Integer") (Building :type "/Game/Assets/BP_Meshes/Architecture/BP_House Object Reference"))
  (returns (ReturnValue :type "Array of Integer"))
  (locals (OutInt :type "Array of Integer"))
  (for _array_element IndexArray
    (if (not (`|GetArrayItem` (`/Game/Assets/BP_Meshes/Architecture/BP_House.MilitOccupied` Building) _array_element))
      (`KismetArrayLibrary.Array_Add` (`local.OutInt`) _array_element)))
  (return (`local.OutInt`)))

(fn `GetBorderMakerArray`
  (params (BuildingArray :type "Array of /Game/Assets/BP_Meshes/Architecture/BP_House Object Reference"))
  (returns (ReturnValue :type "Array of /Game/Assets/BP_Meshes/Architecture/BP_House Object Reference"))
  (locals (OutArray :type "Array of /Game/Assets/BP_Meshes/Architecture/BP_House Object Reference"))
  (for _array_element BuildingArray
    (if (`/Game/Assets/BP_Meshes/Architecture/BP_House.IsBorderMaker` _array_element)
      (`KismetArrayLibrary.Array_Add` (`local.OutArray`) _array_element)))
  (return (`local.OutArray`)))

(fn `GetBuildingsWithFreeMilitPlace`
  (params (BuildingArray :type "Array of /Game/Assets/BP_Meshes/Architecture/BP_House Object Reference"))
  (returns (ReturnValue :type "Array of /Game/Assets/BP_Meshes/Architecture/BP_House Object Reference"))
  (locals (OutArray :type "Array of /Game/Assets/BP_Meshes/Architecture/BP_House Object Reference"))
  (for _array_element BuildingArray
    (bind _found (`self.GetFreeMilitPlaceNew` _array_element))
    (if _found
      (`KismetArrayLibrary.Array_Add` (`local.OutArray`) _array_element)))
  (return (`local.OutArray`)))

(fn `GetBuildingWithMaxItem`
  (params (ItemIndexArray :type "Array of Integer") (BuildingArray :type "Array of /Game/Assets/BP_Meshes/Architecture/BP_House Object Reference"))
  (returns (ReturnValue :type "/Game/Assets/BP_Meshes/Architecture/BP_House Object Reference") (ItemArray :type "Array of /Game/Assets/BP_Meshes/Item/BP_Item Object Reference"))
  (locals (OutBuilding :type "/Game/Assets/BP_Meshes/Architecture/BP_House Object Reference") (MaxCount :type Integer) (OutItem :type "Array of /Game/Assets/BP_Meshes/Item/BP_Item Object Reference"))
  (for _array_element BuildingArray
    (bind _returnvalue (`self.ItemCountInBuilding` (`|GetArrayItem` ItemIndexArray) _array_element))
    (if (> _returnvalue (`local.MaxCount`))
      (set `local.MaxCount` _returnvalue)
      (set `local.OutBuilding` _array_element)))
  (for _array_element_2 ItemIndexArray
    (`KismetArrayLibrary.Array_Add` (`local.OutItem`) (`/Game/Blueprints/Libraries/LibItem.GetItemFromItemArray` _array_element_2 (`/Game/Assets/BP_Meshes/Architecture/BP_House.AvailableItems` (`local.OutBuilding`)))))
  (return (`local.OutBuilding`) (`local.OutItem`)))

(fn `GetClosestBuildingToLocation`
  (params (Location :type "Vector Structure") (BuildingArray :type "Array of /Game/Assets/BP_Meshes/Architecture/BP_House Object Reference"))
  (returns (ReturnValue :type "/Game/Assets/BP_Meshes/Architecture/BP_House Object Reference"))
  (locals (OutBuilding :type "/Game/Assets/BP_Meshes/Architecture/BP_House Object Reference") (Destin :type "Float (double-precision)" :default 0.0))
  (bind _returnvalue (`KismetArrayLibrary.Array_Length` BuildingArray))
  (bind _output (`|GetArrayItem` BuildingArray))
  (if (> _returnvalue 0)
    (set `local.OutBuilding` _output)
    (set `local.Destin` (`self.BuildingDestinationToLocation` Location _output))
    (for _index (range 1 _returnvalue)
      (bind _output_2 (`|GetArrayItem` BuildingArray _index))
      (bind _destination (`self.BuildingDestinationToLocation` Location _output_2))
      (if (< _destination (`local.Destin`))
        (set `local.OutBuilding` _output_2)
        (set `local.Destin` _destination)))
    (return (`local.OutBuilding`))))

(fn `GetFreeCivilPlace`
  (params (Building :type "/Game/Assets/BP_Meshes/Architecture/BP_House Object Reference") (MaxIndex :type Integer))
  (returns (Found :type Boolean) (Index :type Integer))
  (locals (OutBool :type Boolean) (OutIndex :type Integer))
  (for _index (range MaxIndex)
    (if (not (`|GetArrayItem` (`/Game/Assets/BP_Meshes/Architecture/BP_House.CivilOccupied` Building) _index))
      (set `local.OutIndex` _index)
      (set `local.OutBool` true)
      (break)))
  (return (`local.OutBool`) (`local.OutIndex`)))

(fn `GetFreeMilitPlace`
  (params (Building :type "/Game/Assets/BP_Meshes/Architecture/BP_House Object Reference"))
  (returns (Found :type Boolean) (Index :type Integer))
  (locals (OutBool :type Boolean) (OutIndex :type Integer))
  (for _index (range (`/Game/Assets/BP_Meshes/Architecture/BP_House.MaxMilitPop` Building))
    (if (not (`|GetArrayItem` (`/Game/Assets/BP_Meshes/Architecture/BP_House.MilitOccupied` Building) _index))
      (set `local.OutIndex` _index)
      (set `local.OutBool` true)
      (break)))
  (return (`local.OutBool`) (`local.OutIndex`)))

(fn `GetFreeMilitPlaceNew`
  (params (Building :type "/Game/Assets/BP_Meshes/Architecture/BP_House Object Reference"))
  (returns (Found :type Boolean) (Index :type Integer))
  (bind _returnvalue (`self.GetLeastOccupiedFlagNumber` Building))
  (bind _returnvalue_2 (`self.IndexArrayByFlagNumber` _returnvalue Building))
  (bind _returnvalue_3 (`self.FreeIndexes` _returnvalue_2 Building))
  (return (> (`KismetArrayLibrary.Array_Length` _returnvalue_3) 0) (`/Game/Blueprints/Libraries/LibMath.RandomIntegerFromOneArray` _returnvalue_3)))

(fn `GetItemArrayIndexFromBuilding`
  (params (Building :type "/Game/Assets/BP_Meshes/Architecture/BP_House Object Reference") (ItemIndexArray :type "Array of Integer"))
  (returns (ReturnValue :type "Array of /Game/Assets/BP_Meshes/Item/BP_Item Object Reference"))
  (return))

(fn `GetLeastOccupiedFlagNumber`
  (params (Building :type "/Game/Assets/BP_Meshes/Architecture/BP_House Object Reference"))
  (returns (ReturnValue :type Integer))
  (locals (OutFlag :type Integer) (OccupiedCount :type Integer))
  (bind _returnvalue (`self.FlagOccupiedCount` 0 Building))
  (set `local.OccupiedCount` _returnvalue)
  (for _index (range 1 (`/Game/Assets/BP_Meshes/Architecture/BP_House.FlagCount` Building))
    (bind _returnvalue_2 (`self.FlagOccupiedCount` _index Building))
    (if (< _returnvalue_2 (`local.OccupiedCount`))
      (set `local.OccupiedCount` _returnvalue_2)
      (set `local.OutFlag` _index)))
  (return (`local.OutFlag`)))

(fn `GetStackArray`
  (params (BuildingArray :type "Array of /Game/Assets/BP_Meshes/Architecture/BP_House Object Reference"))
  (returns (ReturnValue :type "Array of /Game/Assets/BP_Meshes/Architecture/BP_House Object Reference"))
  (locals (OutArray :type "Array of /Game/Assets/BP_Meshes/Architecture/BP_House Object Reference"))
  (for _array_element BuildingArray
    (if (`/Game/Assets/BP_Meshes/Architecture/BP_House.IsStack` _array_element)
      (`KismetArrayLibrary.Array_Add` (`local.OutArray`) _array_element)))
  (return (`local.OutArray`)))

(fn `IndexArrayByFlagNumber`
  (params (FlagNumber :type Integer) (Building :type "/Game/Assets/BP_Meshes/Architecture/BP_House Object Reference"))
  (returns (ReturnValue :type "Array of Integer"))
  (locals (OutArray :type "Array of Integer"))
  (for _index (range 6)
    (`KismetArrayLibrary.Array_Add` (`local.OutArray`) (+ _index (* FlagNumber (`/Game/Assets/BP_Meshes/Architecture/BP_House.MilitPlacePerFlag` Building)))))
  (return (`local.OutArray`)))

(fn `ItemAvailableInStack`
  (params (ItemIndex :type Integer) (BuildingArray :type "Array of /Game/Assets/BP_Meshes/Architecture/BP_House Object Reference"))
  (returns (ReturnValue :type Boolean))
  (locals (OutBool :type Boolean))
  (for _array_element BuildingArray
    (if (`/Game/Assets/BP_Meshes/Architecture/BP_House.IsStack` _array_element)
      (if (`/Game/Blueprints/Libraries/LibItem.ItemIndexExistsInArray` (`/Game/Assets/BP_Meshes/Architecture/BP_House.AvailableItems` _array_element) ItemIndex)
        (set `local.OutBool` true)
        (break))))
  (return (`local.OutBool`)))

(fn `ItemCountInBuilding`
  (params (ItemIndex :type Integer) (Building :type "/Game/Assets/BP_Meshes/Architecture/BP_House Object Reference"))
  (returns (ReturnValue :type Integer))
  (locals (OutInt :type Integer))
  (for _array_element (`/Game/Assets/BP_Meshes/Architecture/BP_House.AvailableItems` Building)
    (if (and (== (`/Game/Assets/BP_Meshes/Item/BP_Item.Index` _array_element) ItemIndex) (not (`/Game/Assets/BP_Meshes/Item/BP_Item.AssignedForConsume` _array_element)) (not (`/Game/Assets/BP_Meshes/Item/BP_Item.AssignedToCarry` _array_element)))
      (set `local.OutInt` (+ (`local.OutInt`) 1))))
  (return (`local.OutInt`)))

(fn `ItemIndexInCategory`
  (params (ItemIndex :type Integer))
  (returns (Weapon :type Integer) (Material :type Integer) (Food :type Integer))
  (locals (OutWeapon :type Integer :default -1) (OutMaterial :type Integer :default -1) (OutFood :type Integer :default -1))
  (switch `int` ItemIndex
    (:`0`
      (set `local.OutMaterial` 0))
    (:`1`
      (set `local.OutMaterial` 1))
    (:`2`
      (set `local.OutMaterial` 2))
    (:`3`
      (set `local.OutFood` 0))
    (:`4`
      (set `local.OutFood` 1))
    (:`5`
      (set `local.OutFood` 2))
    (:`6`
      (set `local.OutFood` 3))
    (:`7`
      (set `local.OutFood` 4))
    (:`8`
      (set `local.OutFood` 5))
    (:`9`
      (set `local.OutFood` 6))
    (:`10`
      (set `local.OutFood` 7))
    (:`11`
      (set `local.OutFood` 8))
    (:`12`
      (set `local.OutWeapon` 0))
    (:`13`
      (set `local.OutWeapon` 1))
    (:`14`
      (set `local.OutWeapon` 2))
    (:`15`
      (set `local.OutWeapon` 3))
    (:`16`
      (set `local.OutWeapon` 4))
    (:`17`
      (set `local.OutWeapon` 5))
    (:`18`
      (set `local.OutWeapon` 6))
    (:`19`
      (set `local.OutMaterial` 3))
    (:`20`
      (set `local.OutMaterial` 4))
    (:`21`
      (set `local.OutMaterial` 5))
    (:`22`
      (set `local.OutMaterial` 6))
    (:`23`
      (set `local.OutMaterial` 7))
    (:`24`
      (set `local.OutMaterial` 8))
    (:`25`
      (set `local.OutWeapon` 7))
    (:`26`
      (set `local.OutWeapon` 8))
    (:`27`
      (set `local.OutWeapon` 9))
    (:`28`
      (set `local.OutMaterial` 9))
    (:`29`
      (set `local.OutMaterial` 10))
    (:`30`
      (set `local.OutMaterial` 11))
    (:`31`
      (set `local.OutMaterial` 12))
    (:`32`
      (set `local.OutMaterial` 13))
    (:`33`
      (set `local.OutWeapon` 10))
    (:`34`
      (set `local.OutMaterial` 14))
    (:`35`
      (set `local.OutWeapon` 11)))
  (return (`local.OutWeapon`) (`local.OutMaterial`) (`local.OutFood`)))

(fn `LadderByIndex`
  (params (BuildingIndex :type Integer) (LadderIndex :type Integer))
  (returns (LadderStart :type "Vector Structure") (LadderEnd :type "Vector Structure"))
  (locals (OutStart :type "Vector Structure") (OutEnd :type "Vector Structure"))
  (switch `int` BuildingIndex
    (:`23`
      (set `local.OutEnd` (0.0 0.0 0.0)))
    (:`24`
      (switch `int` LadderIndex
        (:`0`
          (set `local.OutEnd` (0.0 -110.0 990.0)))
        (:`1`
          (set `local.OutEnd` (0.0 110.0 990.0)))
        (:`2`
          (set `local.OutEnd` (0.0 -110.0 990.0)))
        (:`3`
          (set `local.OutEnd` (0.0 150.0 996.0)))
        (:`4`
          (set `local.OutEnd` (0.0 130.0 1580.0) :!label _label))
        (:`5`
          (set `local.OutEnd` (0.0 -130.0 1580.0) :!label _label_2))
        (:`6`
          (goto _label))
        (:`7`
          (goto _label_2))
        (:`8`
          (set `local.OutEnd` (0.0 130.0 1180.0)))
        (:`9`
          (set `local.OutEnd` (0.0 -140.0 1180.0)))
        (:`10`
          (set `local.OutEnd` (0.0 -120.0 270.0) :!label _label_3))
        (:`11`
          (goto _label_3))
        (:`12`
          (set `local.OutEnd` (0.0 100.0 270.0) :!label _label_4))
        (:`13`
          (goto _label_4))))
    (:`25`
      (set `local.OutEnd` (0.0 0.0 0.0))))
  (return (`local.OutStart`) (`local.OutEnd`)))

(fn `MilitaryFreePlaceAvailable`
  (params (BuildingArray :type "Array of /Game/Assets/BP_Meshes/Architecture/BP_House Object Reference"))
  (returns (ReturnValue :type Boolean))
  (locals (OutBool :type Boolean))
  (bind _outbool (`local.OutBool`))
  (for _array_element BuildingArray
    (if (`/Game/Assets/BP_Meshes/Architecture/BP_House.IsBorderMaker` _array_element)
      (for _index (range (`/Game/Assets/BP_Meshes/Architecture/BP_House.MaxMilitPop` _array_element))
        (if (not (`|GetArrayItem` (`/Game/Assets/BP_Meshes/Architecture/BP_House.MilitOccupied` _array_element) _index))
          (set `local.OutBool` true)
          (break)))
      (if _outbool
        (break))))
  (return _outbool))

(fn `OccupiedArrayByFlagNumber`
  (params (FlagNumber :type Integer) (Building :type "/Game/Assets/BP_Meshes/Architecture/BP_House Object Reference"))
  (returns (ReturnValue :type "Array of Boolean"))
  (locals (OutArray :type "Array of Boolean"))
  (bind _returnvalue (`self.IndexArrayByFlagNumber` FlagNumber Building))
  (for _array_element _returnvalue
    (`KismetArrayLibrary.Array_Add` (`local.OutArray`) (`|GetArrayItem` (`/Game/Assets/BP_Meshes/Architecture/BP_House.MilitOccupied` Building) _array_element)))
  (return (`local.OutArray`)))