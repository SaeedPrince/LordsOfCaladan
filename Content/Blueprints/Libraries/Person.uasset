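; Function library for Person queries covering inventory display and building membership.
; PersonInventory tallies items by index in parallel lists, capped at MaxNumber distinct types, and returns "name:count" texts.
; ItemIndexExistInItemList is its linear-search helper, returning whether an index is listed and where.
; PersonDoesNotBelongToBuilding searches a building's civil residents if residential, or civil workers if productive, flagging false when the person is found.
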(fn `ItemIndexExistInItemList`
  (params (ItemIndex :type Integer) (ItemList :type "Array of Integer"))
  (returns (Exist :type Boolean) (Index :type Integer))
  (locals (OutBool :type Boolean) (OutIndex :type Integer))
  (for (_array_element _array_index) ItemList
    (if (== _array_element ItemIndex)
      (set `local.OutBool` true)
      (set `local.OutIndex` _array_index)
      (break)))
  (return (`local.OutBool`) (`local.OutIndex`)))

(fn `PersonDoesNotBelongToBuilding`
  (params (Person :type "/Game/Blueprints/Controllers/AIController_Game Object Reference") (Building :type "/Game/Assets/BP_Meshes/Architecture/BP_House Object Reference"))
  (returns (ReturnValue :type Boolean))
  (locals (OutBool :type Boolean :default true))
  (if (`/Game/Assets/BP_Meshes/Architecture/BP_House.IsResident` Building)
    (for _array_element (`/Game/Assets/BP_Meshes/Architecture/BP_House.CivilResident` Building)
      (if (== _array_element Person)
        (set `local.OutBool` false)
        (break)))
    (return (`local.OutBool`))
    (elif (`/Game/Assets/BP_Meshes/Architecture/BP_House.IsProductive` Building)
      (for _array_element_2 (`/Game/Assets/BP_Meshes/Architecture/BP_House.CivilWorker` Building)
        (if (== Person _array_element_2)
          (set `local.OutBool` false)
          (break)))
      (return (`local.OutBool`)))))

(fn `PersonInventory`
  (params (Person :type "/Game/Blueprints/Controllers/AIController_Game Object Reference") (MaxNumber :type Integer))
  (returns (ReturnValue :type "Array of Text"))
  (locals (ItemList :type "Array of Integer") (OutText :type "Array of Text") (ItemCount :type "Array of Integer"))
  (bind _itemcount (`local.ItemCount`))
  (bind _itemlist (`local.ItemList`))
  (for _array_element (`/Game/Blueprints/Controllers/AIController_Game.Inventory` Person)
    (bind _index (`/Game/Assets/BP_Meshes/Item/BP_Item.Index` _array_element))
    (bind (_exist _index_2) (`self.ItemIndexExistInItemList` _index (`local.ItemList`)))
    (if _exist
      (`/Engine/EditorBlueprintResources/StandardMacros.IncrementInt` (`|GetArrayItem` _itemcount _index_2))
      (elif (< (`KismetArrayLibrary.Array_Length` _itemlist) MaxNumber)
        (`KismetArrayLibrary.Array_Add` _itemlist _index)
        (`KismetArrayLibrary.Array_Add` _itemcount 1))))
  (for (_array_element_2 _array_index) _itemlist
    (`KismetArrayLibrary.Array_Add` (`local.OutText`) (`KismetTextLibrary.Conv_StringToText` (`KismetStringLibrary.Concat_StrStr` (`/Game/Blueprints/Libraries/Item.ItemNameByIndex` _array_element_2) " : " (`KismetStringLibrary.Conv_IntToString` (`|GetArrayItem` _itemcount _array_index))))))
  (return (`local.OutText`)))