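; Function library that rolls wound effects for a hit, one each for slashing, smashing and piercing damage.
; Weapon base damage (Sword or Short Bow) minus armor modifier is added to per-body-part severity bonuses, selected by the hit component's name.
; GetEffectsByDamage treats these sums as percentage chances, rolling from instant death down to minor wound until one succeeds.
; GetHitEffects ignores its AttackType and AttackDamage inputs.
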(fn `AttackDamageByWeaponType`
  (params (WeaponType :type "/Game/Blueprints/Enums/EnumWeaponType Enum" :default "NewEnumerator0"))
  (returns (SlashingDamage :type "Float (double-precision)") (SmashingDamage :type "Float (double-precision)") (PiercingDamage :type "Float (double-precision)"))
  (locals (OutSlashing :type "Float (double-precision)") (OutSmashing :type "Float (double-precision)") (OutPiercing :type "Float (double-precision)"))
  (switch `/Game/Blueprints/Enums/EnumWeaponType` WeaponType
    (:`NewEnumerator0`
      (set `local.OutSlashing` 40.0)
      (set `local.OutSmashing` 0.0)
      (set `local.OutPiercing` 0.0))
    (:`NewEnumerator1`
      (set `local.OutSlashing` 0.0)
      (set `local.OutSmashing` 0.0)
      (set `local.OutPiercing` 20.0)))
  (return (`local.OutSlashing`) (`local.OutSmashing`) (`local.OutPiercing`)))

(fn `CalculateAttackModifier`
  (params (WeaponType :type "/Game/Blueprints/Enums/EnumWeaponType Enum" :default "NewEnumerator0") (ArmorType :type "/Game/Blueprints/Enums/EnumArmorType Enum" :default "NewEnumerator0"))
  (returns (SlashingDamage :type "Float (double-precision)") (SmashingDamage :type "Float (double-precision)") (PiercingDamage :type "Float (double-precision)"))
  (bind (_slashingdamage _smashingdamage _piercingdamage) (`self.AttackDamageByWeaponType` WeaponType))
  (bind (_slashing _smashing _piercing) (`/Game/Blueprints/Libraries/LibArmor.CalculateArmorModifier` ArmorType))
  (return (- _slashingdamage _slashing) (- _smashingdamage _smashing) (- _piercingdamage _piercing)))

(fn `GetEffectsByDamage`
  (params (InstantDeathDamage :type "Float (double-precision)") (BluredVisionDamage :type "Float (double-precision)") (CriticalWoundDamage :type "Float (double-precision)") (NastyWoundDamage :type "Float (double-precision)") (MajorWoundDamage :type "Float (double-precision)") (MinorWoundDamage :type "Float (double-precision)"))
  (returns (ReturnValue :type "/Game/Blueprints/Enums/EnumHitEffects Enum"))
  (locals (OutEffect :type "/Game/Blueprints/Enums/EnumHitEffects Enum"))
  (if (`self.IsDamageEffective` InstantDeathDamage)
    (set `local.OutEffect` "NewEnumerator0")
    (return (`local.OutEffect`))
    (elif (`self.IsDamageEffective` BluredVisionDamage)
      (set `local.OutEffect` "NewEnumerator2")
      (return (`local.OutEffect`))
      (elif (`self.IsDamageEffective` CriticalWoundDamage)
        (set `local.OutEffect` "NewEnumerator3")
        (return (`local.OutEffect`))
        (elif (`self.IsDamageEffective` NastyWoundDamage)
          (set `local.OutEffect` "NewEnumerator4")
          (return (`local.OutEffect`))
          (elif (`self.IsDamageEffective` MajorWoundDamage)
            (set `local.OutEffect` "NewEnumerator5")
            (return (`local.OutEffect`))
            (elif (`self.IsDamageEffective` MinorWoundDamage)
              (set `local.OutEffect` "NewEnumerator6")
              (return (`local.OutEffect`)))))))))

(fn `GetHitEffects`
  (params (HitComponent :type "PrimitiveComponent Object Reference") (AttackType :type "/Game/Blueprints/Enums/EnumAttackType Enum" :default "NewEnumerator3") (WeaponType :type "/Game/Blueprints/Enums/EnumWeaponType Enum" :default "NewEnumerator0") (ArmorType :type "/Game/Blueprints/Enums/EnumArmorType Enum" :default "NewEnumerator0") (AttackDamage :type "Float (double-precision)"))
  (returns (HitEffect1 :type "/Game/Blueprints/Enums/EnumHitEffects Enum") (HitEffect2 :type "/Game/Blueprints/Enums/EnumHitEffects Enum") (HitEffect3 :type "/Game/Blueprints/Enums/EnumHitEffects Enum"))
  (bind (_instantdeathdamage _bluredvisiondamage _criticalwounddamage _nastywounddamage _majorwounddamage _minorwounddamage) (`self.SmashingDamageModifier` HitComponent null WeaponType ArmorType))
  (bind (_instantdeathdamage_2 _bluredvisiondamage_2 _criticalwounddamage_2 _nastywounddamage_2 _majorwounddamage_2 _minorwounddamage_2) (`self.PiercingDamageModifier` HitComponent null WeaponType ArmorType))
  (bind (_instantdeathdamage_3 _bluredvisiondamage_3 _criticalwounddamage_3 _nastywounddamage_3 _majorwounddamage_3 _minorwounddamage_3) (`self.SlashingDamageModifier` HitComponent WeaponType ArmorType))
  (return (`self.GetEffectsByDamage` _instantdeathdamage_3 _bluredvisiondamage_3 _criticalwounddamage_3 _nastywounddamage_3 _majorwounddamage_3 _minorwounddamage_3) (`self.GetEffectsByDamage` _instantdeathdamage _bluredvisiondamage _criticalwounddamage _nastywounddamage _majorwounddamage _minorwounddamage) (`self.GetEffectsByDamage` _instantdeathdamage_2 _bluredvisiondamage_2 _criticalwounddamage_2 _nastywounddamage_2 _majorwounddamage_2 _minorwounddamage_2)))

(fn `IsDamageEffective`
  (params (Damage :type "Float (double-precision)"))
  (returns (ReturnValue :type Boolean))
  (locals (RandomInt :type Integer))
  (set `local.RandomInt` (`KismetMathLibrary.RandomIntegerInRange` 0 100))
  (return (<= (`KismetMathLibrary.Conv_IntToDouble` (`local.RandomInt`)) Damage)))

(fn `PiercingDamageModifier`
  (params (HitComponent :type "PrimitiveComponent Object Reference") (WeaponType :type "/Game/Blueprints/Enums/EnumWeaponType Enum" :default "NewEnumerator0") (ArmorType :type "/Game/Blueprints/Enums/EnumArmorType Enum" :default "NewEnumerator0"))
  (returns (InstantDeathDamage :type "Float (double-precision)") (BluredVisionDamage :type "Float (double-precision)") (CriticalWoundDamage :type "Float (double-precision)") (NastyWoundDamage :type "Float (double-precision)") (MajorWoundDamage :type "Float (double-precision)") (MinorWoundDamage :type "Float (double-precision)"))
  (locals (OutDeath :type "Float (double-precision)") (OutBlured :type "Float (double-precision)") (OutCritical :type "Float (double-precision)") (OutNasty :type "Float (double-precision)") (OutMajor :type "Float (double-precision)") (OutMinor :type "Float (double-precision)") (PiercingDamage :type "Float (double-precision)"))
  (bind _piercingdamage (`local.PiercingDamage`))
  (set `local.PiercingDamage` (`.PiercingDamage` (`self.CalculateAttackModifier` WeaponType ArmorType)))
  (switch `string` (`KismetSystemLibrary.GetObjectName` HitComponent)
    (:`LeftArmColl`
      (set `local.OutDeath` 0.0 :!label _label)
      (set `local.OutBlured` 0.0)
      (set `local.OutCritical` 1.0)
      (set `local.OutNasty` 0.0)
      (set `local.OutMajor` 5.0)
      (set `local.OutMinor` 10.0))
    (:`LeftHandColl`
      (goto _label))
    (:`RightArmColl`
      (goto _label))
    (:`RightHandColl`
      (goto _label))
    (:`LeftLegColl`
      (set `local.OutDeath` 0.0 :!label _label_2)
      (set `local.OutBlured` 0.0)
      (set `local.OutCritical` 1.0)
      (set `local.OutNasty` 0.0)
      (set `local.OutMajor` 5.0)
      (set `local.OutMinor` 10.0))
    (:`RightLegColl`
      (goto _label_2))
    (:`HipColl`
      (set `local.OutDeath` 5.0)
      (set `local.OutBlured` 0.0)
      (set `local.OutCritical` 15.0)
      (set `local.OutNasty` 15.0)
      (set `local.OutMajor` 15.0)
      (set `local.OutMinor` 40.0))
    (:`HeadColl`
      (set `local.OutDeath` 35.0)
      (set `local.OutBlured` 0.0)
      (set `local.OutCritical` 45.0)
      (set `local.OutNasty` 25.0)
      (set `local.OutMajor` 55.0)
      (set `local.OutMinor` 80.0)))
  (return (+ _piercingdamage (`local.OutDeath`)) (+ _piercingdamage (`local.OutBlured`)) (+ _piercingdamage (`local.OutCritical`)) (+ _piercingdamage (`local.OutNasty`)) (+ _piercingdamage (`local.OutMajor`)) (+ _piercingdamage (`local.OutMinor`))))

(fn `SlashingDamageModifier`
  (params (HitComponent :type "PrimitiveComponent Object Reference") (WeaponType :type "/Game/Blueprints/Enums/EnumWeaponType Enum" :default "NewEnumerator0") (ArmorType :type "/Game/Blueprints/Enums/EnumArmorType Enum" :default "NewEnumerator0"))
  (returns (InstantDeathDamage :type "Float (double-precision)") (BluredVisionDamage :type "Float (double-precision)") (CriticalWoundDamage :type "Float (double-precision)") (NastyWoundDamage :type "Float (double-precision)") (MajorWoundDamage :type "Float (double-precision)") (MinorWoundDamage :type "Float (double-precision)"))
  (locals (OutDeath :type "Float (double-precision)") (OutBlured :type "Float (double-precision)") (OutCritical :type "Float (double-precision)") (OutNasty :type "Float (double-precision)") (OutMajor :type "Float (double-precision)") (OutMinor :type "Float (double-precision)") (SlashingDamage :type "Float (double-precision)"))
  (bind _slashingdamage (`local.SlashingDamage`))
  (set `local.SlashingDamage` (`self.CalculateAttackModifier` WeaponType ArmorType))
  (switch `string` (`KismetSystemLibrary.GetObjectName` HitComponent)
    (:`LeftArmColl`
      (set `local.OutDeath` 1.0 :!label _label)
      (set `local.OutBlured` 0.0)
      (set `local.OutCritical` 5.0)
      (set `local.OutNasty` 7.0)
      (set `local.OutMajor` 10.0)
      (set `local.OutMinor` 30.0))
    (:`LeftHandColl`
      (goto _label))
    (:`RightArmColl`
      (goto _label))
    (:`RightHandColl`
      (goto _label))
    (:`LeftLegColl`
      (set `local.OutDeath` 1.0 :!label _label_2)
      (set `local.OutBlured` 0.0)
      (set `local.OutCritical` 5.0)
      (set `local.OutNasty` 7.0)
      (set `local.OutMajor` 10.0)
      (set `local.OutMinor` 30.0))
    (:`RightLegColl`
      (goto _label_2))
    (:`HipColl`
      (set `local.OutDeath` 2.0)
      (set `local.OutBlured` 0.0)
      (set `local.OutCritical` 10.0)
      (set `local.OutNasty` 12.0)
      (set `local.OutMajor` 20.0)
      (set `local.OutMinor` 40.0))
    (:`HeadColl`
      (set `local.OutDeath` 25.0)
      (set `local.OutBlured` 10.0)
      (set `local.OutCritical` 40.0)
      (set `local.OutNasty` 0.0)
      (set `local.OutMajor` 50.0)
      (set `local.OutMinor` 70.0)))
  (return (+ _slashingdamage (`local.OutDeath`)) (+ _slashingdamage (`local.OutBlured`)) (+ _slashingdamage (`local.OutCritical`)) (+ _slashingdamage (`local.OutNasty`)) (+ _slashingdamage (`local.OutMajor`)) (+ _slashingdamage (`local.OutMinor`))))

(fn `SmashingDamageModifier`
  (params (HitComponent :type "PrimitiveComponent Object Reference") (WeaponType :type "/Game/Blueprints/Enums/EnumWeaponType Enum" :default "NewEnumerator0") (ArmorType :type "/Game/Blueprints/Enums/EnumArmorType Enum" :default "NewEnumerator0"))
  (returns (InstantDeathDamage :type "Float (double-precision)") (BluredVisionDamage :type "Float (double-precision)") (CriticalWoundDamage :type "Float (double-precision)") (NastyWoundDamage :type "Float (double-precision)") (MajorWoundDamage :type "Float (double-precision)") (MinorWoundDamage :type "Float (double-precision)"))
  (locals (OutDeath :type "Float (double-precision)") (OutBlured :type "Float (double-precision)") (OutCritical :type "Float (double-precision)") (OutNasty :type "Float (double-precision)") (OutMajor :type "Float (double-precision)") (OutMinor :type "Float (double-precision)") (SmashingDamage :type "Float (double-precision)"))
  (bind _smashingdamage (`local.SmashingDamage`))
  (set `local.SmashingDamage` (`.SmashingDamage` (`self.CalculateAttackModifier` WeaponType ArmorType)))
  (switch `string` (`KismetSystemLibrary.GetObjectName` HitComponent)
    (:`LeftArmColl`
      (set `local.OutDeath` 0.0 :!label _label)
      (set `local.OutBlured` 0.0)
      (set `local.OutCritical` 1.0)
      (set `local.OutNasty` 1.0)
      (set `local.OutMajor` 5.0)
      (set `local.OutMinor` 10.0))
    (:`LeftHandColl`
      (goto _label))
    (:`RightArmColl`
      (goto _label))
    (:`RightHandColl`
      (goto _label))
    (:`LeftLegColl`
      (set `local.OutDeath` 0.0 :!label _label_2)
      (set `local.OutBlured` 0.0)
      (set `local.OutCritical` 1.0)
      (set `local.OutNasty` 1.0)
      (set `local.OutMajor` 5.0)
      (set `local.OutMinor` 10.0))
    (:`RightLegColl`
      (goto _label_2))
    (:`HipColl`
      (set `local.OutDeath` 2.0)
      (set `local.OutBlured` 0.0)
      (set `local.OutCritical` 5.0)
      (set `local.OutNasty` 7.0)
      (set `local.OutMajor` 10.0)
      (set `local.OutMinor` 20.0))
    (:`HeadColl`
      (set `local.OutDeath` 15.0)
      (set `local.OutBlured` 30.0)
      (set `local.OutCritical` 0.0)
      (set `local.OutNasty` 20.0)
      (set `local.OutMajor` 0.0)
      (set `local.OutMinor` 0.0)))
  (return (+ _smashingdamage (`local.OutDeath`)) (+ _smashingdamage (`local.OutBlured`)) (+ _smashingdamage (`local.OutCritical`)) (+ _smashingdamage (`local.OutNasty`)) (+ _smashingdamage (`local.OutMajor`)) (+ _smashingdamage (`local.OutMinor`))))