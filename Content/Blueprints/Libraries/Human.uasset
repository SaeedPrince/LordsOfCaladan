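; Human function library that builds a randomized human Body struct: face and proportions, skeletal clothing, hair and armor, plus sword and shield.
; RandomBody combines RandomHumanFace and RandomHumanOrgan, which gathers per-slot functions pairing meshes with materials and color parameters.
; GetMeshMat and GetStaticMat pick from asset arrays, wrapping and clamping indices to tolerate out-of-range rolls.
; Chest and skirt use default IDs, randomizing only chest colors.
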(fn `CreateShield`
  (returns (Mesh :type "StaticMesh Object Reference") (Material :type "MaterialInstance Object Reference") (Color :type "Array of LinearColor Structure") (Parameter :type "Array of Name"))
  (locals (Shields :type "Array of /Game/Blueprints/Structures/Character/StaticToMaterials Structure"))
  (bind (_stroke _front _back _half) (`self.RandomShieldColor` null))
  (bind _shields (`local.Shields`))
  (bind (_staticmesh _material) (`self.GetStaticMat` _shields (`KismetMathLibrary.RandomIntegerInRange` 0 (- (`KismetArrayLibrary.Array_Length` _shields) 1)) (`KismetMathLibrary.RandomIntegerInRange` 0 10) (`KismetMathLibrary.RandomIntegerInRange` 0 10)))
  (return _staticmesh _material (`|MakeArray` _stroke _front _back _half) (`|MakeArray` "RedHsl" "GreenHSL" "BlueHSL" "BlackHSL" :!type "Name")))

(fn `CreateSword`
  (returns (Mesh :type "StaticMesh Object Reference") (Material :type "MaterialInstance Object Reference") (Color :type "LinearColor Structure") (Parameter :type Name))
  (locals (Weapons :type "Array of /Game/Blueprints/Structures/Character/StaticToMaterials Structure"))
  (bind _weapons (`local.Weapons`))
  (bind (_staticmesh _material) (`self.GetStaticMat` _weapons (`KismetMathLibrary.RandomIntegerInRange` 0 (- (`KismetArrayLibrary.Array_Length` _weapons) 1)) (`KismetMathLibrary.RandomIntegerInRange` 0 10)))
  (return _staticmesh _material (`self.RandomSwordColor` null) "HSL"))

(fn `GetMeshMat`
  (params (TargetArray :type "Array of /Game/Blueprints/Structures/Character/ModelsToMaterials Structure") (StructID :type Integer) (MeshID :type Integer) (MaterialID :type Integer))
  (returns (Mesh :type "SkeletalMesh Object Reference") (Material :type "MaterialInstance Object Reference"))
  (locals (OutMesh :type "SkeletalMesh Object Reference"))
  (bind (_models _materials) (break `/Game/Blueprints/Structures/Character/ModelsToMaterials` (`|GetArrayItem` TargetArray (`KismetMathLibrary.Clamp` StructID 0 (- (`KismetArrayLibrary.Array_Length` TargetArray) 1)))))
  (bind _returnvalue (`KismetArrayLibrary.Array_Length` _models))
  (bind _returnvalue_2 (`KismetArrayLibrary.Array_Length` _materials))
  (if (> _returnvalue 0)
    (set `local.OutMesh` (`|GetArrayItem` _models (`KismetMathLibrary.Clamp` (`self.LoopThroughInt` _returnvalue MeshID) 0 (- _returnvalue 1)))))
  (return (`local.OutMesh`) (`|GetArrayItem` _materials (`KismetMathLibrary.Clamp` (`self.LoopThroughInt` _returnvalue_2 MaterialID) 0 (- _returnvalue_2 1)))))

(fn `GetRandomOnLength`
  (params (TargetArray :type "Array of /Game/Blueprints/Structures/Character/ModelsToMaterials Structure"))
  (returns (ReturnValue :type Integer))
  (return (`KismetMathLibrary.RandomIntegerInRange` 0 (- (`KismetArrayLibrary.Array_Length` TargetArray) 1))))

(fn `GetStaticMat`
  (params (TargetArray :type "Array of /Game/Blueprints/Structures/Character/StaticToMaterials Structure") (StructID :type Integer) (MeshID :type Integer) (MaterialID :type Integer))
  (returns (StaticMesh :type "StaticMesh Object Reference") (Material :type "MaterialInstance Object Reference"))
  (bind (_models _materials) (break `/Game/Blueprints/Structures/Character/StaticToMaterials` (`|GetArrayItem` TargetArray (`KismetMathLibrary.Clamp` StructID 0 (- (`KismetArrayLibrary.Array_Length` TargetArray) 1)))))
  (bind _returnvalue (`KismetArrayLibrary.Array_Length` _models))
  (bind _returnvalue_2 (`KismetArrayLibrary.Array_Length` _materials))
  (return (`|GetArrayItem` _models (`KismetMathLibrary.Clamp` (`self.LoopThroughInt` _returnvalue MeshID) 0 (- _returnvalue 1))) (`|GetArrayItem` _materials (`KismetMathLibrary.Clamp` (`self.LoopThroughInt` _returnvalue_2 MaterialID) 0 (- _returnvalue_2 1)))))

(fn `LoopThroughInt`
  (params (Length :type Integer) (Int :type Integer))
  (returns (ReturnValue :type Integer))
  (locals (OutInt :type Integer))
  (if (> Length 0)
    (set `local.OutInt` (`KismetMathLibrary.SelectInt` (- Int (* Length (/ Int Length))) Int (> Int (- Length 1))))
    (else
      (set `local.OutInt` 0)))
  (return (`local.OutInt`)))

(fn `RandomBody`
  (returns (ReturnValue :type "/Game/Blueprints/Structures/Game/StructBody Structure"))
  (bind (_skelethalarray _staticarray) (`self.RandomHumanOrgan` null))
  (return (make `/Game/Blueprints/Structures/Game/StructBody` (`self.RandomHumanFace` null) _skelethalarray _staticarray)))

(fn `RandomBoots`
  (returns (Mesh :type "SkeletalMesh Object Reference") (Material :type "MaterialInstance Object Reference") (PantsColor :type "LinearColor Structure"))
  (locals (Boots :type "Array of /Game/Blueprints/Structures/Character/ModelsToMaterials Structure"))
  (bind _boots (`local.Boots`))
  (bind (_mesh _material) (`self.GetMeshMat` _boots (`self.GetRandomOnLength` _boots) (`KismetMathLibrary.RandomIntegerInRange` 0 10) (`KismetMathLibrary.RandomIntegerInRange` 0 10)))
  (return _mesh _material (`self.RandomPantsColor` null)))

(fn `RandomChest`
  (returns (Mesh :type "SkeletalMesh Object Reference") (Material :type "Array of MaterialInstance Object Reference") (ChestColor :type "Array of LinearColor Structure"))
  (locals (Chests :type "Array of /Game/Blueprints/Structures/Character/ModelsToMaterials Structure") (DefaultHumanChestType :type Integer) (DefaultHumanChestModel :type Integer :default 4) (DefaultHumanChestMaterial :type Integer :default 8) (Skirt :type "Array of /Game/Blueprints/Structures/Character/ModelsToMaterials Structure") (DefaultHumanSkirtMaterial :type Integer :default 9))
  (bind (_chest _upperarm _lowerarm) (`self.RandomChestColor` null))
  (bind (_mesh _material) (`self.GetMeshMat` (`local.Chests`) (`local.DefaultHumanChestType`) (`local.DefaultHumanChestModel`) (`local.DefaultHumanChestMaterial`)))
  (return _mesh (`|MakeArray` _material (`.Material` (`self.GetMeshMat` (`local.Skirt`) 0 0 (`local.DefaultHumanSkirtMaterial`)))) (`|MakeArray` _chest _upperarm _lowerarm (struct :`R` 1.0 :`G` 1.0 :`B` 1.0))))

(fn `RandomChestColor`
  (returns (Chest :type "LinearColor Structure") (UpperArm :type "LinearColor Structure") (LowerArm :type "LinearColor Structure"))
  (bind _returnvalue (`self.RandomColor` 0.0 1.3 0.0 1.5 0.0 1.5))
  (return _returnvalue _returnvalue (`self.RandomColor` 0.9 1.1 0.0 1.5 0.0 1.2)))

(fn `RandomColor`
  (params (RMin :type "Float (double-precision)") (RMax :type "Float (double-precision)") (GMin :type "Float (double-precision)") (Gmax :type "Float (double-precision)") (BMin :type "Float (double-precision)") (BMax :type "Float (double-precision)"))
  (returns (ReturnValue :type "LinearColor Structure"))
  (return (`KismetMathLibrary.MakeColor` (select `bool` (`KismetMathLibrary.RandomBool`) :`false` (`KismetMathLibrary.RandomFloatInRange` 0.9 1.1) :`true` (`KismetMathLibrary.RandomFloatInRange` RMin RMax)) (`KismetMathLibrary.RandomFloatInRange` GMin Gmax) (`KismetMathLibrary.RandomFloatInRange` BMin BMax))))

(fn `RandomGloves`
  (returns (Mesh :type "SkeletalMesh Object Reference") (Material :type "Array of MaterialInstance Object Reference") (ShoulderColor :type "Array of LinearColor Structure") (Parameters :type "Array of Name"))
  (locals (Gloves :type "Array of /Game/Blueprints/Structures/Character/ModelsToMaterials Structure"))
  (bind (_top _stroke _shoulder) (`self.RandomShouldColor` null))
  (bind _gloves (`local.Gloves`))
  (bind (_mesh _material) (`self.GetMeshMat` _gloves (`self.GetRandomOnLength` _gloves) (`KismetMathLibrary.RandomIntegerInRange` 0 4) (`KismetMathLibrary.RandomIntegerInRange` 0 4)))
  (return _mesh (`|MakeArray` _material) (`|MakeArray` _top _stroke _shoulder) (`|MakeArray` "RedHsl" "BlueHSL" "BlackHSL" "GreenHSL" :!type "Name")))

(fn `RandomHair`
  (returns (HairMesh :type "SkeletalMesh Object Reference") (BeardMesh :type "SkeletalMesh Object Reference") (HairMaterial :type "MaterialInstance Object Reference") (BeardMaterial :type "MaterialInstance Object Reference") (HairColor :type "LinearColor Structure"))
  (locals (Hairs :type "Array of /Game/Blueprints/Structures/Character/ModelsToMaterials Structure") (Beards :type "Array of /Game/Blueprints/Structures/Character/ModelsToMaterials Structure"))
  (bind (_mesh _material) (`self.GetMeshMat` (`local.Beards`) 0 (`KismetMathLibrary.RandomIntegerInRange` 0 7)))
  (bind (_mesh_2 _material_2) (`self.GetMeshMat` (`local.Hairs`) 0 (`KismetMathLibrary.RandomIntegerInRange` 0 6)))
  (return _mesh_2 _mesh _material_2 _material (select `int` (`KismetMathLibrary.RandomIntegerInRange` 0 5) :`0` (struct :`R` 0.965 :`G` 0.702598 :`B` 0.214586 :`A` 1.0) :`1` (struct :`R` 0.04 :`G` 0.04 :`B` 0.04 :`A` 1.0) :`2` (struct :`R` 0.327778 :`G` 0.127438 :`B` 0.043735 :`A` 1.0) :`3` (struct :`R` 0.695 :`G` 0.695 :`B` 0.695 :`A` 1.0) :`4` (struct :`R` 0.505 :`G` 0.095155 :`B` 0.03535 :`A` 1.0) :`5` (struct :`R` 0.095 :`G` 0.037655 :`B` 0.012308 :`A` 1.0) :!type "LinearColor Structure")))

(fn `RandomHelmet`
  (returns (Mesh :type "SkeletalMesh Object Reference") (Material :type "Array of MaterialInstance Object Reference") (ShoulderColor :type "Array of LinearColor Structure") (Parameters :type "Array of Name"))
  (locals (Helmets :type "Array of /Game/Blueprints/Structures/Character/ModelsToMaterials Structure"))
  (bind _helmets (`local.Helmets`))
  (bind (_mesh _material) (`self.GetMeshMat` _helmets (`self.GetRandomOnLength` _helmets) (`KismetMathLibrary.RandomIntegerInRange` 0 10) (`KismetMathLibrary.RandomIntegerInRange` 0 10)))
  (return _mesh (`|MakeArray` _material) (`|MakeArray` (`self.RandomHelmetColor` null)) (`|MakeArray` "HSL" :!type "Name")))

(fn `RandomHelmetColor`
  (returns (Helmet :type "LinearColor Structure"))
  (return (`self.RandomColor` 0.0 1.0 0.0 1.0 0.0 1.5)))

(fn `RandomHumanFace`
  (returns (ReturnValue :type "/Game/Blueprints/Structures/Game/StructHumanFaceAndProportion Structure"))
  (bind _returnvalue (`KismetMathLibrary.HSVToRGB` (`KismetMathLibrary.RandomFloatInRange` 0.0 200.0) (`KismetMathLibrary.RandomFloatInRange` 0.0 0.15) (`KismetMathLibrary.RandomFloatInRange` 0.2 1.1) 0.0))
  (return (make `/Game/Blueprints/Structures/Game/StructHumanFaceAndProportion` (* (`KismetMathLibrary.RandomFloatInRange` 0.7 1.7) (`.V` (`KismetMathLibrary.RGBToHSV` _returnvalue))) (`KismetMathLibrary.RandomFloatInRange` 0.0 1.0) (`KismetMathLibrary.RandomFloatInRange` -0.5 1.0) (`KismetMathLibrary.RandomFloatInRange` 1.0 1.3) (`KismetMathLibrary.FClamp` (`KismetMathLibrary.RandomFloatInRange` -1.0 2.0) 0.0 2.0) _returnvalue (`KismetMathLibrary.RandomFloatInRange` -1.0 1.3) (`KismetMathLibrary.RandomFloatInRange` 0.85 1.2))))

(fn `RandomHumanOrgan`
  (returns (SkelethalArray :type "Array of /Game/Blueprints/Structures/Game/StructSkelethalOrgan Structure") (StaticArray :type "Array of /Game/Blueprints/Structures/Game/StructStaticOrgan Structure"))
  (bind (_mesh _material _chestcolor) (`self.RandomChest` null))
  (bind (_mesh_2 _material_2 _pantscolor) (`self.RandomPants` null))
  (bind (_mesh_3 _material_3 _pantscolor_2) (`self.RandomBoots` null))
  (bind (_hairmesh _beardmesh _hairmaterial _beardmaterial _haircolor) (`self.RandomHair` null))
  (bind (_mesh_4 _material_4 _shouldercolor _parameters) (`self.RandomShoulder` null))
  (bind (_mesh_5 _material_5 _shouldercolor_2 _parameters_2) (`self.RandomGloves` null))
  (bind (_mesh_6 _material_6 _shouldercolor_3 _parameters_3) (`self.RandomHelmet` null))
  (bind (_mesh_7 _material_7 _color _parameter) (`self.CreateSword` null))
  (bind (_mesh_8 _material_8 _color_2 _parameter_2) (`self.CreateShield` null))
  (bind _array (`|MakeArray` "HSL" :!type "Name"))
  (bind _array_2 (`|MakeArray` "TipColor" :!type "Name"))
  (bind _array_3 (`|MakeArray` _haircolor))
  (return (`|MakeArray` (make `/Game/Blueprints/Structures/Game/StructSkelethalOrgan` _mesh (make `/Game/Blueprints/Structures/Character/StructMeshParameters` _material _chestcolor (`|MakeArray` "RedHsl" "GreenHSL" "BlueHSL" "BlackHSL" :!type "Name") true)) (make `/Game/Blueprints/Structures/Game/StructSkelethalOrgan` _mesh_2 (make `/Game/Blueprints/Structures/Character/StructMeshParameters` (`|MakeArray` _material_2) (`|MakeArray` _pantscolor) _array true)) (make `/Game/Blueprints/Structures/Game/StructSkelethalOrgan` _mesh_3 (make `/Game/Blueprints/Structures/Character/StructMeshParameters` (`|MakeArray` _material_3) (`|MakeArray` _pantscolor_2) _array true)) (make `/Game/Blueprints/Structures/Game/StructSkelethalOrgan` _hairmesh (make `/Game/Blueprints/Structures/Character/StructMeshParameters` (`|MakeArray` _hairmaterial) _array_3 _array_2 true)) (make `/Game/Blueprints/Structures/Game/StructSkelethalOrgan` _beardmesh (make `/Game/Blueprints/Structures/Character/StructMeshParameters` (`|MakeArray` _beardmaterial) _array_3 _array_2 true)) (make `/Game/Blueprints/Structures/Game/StructSkelethalOrgan` _mesh_4 (make `/Game/Blueprints/Structures/Character/StructMeshParameters` _material_4 _shouldercolor _parameters)) (make `/Game/Blueprints/Structures/Game/StructSkelethalOrgan` _mesh_5 (make `/Game/Blueprints/Structures/Character/StructMeshParameters` _material_5 _shouldercolor_2 _parameters_2)) (make `/Game/Blueprints/Structures/Game/StructSkelethalOrgan` _mesh_6 (make `/Game/Blueprints/Structures/Character/StructMeshParameters` _material_6 _shouldercolor_3 _parameters_3))) (`|MakeArray` (make `/Game/Blueprints/Structures/Game/StructStaticOrgan` _mesh_7 (make `/Game/Blueprints/Structures/Character/StructMeshParameters` (`|MakeArray` _material_7) (`|MakeArray` _color) (`|MakeArray` _parameter))) (make `/Game/Blueprints/Structures/Game/StructStaticOrgan` _mesh_8 (make `/Game/Blueprints/Structures/Character/StructMeshParameters` (`|MakeArray` _material_8) _color_2 _parameter_2)))))

(fn `RandomPants`
  (returns (Mesh :type "SkeletalMesh Object Reference") (Material :type "MaterialInstance Object Reference") (PantsColor :type "LinearColor Structure"))
  (locals (Pants :type "Array of /Game/Blueprints/Structures/Character/ModelsToMaterials Structure"))
  (bind _pants (`local.Pants`))
  (bind (_mesh _material) (`self.GetMeshMat` _pants (`self.GetRandomOnLength` _pants) (`KismetMathLibrary.RandomIntegerInRange` 0 10) (`KismetMathLibrary.RandomIntegerInRange` 0 10)))
  (return _mesh _material (`self.RandomPantsColor` null)))

(fn `RandomPantsColor`
  (returns (Pants :type "LinearColor Structure"))
  (return (`self.RandomColor` 0.0 1.0 0.0 1.2 0.0 1.5)))

(fn `RandomShieldColor`
  (returns (Stroke :type "LinearColor Structure") (Front :type "LinearColor Structure") (Back :type "LinearColor Structure") (Half :type "LinearColor Structure"))
  (bind _returnvalue (`self.RandomColor` 0.0 2.0 0.0 1.3 0.0 1.3))
  (return _returnvalue _returnvalue _returnvalue _returnvalue))

(fn `RandomShouldColor`
  (returns (Top :type "LinearColor Structure") (Stroke :type "LinearColor Structure") (Shoulder :type "LinearColor Structure"))
  (bind _returnvalue (`self.RandomColor` 0.0 1.0 0.0 1.0 0.0 1.3))
  (return _returnvalue _returnvalue _returnvalue))

(fn `RandomShoulder`
  (returns (Mesh :type "SkeletalMesh Object Reference") (Material :type "Array of MaterialInstance Object Reference") (ShoulderColor :type "Array of LinearColor Structure") (Parameters :type "Array of Name"))
  (locals (Shoulders :type "Array of /Game/Blueprints/Structures/Character/ModelsToMaterials Structure"))
  (bind (_top _stroke _shoulder) (`self.RandomShouldColor` null))
  (bind _shoulders (`local.Shoulders`))
  (bind (_mesh _material) (`self.GetMeshMat` _shoulders (`self.GetRandomOnLength` _shoulders) (`KismetMathLibrary.RandomIntegerInRange` 0 10) (`KismetMathLibrary.RandomIntegerInRange` 0 10)))
  (return _mesh (`|MakeArray` _material) (`|MakeArray` _top _stroke _shoulder) (`|MakeArray` "RedHsl" "GreenHSL" "BlueHSL" :!type "Name")))

(fn `RandomSwordColor`
  (returns (Color :type "LinearColor Structure"))
  (return (`self.RandomColor` 0.0 1.0 0.0 1.0 0.0 1.0)))