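; LibArmor is a combat function library that decides whether an attack hits through armor.
; CalculateArmorModifier returns slashing, smashing and piercing modifiers, currently the same fixed values with no distinct cases per armor type.
; HitSuccess picks the modifier matching the attack type and succeeds when a random 0–100 roll exceeds its truncated value.
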(fn `CalculateArmorModifier`
  (params (ArmorType :type "/Game/Blueprints/Enums/EnumArmorType Enum" :default "NewEnumerator0"))
  (returns (Slashing :type "Float (double-precision)") (Smashing :type "Float (double-precision)") (Piercing :type "Float (double-precision)"))
  (locals (OutSlashing :type "Float (double-precision)") (OutSmashing :type "Float (double-precision)") (OutPiercing :type "Float (double-precision)"))
  (switch `/Game/Blueprints/Enums/EnumArmorType` ArmorType
    (:`NewEnumerator0`
      (set `local.OutSlashing` 20.0)
      (set `local.OutSmashing` 16.0)
      (set `local.OutPiercing` 22.0)
      (return (`local.OutSlashing`) (`local.OutSmashing`) (`local.OutPiercing`)))))

(fn `HitSuccess`
  (params (AttackType :type "/Game/Blueprints/Enums/EnumAttackType Enum" :default "NewEnumerator0") (ArmorType :type "/Game/Blueprints/Enums/EnumArmorType Enum" :default "NewEnumerator0"))
  (returns (ReturnValue :type Boolean))
  (locals (OutBool :type Boolean) (RandomInt :type Integer))
  (bind (_slashing _smashing _piercing) (`self.CalculateArmorModifier` ArmorType))
  (bind _randomint (`local.RandomInt`))
  (set `local.RandomInt` (`KismetMathLibrary.RandomIntegerInRange` 0 100))
  (switch `/Game/Blueprints/Enums/EnumAttackType` AttackType
    (:`NewEnumerator0`
      (set `local.OutBool` (> _randomint (`KismetMathLibrary.FTrunc` _slashing))))
    (:`NewEnumerator2`
      (set `local.OutBool` (> _randomint (`KismetMathLibrary.FTrunc` _smashing))))
    (:`NewEnumerator1`
      (set `local.OutBool` (> _randomint (`KismetMathLibrary.FTrunc` _piercing)))))
  (return (`local.OutBool`)))