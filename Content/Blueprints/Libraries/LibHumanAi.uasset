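; LibHumanAi is a helper function library for human AI units, covering soldier combat tuning, unit filtering and navigation avoidance.
; Soldier type (sword, archer, mace) selects attack ranges, frequency and weapon state, with both melee types sharing distance values.
; Other helpers compute 2D flanking points, check attack range and filter actors by player or soldiers by person type.
; Avoidance masks isolate one group index, ignoring all others.
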(fn `AvoidanceByIndex`
  (params (Index :type Integer))
  (returns (Group :type "NavAvoidanceMask Structure") (Avoid :type "NavAvoidanceMask Structure") (Ignore :type "NavAvoidanceMask Structure"))
  (locals (Max :type Integer :default 32) (OutGroup :type "Array of Boolean") (OutAvoid :type "Array of Boolean") (OutIgnore :type "Array of Boolean"))
  (bind _outgroup (`local.OutGroup`))
  (bind _outavoid (`local.OutAvoid`))
  (bind _outignore (`local.OutIgnore`))
  (for _index (range (+ (`local.Max`) 1))
    (if (== _index Index)
      (`KismetArrayLibrary.Array_Add` _outgroup true)
      (`KismetArrayLibrary.Array_Add` _outavoid true)
      (`KismetArrayLibrary.Array_Add` _outignore)
      (else
        (`KismetArrayLibrary.Array_Add` _outgroup)
        (`KismetArrayLibrary.Array_Add` _outavoid)
        (`KismetArrayLibrary.Array_Add` _outignore true))))
  (return (`self.BooleanArrayToNavAvoidance` _outgroup) (`self.BooleanArrayToNavAvoidance` _outavoid) (`self.BooleanArrayToNavAvoidance` _outignore)))

(fn `BooleanArrayToNavAvoidance`
  (params (BoolArray :type "Array of Boolean"))
  (returns (ReturnValue :type "NavAvoidanceMask Structure"))
  (return (make `NavAvoidanceMask` (`|GetArrayItem` BoolArray) (`|GetArrayItem` BoolArray 1) (`|GetArrayItem` BoolArray 2) (`|GetArrayItem` BoolArray 3) (`|GetArrayItem` BoolArray 4) (`|GetArrayItem` BoolArray 5) (`|GetArrayItem` BoolArray 6) (`|GetArrayItem` BoolArray 7) (`|GetArrayItem` BoolArray 8) (`|GetArrayItem` BoolArray 9) (`|GetArrayItem` BoolArray 10) (`|GetArrayItem` BoolArray 11) (`|GetArrayItem` BoolArray 12) (`|GetArrayItem` BoolArray 13) (`|GetArrayItem` BoolArray 14) (`|GetArrayItem` BoolArray 15) (`|GetArrayItem` BoolArray 16) (`|GetArrayItem` BoolArray 17) (`|GetArrayItem` BoolArray 18) (`|GetArrayItem` BoolArray 19) (`|GetArrayItem` BoolArray 20) (`|GetArrayItem` BoolArray 21) (`|GetArrayItem` BoolArray 22) (`|GetArrayItem` BoolArray 23) (`|GetArrayItem` BoolArray 24) (`|GetArrayItem` BoolArray 25) (`|GetArrayItem` BoolArray 26) (`|GetArrayItem` BoolArray 27) (`|GetArrayItem` BoolArray 28) (`|GetArrayItem` BoolArray 29) (`|GetArrayItem` BoolArray 30) (`|GetArrayItem` BoolArray 31))))

(fn `DistanceOkayToAttack`
  (params (Controller :type "/Game/Blueprints/Controllers/AIController_Game Object Reference"))
  (returns (ReturnValue :type Boolean))
  (return (not (`/Game/Blueprints/Libraries/LibCharacter.CharacterNeedMove` (`Actor.K2_GetActorLocation` (`/Game/Blueprints/Controllers/AIController_Game.TargetChari` Controller)) (`Actor.K2_GetActorLocation` (`/Game/Blueprints/Controllers/AIController_Game.CharacterRef` Controller)) (`/Game/Blueprints/Controllers/AIController_Game.FightMinDistance` Controller) (`/Game/Blueprints/Controllers/AIController_Game.FightMaxDistance` Controller)))))

(fn `FlankedLocation2D`
  (params (CharacterLocation :type "Vector Structure") (TargetLocation :type "Vector Structure") (FlankedAngel :type "Float (double-precision)"))
  (returns (FlankedLocation :type "Vector Structure"))
  (bind _returnvalue (`/Game/Blueprints/Libraries/LibMath.VectorLenghth2D` CharacterLocation TargetLocation))
  (bind _returnvalue_2 (/ FlankedAngel 2.0))
  (return (`KismetMathLibrary.MakeVector` (- (.x TargetLocation) (* (`KismetMathLibrary.DegCos` _returnvalue_2) _returnvalue)) (- (.y TargetLocation) (* _returnvalue (`KismetMathLibrary.DegSin` _returnvalue_2))))))

(fn `HumanAIArrayByActorArray`
  (params (ActorArray :type "Array of Actor Object Reference") (PlayerIndex :type Integer))
  (returns (ReturnValue :type "Array of /Game/Blueprints/Characters/HumanAI Object Reference"))
  (locals (OutArray :type "Array of /Game/Blueprints/Characters/HumanAI Object Reference"))
  (bind _outarray (`local.OutArray`))
  (for _array_element ActorArray
    (bind _ashuman_ai (cast `/Game/Blueprints/Characters/HumanAI` _array_element))
    (if (== (`/Game/Blueprints/Characters/HumanBP.PlayerIndex` _ashuman_ai) PlayerIndex)
      (`KismetArrayLibrary.Array_Add` _outarray _ashuman_ai)))
  (return _outarray))

(fn `SoldierExistsInHumanAIArray`
  (params (HumanAIArray :type "Array of /Game/Blueprints/Characters/HumanAI Object Reference"))
  (returns (ReturnValue :type Boolean))
  (locals (OutBool :type Boolean))
  (for _array_element HumanAIArray
    (if (`|EnumEquality` (`/Game/Blueprints/Characters/HumanBP.PersonType` _array_element) "NewEnumerator1")
      (set `local.OutBool` true)
      (break)))
  (return (`local.OutBool`)))

(fn `SoldiersArrayByHumanAIArray`
  (params (HumanAIArray :type "Array of /Game/Blueprints/Characters/HumanAI Object Reference"))
  (returns (ReturnValue :type "Array of /Game/Blueprints/Characters/HumanAI Object Reference"))
  (locals (OutArray :type "Array of /Game/Blueprints/Characters/HumanAI Object Reference"))
  (bind _outarray (`local.OutArray`))
  (for _array_element HumanAIArray
    (if (`|EnumEquality` (`/Game/Blueprints/Characters/HumanBP.PersonType` _array_element) "NewEnumerator1")
      (`KismetArrayLibrary.Array_Add` _outarray _array_element)))
  (return _outarray))

(fn `SuitableDistanceBySoldierType`
  (params (SoldierType :type "/Game/Blueprints/Enums/EnumSoldierType Enum" :default "NewEnumerator0"))
  (returns (Min :type "Float (double-precision)") (Max :type "Float (double-precision)") (WeaponRadius :type "Float (double-precision)") (Frequency :type "Float (double-precision)"))
  (locals (OutMin :type "Float (double-precision)") (OutMax :type "Float (double-precision)") (OutRadius :type "Float (double-precision)") (OutFrequency :type "Float (double-precision)"))
  (switch `/Game/Blueprints/Enums/EnumSoldierType` SoldierType
    (:`NewEnumerator0`
      (set `local.OutMin` 110.0 :!label _label)
      (set `local.OutMax` 180.0)
      (set `local.OutRadius` 140.0)
      (set `local.OutFrequency` 1.8))
    (:`NewEnumerator1`
      (set `local.OutMin` 500.0)
      (set `local.OutMax` 5100.0)
      (set `local.OutRadius` 5000.0)
      (set `local.OutFrequency` 6.5))
    (:`NewEnumerator2`
      (goto _label)))
  (return (`local.OutMin`) (`local.OutMax`) (`local.OutRadius`) (`local.OutFrequency`)))

(fn `WeaponStateBySoldierType`
  (params (SoldierType :type "/Game/Blueprints/Enums/EnumSoldierType Enum" :default "NewEnumerator0"))
  (returns (ReturnValue :type "/Game/Blueprints/Enums/EnumWeaponState Enum"))
  (locals (OutState :type "/Game/Blueprints/Enums/EnumWeaponState Enum"))
  (switch `/Game/Blueprints/Enums/EnumSoldierType` SoldierType
    (:`NewEnumerator0`
      (set `local.OutState` "NewEnumerator1"))
    (:`NewEnumerator1`
      (set `local.OutState` "NewEnumerator2"))
    (:`NewEnumerator2`
      (set `local.OutState` "NewEnumerator3")))
  (return (`local.OutState`)))