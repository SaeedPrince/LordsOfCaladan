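; Player function library with a check for whether a player can create Warrior or Archer soldiers.
; Both results require a free military place in the building array and a non-empty idle pool.
; Warrior also needs a sword and shield in the buildings' item stacks, while Archer needs a bow and quiver.
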(fn `SoldierCreationPossibility`
  (params (BuildingArray :type "Array of /Game/Assets/BP_Meshes/Architecture/BP_House Object Reference") (IdlePool :type "Array of /Game/Blueprints/Controllers/AIController_Game Object Reference"))
  (returns (Warrior :type Boolean) (Archer :type Boolean))
  (locals (BowItemIndex :type Integer :default 18) (QuiverItemIndex :type Integer :default 33) (SwordItemIndex :type Integer :default 12) (ShieldItemIndex :type Integer :default 13))
  (bind _returnvalue (`/Game/Blueprints/Libraries/Building.MilitaryFreePlaceAvailable` BuildingArray))
  (bind _returnvalue_2 (> (`KismetArrayLibrary.Array_Length` IdlePool) 0))
  (return (and _returnvalue _returnvalue_2 (`/Game/Blueprints/Libraries/Building.ItemAvailableInStack` (`local.SwordItemIndex`) BuildingArray) (`/Game/Blueprints/Libraries/Building.ItemAvailableInStack` (`local.ShieldItemIndex`) BuildingArray)) (and _returnvalue _returnvalue_2 (`/Game/Blueprints/Libraries/Building.ItemAvailableInStack` (`local.BowItemIndex`) BuildingArray) (`/Game/Blueprints/Libraries/Building.ItemAvailableInStack` (`local.QuiverItemIndex`) BuildingArray))))