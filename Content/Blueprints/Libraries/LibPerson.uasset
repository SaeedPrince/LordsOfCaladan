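; Blueprint function library of helpers for Persons, the AI controllers behind civilian and soldier characters that live or work in buildings.
; Membership checks compare a Person against building resident and worker lists by person type, alongside an older type-agnostic version.
; Linear-scan helpers search arrays and garrison indices, filter soldiers, find the closest Person to a location and convert actors to controllers.
; PersonInventory tallies items into capped name-and-count text lines.
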(fn `ClosestPersonToLocation`
  (params (Location :type "Vector Structure") (PersonArray :type "Array of /Game/Blueprints/Controllers/AIController_Game Object Reference"))
  (returns (ReturnValue :type "/Game/Blueprints/Controllers/AIController_Game Object Reference"))
  (locals (OutPerson :type "/Game/Blueprints/Controllers/AIController_Game Object Reference") (Destin :type "Float (double-precision)"))
  (bind _returnvalue (`KismetArrayLibrary.Array_Length` PersonArray))
  (bind _output (`|GetArrayItem` PersonArray))
  (if (> _returnvalue 0)
    (set `local.OutPerson` _output)
    (set `local.Destin` (`self.PersonDestinationToLocation` _output Location))
    (for _index (range 1 _returnvalue)
      (bind _output_2 (`|GetArrayItem` PersonArray _index))
      (bind _destination (`self.PersonDestinationToLocation` _output_2 Location))
      (if (< _destination (`local.Destin`))
        (set `local.Destin` _destination)
        (set `local.OutPerson` _output_2)))
    (return (`local.OutPerson`))))

(fn `FindMilitPersonByIndex`
  (params (Building :type "/Game/Assets/BP_Meshes/Architecture/BP_House Object Reference") (Index :type Integer))
  (returns (Found :type Boolean) (Person :type "/Game/Blueprints/Controllers/AIController_Game Object Reference"))
  (locals (OutPerson :type "/Game/Blueprints/Controllers/AIController_Game Object Reference") (OutBool :type Boolean))
  (for _array_element (`/Game/Assets/BP_Meshes/Architecture/BP_House.MilitResident` Building)
    (if (== (`/Game/Blueprints/Controllers/AIController_Game.IndexInGarrison` _array_element) Index)
      (set `local.OutBool` true)
      (set `local.OutPerson` _array_element)
      (break)))
  (return (`local.OutBool`) (`local.OutPerson`)))

(fn `GetPersonIndex`
  (params (PersonArray :type "Array of /Game/Blueprints/Controllers/AIController_Game Object Reference") (Person :type "/Game/Blueprints/Controllers/AIController_Game Object Reference"))
  (returns (Found :type Boolean) (Index :type Integer))
  (locals (OutBool :type Boolean) (OutIndex :type Integer))
  (for (_array_element _array_index) PersonArray
    (if (== _array_element Person)
      (set `local.OutBool` true)
      (set `local.OutIndex` _array_index)
      (break)))
  (return (`local.OutBool`) (`local.OutIndex`)))

(fn `ItemIndexExistInItemList`
  (params (ItemIndex :type Integer) (ItemList :type "Array of Integer"))
  (returns (Exist :type Boolean) (Index :type Integer))
  (locals (OutBool :type Boolean) (OutIndex :type Integer))
  (for (_array_element _array_index) ItemList
    (if (== _array_element ItemIndex)
      (set `local.OutBool` true)
      (set `local.OutIndex` _array_index)
      (break)))
  (return (`local.OutBool`) (`local.OutIndex`)))

(fn `PersonArrayByActorArray`
  (params (ActorArray :type "Array of Actor Object Reference"))
  (returns (PersonArray :type "Array of /Game/Blueprints/Controllers/AIController_Game Object Reference"))
  (locals (OutArray :type "Array of /Game/Blueprints/Controllers/AIController_Game Object Reference"))
  (bind _outarray (`local.OutArray`))
  (for _array_element ActorArray
    (bind _ashuman_ai (cast `/Game/Blueprints/Characters/HumanAI` _array_element))
    (`KismetArrayLibrary.Array_Add` _outarray (`/Game/Blueprints/Characters/HumanBP.AIControllerRef` _ashuman_ai)))
  (return _outarray))

(fn `PersonArrayByHumanAIArray`
  (params (HumanAIArray :type "Array of /Game/Blueprints/Characters/HumanAI Object Reference"))
  (returns (ReturnValue :type "Array of /Game/Blueprints/Controllers/AIController_Game Object Reference"))
  (locals (OutPersonArray :type "Array of /Game/Blueprints/Controllers/AIController_Game Object Reference"))
  (bind _outpersonarray (`local.OutPersonArray`))
  (for _array_element HumanAIArray
    (`KismetArrayLibrary.Array_Add` _outpersonarray (`/Game/Blueprints/Characters/HumanBP.AIControllerRef` _array_element)))
  (return _outpersonarray))

(fn `PersonDestinationToLocation`
  (params (Person :type "/Game/Blueprints/Controllers/AIController_Game Object Reference") (Location :type "Vector Structure"))
  (returns (Destination :type "Float (double-precision)"))
  (return (`KismetMathLibrary.VSize` (- Location (`Actor.K2_GetActorLocation` (`Controller.K2_GetPawn` Person))))))

(fn `PersonDoesNotBelongToBuilding`
  (params (Person :type "/Game/Blueprints/Controllers/AIController_Game Object Reference") (Building :type "/Game/Assets/BP_Meshes/Architecture/BP_House Object Reference"))
  (returns (ReturnValue :type Boolean))
  (locals (OutBool :type Boolean :default true))
  (bind _isresident (`/Game/Assets/BP_Meshes/Architecture/BP_House.IsResident` Building))
  (switch `/Game/Blueprints/Enums/EnumPersonType` (`/Game/Blueprints/Characters/HumanBP.PersonType` (`/Game/Blueprints/Controllers/AIController_Game.CharacterRef` Person))
    (:`NewEnumerator0`
      (if _isresident
        (for _array_element (`/Game/Assets/BP_Meshes/Architecture/BP_House.CivilResident` Building)
          (if (== _array_element Person)
            (set `local.OutBool` false)
            (break)))
        (return (`local.OutBool`))
        (elif (`/Game/Assets/BP_Meshes/Architecture/BP_House.IsProductive` Building)
          (for _array_element_2 (`/Game/Assets/BP_Meshes/Architecture/BP_House.CivilWorker` Building)
            (if (== Person _array_element_2)
              (set `local.OutBool` false)
              (break)))
          (return (`local.OutBool`)))))
    (:`NewEnumerator1`
      (if _isresident
        (for _array_element_3 (`/Game/Assets/BP_Meshes/Architecture/BP_House.MilitResident` Building)
          (if (== Person _array_element_3)
            (set `local.OutBool` false)
            (break))))
      (return (`local.OutBool`)))))

(fn `PersonDoesNotBelongToBuildingOld`
  (params (Person :type "/Game/Blueprints/Controllers/AIController_Game Object Reference") (Building :type "/Game/Assets/BP_Meshes/Architecture/BP_House Object Reference"))
  (returns (ReturnValue :type Boolean))
  (locals (OutBool :type Boolean :default true))
  (if (`/Game/Assets/BP_Meshes/Architecture/BP_House.IsResident` Building)
    (for _array_element (`/Game/Assets/BP_Meshes/Architecture/BP_House.CivilResident` Building)
      (if (== _array_element Person)
        (set `local.OutBool` false)
        (break)))
    (return (`local.OutBool`))
    (elif (`/Game/Assets/BP_Meshes/Architecture/BP_House.IsProductive` Building)
      (for _array_element_2 (`/Game/Assets/BP_Meshes/Architecture/BP_House.CivilWorker` Building)
        (if (== Person _array_element_2)
          (set `local.OutBool` false)
          (break)))
      (return (`local.OutBool`)))))

(fn `PersonExistInIdlePool`
  (params (Person :type "/Game/Blueprints/Controllers/AIController_Game Object Reference") (IdlePool :type "Array of /Game/Blueprints/Controllers/AIController_Game Object Reference"))
  (returns (ReturnValue :type Boolean))
  (locals (OutBool :type Boolean))
  (for _array_element IdlePool
    (if (== _array_element Person)
      (set `local.OutBool` true)
      (break)))
  (return (`local.OutBool`)))

(fn `PersonInventory`
  (params (Person :type "/Game/Blueprints/Controllers/AIController_Game Object Reference") (MaxNumber :type Integer))
  (returns (ReturnValue :type "Array of Text"))
  (locals (ItemList :type "Array of Integer") (OutText :type "Array of Text") (ItemCount :type "Array of Integer"))
  (bind _itemcount (`local.ItemCount`))
  (bind _itemlist (`local.ItemList`))
  (for _array_element (`/Game/Blueprints/Controllers/AIController_Game.Inventory` Person)
    (bind _index (`/Game/Assets/BP_Meshes/Item/BP_Item.Index` _array_element))
    (bind (_exist _index_2) (`self.ItemIndexExistInItemList` _index (`local.ItemList`)))
    (if _exist
      (`/Engine/EditorBlueprintResources/StandardMacros.IncrementInt` (`|GetArrayItem` _itemcount _index_2))
      (elif (< (`KismetArrayLibrary.Array_Length` _itemlist) MaxNumber)
        (`KismetArrayLibrary.Array_Add` _itemlist _index)
        (`KismetArrayLibrary.Array_Add` _itemcount 1))))
  (for (_array_element_2 _array_index) _itemlist
    (`KismetArrayLibrary.Array_Add` (`local.OutText`) (`KismetTextLibrary.Conv_StringToText` (`KismetStringLibrary.Concat_StrStr` (`/Game/Blueprints/Libraries/LibItem.ItemNameByIndex` _array_element_2) " : " (`KismetStringLibrary.Conv_IntToString` (`|GetArrayItem` _itemcount _array_index))))))
  (return (`local.OutText`)))

(fn `SoldierExistsInPersonArray`
  (params (PersonArray :type "Array of /Game/Blueprints/Controllers/AIController_Game Object Reference"))
  (returns (ReturnValue :type Boolean))
  (locals (OutBool :type Boolean))
  (for _array_element PersonArray
    (if (`|EnumEquality` (`/Game/Blueprints/Characters/HumanBP.PersonType` (`/Game/Blueprints/Controllers/AIController_Game.CharacterRef` _array_element)) "NewEnumerator1")
      (set `local.OutBool` true)
      (break)))
  (return (`local.OutBool`)))

(fn `SoldiersArrayByPersonArray`
  (params (PersonArray :type "Array of /Game/Blueprints/Controllers/AIController_Game Object Reference"))
  (returns (ReturnValue :type "Array of /Game/Blueprints/Controllers/AIController_Game Object Reference"))
  (locals (OutPersonArray :type "Array of /Game/Blueprints/Controllers/AIController_Game Object Reference"))
  (bind _outpersonarray (`local.OutPersonArray`))
  (for _array_element PersonArray
    (if (`|EnumEquality` (`/Game/Blueprints/Characters/HumanBP.PersonType` (`/Game/Blueprints/Controllers/AIController_Game.CharacterRef` _array_element)) "NewEnumerator1")
      (`KismetArrayLibrary.Array_Add` _outpersonarray _array_element)))
  (return _outpersonarray))