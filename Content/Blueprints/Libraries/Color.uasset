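; Blueprint function library of color helpers for mapping named colors and tinting primitive components.
; GetColorByString turns seven color names into opaque linear colors.
; Two setters create a dynamic material instance on material slot 0 and write a named vector parameter, taking either a color name or a linear color.
; GetColorName is only a partial inverse, checking red and green channels to return Yellow, Red or, otherwise, Green.
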(fn `GetColorByString`
  (params (Color :type String))
  (returns (ReturnValue :type "LinearColor Structure"))
  (locals (OutColor :type "LinearColor Structure"))
  (switch `string` Color
    (:`Red`
      (set `local.OutColor` (make `LinearColor` 1.0 0.0 0.0 1.0)))
    (:`Green`
      (set `local.OutColor` (make `LinearColor` 0.0 1.0 0.0 1.0)))
    (:`Blue`
      (set `local.OutColor` (make `LinearColor` 0.0 0.0 1.0 1.0)))
    (:`Yellow`
      (set `local.OutColor` (make `LinearColor` 1.0 1.0 0.0 1.0)))
    (:`Cyan`
      (set `local.OutColor` (make `LinearColor` 0.0 1.0 1.0 1.0)))
    (:`Purple`
      (set `local.OutColor` (make `LinearColor` 1.0 0.0 1.0 1.0)))
    (:`White`
      (set `local.OutColor` (make `LinearColor` 1.0 1.0 1.0 1.0))))
  (return (`local.OutColor`)))

(fn `GetColorName`
  (params (Color :type "LinearColor Structure"))
  (returns (ReturnValue :type String))
  (locals (OutString :type String))
  (bind (_r _g) (break `LinearColor` Color))
  (if (== _r 1.0)
    (if (== _g 1.0)
      (set `local.OutString` "Yellow")
      (else
        (set `local.OutString` "Red")))
    (else
      (set `local.OutString` "Green")))
  (return (`local.OutString`)))

(fn `SetComponentColorByLinearColor`
  (params (PrimitiveComponent :type "PrimitiveComponent Object Reference") (Parameter :type Name) (Color :type "LinearColor Structure"))
  (bind _returnvalue (`PrimitiveComponent.CreateDynamicMaterialInstance` PrimitiveComponent 0 null))
  (`MaterialInstanceDynamic.SetVectorParameterValue` _returnvalue Parameter Color))

(fn `SetComponentColorByString`
  (params (PrimitiveComponent :type "PrimitiveComponent Object Reference") (Parameter :type Name) (Color :type String))
  (bind _returnvalue (`PrimitiveComponent.CreateDynamicMaterialInstance` PrimitiveComponent 0 null))
  (`MaterialInstanceDynamic.SetVectorParameterValue` _returnvalue Parameter (`self.GetColorByString` Color)))