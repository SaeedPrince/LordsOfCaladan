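; Blueprint function library of helpers for the game's item system, where items are identified by an integer index.
; One function maps each index to a display name, covering resources, food, weapons, armor and currency.
; Others linearly search item arrays by index or reference to test presence or return the matching item.
; Another returns the warrior's primary item indices, the sword and shield.
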(fn `GetItemFromItemArray`
  (params (Index :type Integer) (ItemArray :type "Array of /Game/Assets/BP_Meshes/Item/BP_Item Object Reference"))
  (returns (ReturnValue :type "/Game/Assets/BP_Meshes/Item/BP_Item Object Reference"))
  (locals (OutItem :type "/Game/Assets/BP_Meshes/Item/BP_Item Object Reference"))
  (for _array_element ItemArray
    (if (== (`/Game/Assets/BP_Meshes/Item/BP_Item.Index` _array_element) Index)
      (set `local.OutItem` _array_element)
      (break)))
  (return (`local.OutItem`)))

(fn `ItemIndexExistsInArray`
  (params (ItemArray :type "Array of /Game/Assets/BP_Meshes/Item/BP_Item Object Reference") (ItemIndex :type Integer))
  (returns (ReturnValue :type Boolean))
  (locals (OutBool :type Boolean))
  (for _array_element ItemArray
    (if (== (`/Game/Assets/BP_Meshes/Item/BP_Item.Index` _array_element) ItemIndex)
      (set `local.OutBool` true)
      (break)))
  (return (`local.OutBool`)))

(fn `ItemNameByIndex`
  (params (ItemIndex :type Integer))
  (returns (ReturnValue :type String))
  (locals (OutName :type String))
  (switch `int` ItemIndex
    (:`0`
      (set `local.OutName` "Wood"))
    (:`1`
      (set `local.OutName` "Stone"))
    (:`2`
      (set `local.OutName` "Planks"))
    (:`3`
      (set `local.OutName` "Grain"))
    (:`4`
      (set `local.OutName` "Flour"))
    (:`5`
      (set `local.OutName` "Honey"))
    (:`6`
      (set `local.OutName` "Bread"))
    (:`7`
      (set `local.OutName` "Cake"))
    (:`8`
      (set `local.OutName` "Fish"))
    (:`9`
      (set `local.OutName` "Meat"))
    (:`10`
      (set `local.OutName` "Sausage"))
    (:`11`
      (set `local.OutName` "Smoked Beef"))
    (:`12`
      (set `local.OutName` "Sword"))
    (:`13`
      (set `local.OutName` "Shield"))
    (:`14`
      (set `local.OutName` "Cooper Armor"))
    (:`15`
      (set `local.OutName` "Iron Armor"))
    (:`16`
      (set `local.OutName` "Cannon"))
    (:`17`
      (set `local.OutName` "Cannon Ball"))
    (:`18`
      (set `local.OutName` "Bow"))
    (:`19`
      (set `local.OutName` "Iron Ore"))
    (:`20`
      (set `local.OutName` "Gold Ore"))
    (:`21`
      (set `local.OutName` "Copper Ore"))
    (:`22`
      (set `local.OutName` "Coal"))
    (:`23`
      (set `local.OutName` "Sulfur"))
    (:`24`
      (set `local.OutName` "Gunpowder"))
    (:`25`
      (set `local.OutName` "Light Armor"))
    (:`26`
      (set `local.OutName` "Gambeson"))
    (:`27`
      (set `local.OutName` "Arrow"))
    (:`28`
      (set `local.OutName` "Leather"))
    (:`29`
      (set `local.OutName` "Wool"))
    (:`30`
      (set `local.OutName` "Iron Bar"))
    (:`31`
      (set `local.OutName` "Copper Bar"))
    (:`32`
      (set `local.OutName` "Gold Bar"))
    (:`33`
      (set `local.OutName` "Quiver"))
    (:`34`
      (set `local.OutName` "Gold Coin"))
    (:`35`
      (set `local.OutName` "Ball Chest")))
  (return (`local.OutName`)))

(fn `ItemRefExistsInArray`
  (params (ItemRef :type "/Game/Assets/BP_Meshes/Item/BP_Item Object Reference") (ItemArray :type "Array of /Game/Assets/BP_Meshes/Item/BP_Item Object Reference"))
  (returns (ReturnValue :type Boolean))
  (locals (OutBool :type Boolean))
  (for _array_element ItemArray
    (if (== _array_element ItemRef)
      (set `local.OutBool` true)
      (break)))
  (return (`local.OutBool`)))

(fn `WarriorPrimaryItemIndexArray`
  (returns (ReturnValue :type "Array of Integer"))
  (return (`|MakeArray` 12 13)))