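; Blueprint function library of projectile ballistics math for launching at a target point.
; A helper splits start and end points into height difference, horizontal distance and straight-line range, the geometry the other formulas take as inputs.
; Closed-form solvers derive a launch angle, both angles that reach a target at a given speed and gravity, or the gravity needed from flight time or target offset.
; Another helper builds quadratic coefficients for the launch-angle tangent.
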(fn `AngleOfReach`
  (params (Speed :type "Float (double-precision)") (GravityScale :type "Float (double-precision)") (Height :type "Float (double-precision)") (Destination :type "Float (double-precision)"))
  (returns (Angle1 :type "Float (double-precision)") (Angle2 :type "Float (double-precision)"))
  (bind _returnvalue (`KismetMathLibrary.Square` Speed))
  (bind _returnvalue_2 (* GravityScale Destination))
  (bind _returnvalue_3 (`KismetMathLibrary.Sqrt` (- (`KismetMathLibrary.Square` _returnvalue) (* GravityScale (+ (* _returnvalue Height 2.0) (* GravityScale (`KismetMathLibrary.Square` Destination)))))))
  (return (`KismetMathLibrary.DegAtan` (/ (+ _returnvalue _returnvalue_3) _returnvalue_2)) (`KismetMathLibrary.DegAtan` (/ (- _returnvalue _returnvalue_3) _returnvalue_2))))

(fn `CreateQuadraticEquationFactors`
  (params (Height :type "Float (double-precision)") (Destination :type "Float (double-precision)") (Gravity :type "Float (double-precision)") (Speed :type "Float (double-precision)"))
  (returns (A :type "Float (double-precision)") (B :type "Float (double-precision)") (C :type "Float (double-precision)"))
  (bind _returnvalue (/ (* Destination Gravity) (* (`KismetMathLibrary.Square` Speed) 2.0)))
  (return _returnvalue -1.0 (+ _returnvalue (/ Height Destination))))

(fn `GravityScale`
  (params (Speed :type "Float (double-precision)") (Angle :type "Float (double-precision)") (Height :type "Float (double-precision)") (Time :type "Float (double-precision)"))
  (returns (ReturnValue :type "Float (double-precision)"))
  (return (/ (* (- (* (* Speed Time) (`KismetMathLibrary.DegSin` Angle)) Height) 2.0) (`KismetMathLibrary.Square` Time))))

(fn `GravityScaleByXAndY`
  (params (Height :type "Float (double-precision)") (Speed :type "Float (double-precision)") (Angle :type "Float (double-precision)") (Destination :type "Float (double-precision)"))
  (returns (ReturnValue :type "Float (double-precision)"))
  (return (/ (* (- (* (`KismetMathLibrary.DegSin` (* Angle 2.0)) Destination) (* Height (`KismetMathLibrary.Square` (`KismetMathLibrary.DegCos` Angle)) 2.0)) (`KismetMathLibrary.Square` Speed)) (`KismetMathLibrary.Square` Destination))))

(fn `HeightAndDestination`
  (params (Start :type "Vector Structure") (End :type "Vector Structure"))
  (returns (Height :type "Float (double-precision)") (Destination :type "Float (double-precision)") (Range :type "Float (double-precision)"))
  (return (- (.z End) (.z Start)) (`KismetMathLibrary.Sqrt` (+ (`KismetMathLibrary.Square` (- (.x End) (.x Start))) (`KismetMathLibrary.Square` (- (.y End) (.y Start))))) (`KismetMathLibrary.VSize` (- End Start))))

(fn `ShootAngle`
  (params (Height :type "Float (double-precision)") (Destination :type "Float (double-precision)"))
  (returns (ReturnValue :type "Float (double-precision)"))
  (return (`KismetMathLibrary.DegAtan` (+ (`KismetMathLibrary.Sqrt` (+ (/ (`KismetMathLibrary.Square` Height) (`KismetMathLibrary.Square` Destination)) 1.0)) (/ Height Destination)))))