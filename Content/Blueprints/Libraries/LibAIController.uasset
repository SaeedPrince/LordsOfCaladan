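; Function library for AI controllers that resolves civilian and soldier differences and builds orders and jobs for people.
; Type switches choose behavior tree and blackboard, plus residence or garrison building, slot index, placement and location tag.
; GoHomeJob combines these with a per-location acceptable distance into a go-home order.
; JobFromOrder converts movement, stay and attack-person orders into job structs, while AttackBuildingJob is an empty stub.
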(fn `AcceptableDistanceByLocation`
  (params (Location :type "/Game/Blueprints/Enums/EnumLocations Enum" :default "NewEnumerator3"))
  (returns (ReturnValue :type "Float (double-precision)"))
  (locals (OutDistance :type "Float (double-precision)"))
  (switch `/Game/Blueprints/Enums/EnumLocations` Location
    (:`NewEnumerator3`
      (set `local.OutDistance` 50.0))
    (:`NewEnumerator0`
      (set `local.OutDistance` 20.0))
    (:`NewEnumerator1`
      (set `local.OutDistance` 20.0))
    (:`NewEnumerator4`
      (set `local.OutDistance` 20.0))
    (:`NewEnumerator2`
      (set `local.OutDistance` 300.0)))
  (return (`local.OutDistance`)))

(fn `AttackBuildingJob`
  (returns (ReturnValue :type "/Game/Blueprints/Structures/Game/StructNormalJob Structure"))
  (return))

(fn `GetBehaviorTreeByPersonType`
  (params (PersonType :type "/Game/Blueprints/Enums/EnumPersonType Enum" :default "NewEnumerator0"))
  (returns (BehaviorTree :type "BehaviorTree Object Reference") (Blackboard :type "BlackboardData Object Reference"))
  (locals (OutBehavior :type "BehaviorTree Object Reference") (OutBlackboard :type "BlackboardData Object Reference"))
  (switch `/Game/Blueprints/Enums/EnumPersonType` PersonType
    (:`NewEnumerator0`
      (set `local.OutBehavior` "/Game/Blueprints/AI/BehaviorTree/BT_Civilian.BT_Civilian")
      (set `local.OutBlackboard` null))
    (:`NewEnumerator1`
      (set `local.OutBehavior` "/Game/Blueprints/AI/BehaviorTree/BT_Miltary.BT_Miltary")
      (set `local.OutBlackboard` "/Game/Blueprints/AI/BehaviorTree/BB_Military.BB_Military")))
  (return (`local.OutBehavior`) (`local.OutBlackboard`)))

(fn `GetIndexInResidenceByType`
  (params (Person :type "/Game/Blueprints/Controllers/AIController_Game Object Reference"))
  (returns (ReturnValue :type Integer))
  (locals (OutInt :type Integer))
  (switch `/Game/Blueprints/Enums/EnumPersonType` (`/Game/Blueprints/Characters/HumanBP.PersonType` (`/Game/Blueprints/Controllers/AIController_Game.CharacterRef` Person))
    (:`NewEnumerator0`
      (set `local.OutInt` (`/Game/Blueprints/Controllers/AIController_Game.IndexInResidence` Person)))
    (:`NewEnumerator1`
      (set `local.OutInt` (`/Game/Blueprints/Controllers/AIController_Game.IndexInGarrison` Person))))
  (return (`local.OutInt`)))

(fn `GoHomeJob`
  (params (Person :type "/Game/Blueprints/Controllers/AIController_Game Object Reference"))
  (returns (ReturnValue :type "/Game/Blueprints/Structures/Game/StructOrder Structure"))
  (bind _returnvalue (`self.HomeLocationByType` Person))
  (return (make `/Game/Blueprints/Structures/Game/StructOrder` :`Location` (`self.LocationByType` Person (`/Game/Blueprints/Characters/HumanBP.PersonType` (`/Game/Blueprints/Controllers/AIController_Game.CharacterRef` Person))) :`AcceptableDistance` (`self.AcceptableDistanceByLocation` _returnvalue) :`LocationName` _returnvalue)))

(fn `HomeLocationByType`
  (params (Person :type "/Game/Blueprints/Controllers/AIController_Game Object Reference"))
  (returns (ReturnValue :type "/Game/Blueprints/Enums/EnumLocations Enum"))
  (locals (OutLocation :type "/Game/Blueprints/Enums/EnumLocations Enum"))
  (switch `/Game/Blueprints/Enums/EnumPersonType` (`/Game/Blueprints/Characters/HumanBP.PersonType` (`/Game/Blueprints/Controllers/AIController_Game.CharacterRef` Person))
    (:`NewEnumerator0`
      (set `local.OutLocation` "NewEnumerator0"))
    (:`NewEnumerator1`
      (set `local.OutLocation` "NewEnumerator4")))
  (return (`local.OutLocation`)))

(fn `JobFromOrder`
  (params (Order :type "/Game/Blueprints/Structures/Game/StructOrder Structure"))
  (returns (Job :type "/Game/Blueprints/Structures/Game/StructNormalJob Structure"))
  (locals (OutID :type "/Game/Blueprints/Enums/EnumNormalJob Enum") (OouLocation :type "Vector Structure") (OutDistance :type "Float (double-precision)") (OutCharacter :type "/Game/Blueprints/Characters/HumanBP Object Reference") (OutLocationName :type "/Game/Blueprints/Enums/EnumLocations Enum"))
  (bind ((`ID_35_AC04C87D43E4199B0062C4BB682719AE` _id) (`Location_17_63C4BC394B3E41CED6A9CE92D794BC4A` _location) (`AcceptableDistance_18_1608884F4BB24D81A775E88FC7979BDF` _acceptabledistance) (`TargetActor_33_26A6FFB849E17320017F01978D5BC46F` _targetactor) (`LocationName_39_8273CDE24B77EEF59DD25A8264B2E180` _locationname)) (break `/Game/Blueprints/Structures/Game/StructOrder` Order))
  (switch `/Game/Blueprints/Enums/EnumOrder` _id
    (:`NewEnumerator11`
      (set `local.OutID` "NewEnumerator11"))
    (:`NewEnumerator4`
      (set `local.OutID` "NewEnumerator4")
      (set `local.OouLocation` _location :!label _label)
      (set `local.OutDistance` _acceptabledistance)
      (set `local.OutLocationName` _locationname))
    (:`NewEnumerator10`
      (set `local.OutID` "NewEnumerator10")
      (goto _label))
    (:`NewEnumerator1`
      (set `local.OutID` "NewEnumerator1")
      (bind _ashuman_bp (cast `/Game/Blueprints/Characters/HumanBP` _targetactor))
      (set `local.OutCharacter` _ashuman_bp))
    (:`NewEnumerator8`
      (set `local.OutID` "NewEnumerator8")
      (goto _label)))
  (return (make `/Game/Blueprints/Structures/Game/StructNormalJob` (`local.OutID`) (`local.OouLocation`) (`local.OutDistance`) (`local.OutCharacter`) (`local.OutLocationName`))))

(fn `LocationByType`
  (params (Person :type "/Game/Blueprints/Controllers/AIController_Game Object Reference") (PersonType :type "/Game/Blueprints/Enums/EnumPersonType Enum" :default "NewEnumerator0"))
  (returns (ReturnValue :type "Vector Structure"))
  (locals (OutLocation :type "Vector Structure"))
  (switch `/Game/Blueprints/Enums/EnumPersonType` PersonType
    (:`NewEnumerator0`
      (set `local.OutLocation` (`/Game/Blueprints/Controllers/AIController_Game.ResidentPlacement` Person)))
    (:`NewEnumerator1`
      (set `local.OutLocation` (`/Game/Blueprints/Controllers/AIController_Game.SoldierPlacement` Person))))
  (return (`local.OutLocation`)))

(fn `ResidenceByType`
  (params (Person :type "/Game/Blueprints/Controllers/AIController_Game Object Reference"))
  (returns (ReturnValue :type "/Game/Assets/BP_Meshes/Architecture/BP_House Object Reference"))
  (locals (OutBuilding :type "/Game/Assets/BP_Meshes/Architecture/BP_House Object Reference"))
  (switch `/Game/Blueprints/Enums/EnumPersonType` (`/Game/Blueprints/Characters/HumanBP.PersonType` (`/Game/Blueprints/Controllers/AIController_Game.CharacterRef` Person))
    (:`NewEnumerator0`
      (set `local.OutBuilding` (`/Game/Blueprints/Controllers/AIController_Game.BuildingResidence` Person)))
    (:`NewEnumerator1`
      (set `local.OutBuilding` (`/Game/Blueprints/Controllers/AIController_Game.BuildingGarrison` Person))))
  (return (`local.OutBuilding`)))