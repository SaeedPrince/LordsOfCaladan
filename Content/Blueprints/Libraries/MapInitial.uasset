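; Blueprint function library that supplies the initial map layout: Hilltop and Lowland sites, spawners, mines and their borders.
; MapObjects bundles the data, offsetting two spawners from the sites, leaving four zeroed, and building square borders with Box2DVertices.
; TestMineLocations lays mines out in an evenly spaced grid from count and row inputs.
; Mine products come from RandomArray with fixed occurrence values.
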(fn `MapObjects`
  (returns (Hilltop :type "Vector Structure") (Lowland :type "Vector Structure") (Spawners :type "Array of Vector Structure") (Mines :type "Array of Vector Structure") (HilltopBorder :type "Array of Vector Structure") (LowlandBorder :type "Array of Vector Structure") (HouseScale :type "Vector Structure") (BorderSide :type "Float (double-precision)") (MineProducts :type "Array of Integer"))
  (locals (HilltopLocation :type "Vector Structure" :default (0.0 0.0 20.0)) (LowlandLocation :type "Vector Structure" :default (70000.0 70000.0 20.0)) (SpawnerDistance :type "Vector Structure" :default (6000.0 0.0 100.0)) (MineCount :type Integer :default 40) (MineRow :type Integer :default 5) (OuterBorderSide :type "Float (double-precision)" :default 30000.0) (LowlandTestLocation :type "Vector Structure" :default (10000.0 10000.0 20.0)))
  (bind _hilltoplocation (`local.HilltopLocation`))
  (bind _spawnerdistance (`local.SpawnerDistance`))
  (bind _lowlandlocation (`local.LowlandLocation`))
  (bind _minecount (`local.MineCount`))
  (bind _outerborderside (`local.OuterBorderSide`))
  (return _hilltoplocation _lowlandlocation (`|MakeArray` (+ _hilltoplocation _spawnerdistance) (+ _lowlandlocation _spawnerdistance) (0.0 0.0 0.0) (0.0 0.0 0.0) (0.0 0.0 0.0) (0.0 0.0 0.0)) (`self.TestMineLocations` _minecount (`local.MineRow`)) (`/Game/Blueprints/Libraries/Math.Box2DVertices` _hilltoplocation _outerborderside) (`/Game/Blueprints/Libraries/Math.Box2DVertices` _lowlandlocation _outerborderside) (100.0 100.0 50.0) _outerborderside (`/Game/Blueprints/Libraries/Math.RandomArray` _minecount (`|MakeArray` 19 20 21 22 23))))

(fn `TestMineLocations`
  (params (MineCount :type Integer) (MineRow :type Integer))
  (returns (ReturnValue :type "Array of Vector Structure"))
  (locals (Column :type Integer) (Offset :type "Float (double-precision)" :default 4000.0) (Origin :type "Vector Structure" :default (5000.0 40000.0 0.0)) (OutLocations :type "Array of Vector Structure"))
  (bind _offset (`local.Offset`))
  (set `local.Column` (/ MineCount MineRow))
  (for _index (range MineRow)
    (for _index_2 (range (`local.Column`))
      (`KismetArrayLibrary.Array_Add` (`local.OutLocations`) (`KismetMathLibrary.MakeVector` (+ (* _index_2 _offset) (.x (`local.Origin`))) (+ (* _index _offset) (.y (`local.Origin`))) (.z (`local.Origin`))))))
  (return (`local.OutLocations`)))