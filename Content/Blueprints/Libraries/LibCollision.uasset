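; Blueprint function library that applies one of two collision presets, No Collision or Overlap All Dynamic, to a primitive component.
; SetComponentCollision sets enabled state, object type and eight channel responses from three per-preset lookup functions.
; As wired, the enabled lookup always returns NoCollision and the response lookup always returns Ignore for Visibility and Camera, whatever the preset assigns.
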(fn `CollisionEnabledByPreset`
  (params (CollisionPreset :type "/Game/Blueprints/Enums/EnumCollisionPreset Enum" :default "NewEnumerator0"))
  (returns (ReturnValue :type "ECollisionEnabled Enum"))
  (locals (OutEnum :type "ECollisionEnabled Enum"))
  (switch `/Game/Blueprints/Enums/EnumCollisionPreset` CollisionPreset
    (:`NewEnumerator0`
      (set `local.OutEnum` "NoCollision"))
    (:`NewEnumerator1`
      (set `local.OutEnum` "QueryOnly")))
  (return "NoCollision"))

(fn `CollisionResponseByPreset`
  (params (CollisionPreset :type "/Game/Blueprints/Enums/EnumCollisionPreset Enum" :default "NewEnumerator0"))
  (returns (Visibility :type "ECollisionResponse Enum") (Camera :type "ECollisionResponse Enum") (WorldStatic :type "ECollisionResponse Enum") (WorldDynamic :type "ECollisionResponse Enum") (Pawn :type "ECollisionResponse Enum") (PhysicsBody :type "ECollisionResponse Enum") (Vehicle :type "ECollisionResponse Enum") (Destructible :type "ECollisionResponse Enum"))
  (locals (OutWorldStatic :type "ECollisionResponse Enum") (OutWorldDynamic :type "ECollisionResponse Enum") (OutPawn :type "ECollisionResponse Enum") (OutPhysicsBody :type "ECollisionResponse Enum") (OutVehicle :type "ECollisionResponse Enum") (OutDestructible :type "ECollisionResponse Enum") (OutVisibility :type "ECollisionResponse Enum") (OutCamera :type "ECollisionResponse Enum"))
  (switch `/Game/Blueprints/Enums/EnumCollisionPreset` CollisionPreset
    (:`NewEnumerator0`
      (set `local.OutVisibility` "ECR_Ignore")
      (set `local.OutCamera` "ECR_Ignore")
      (set `local.OutWorldStatic` "ECR_Ignore")
      (set `local.OutWorldDynamic` "ECR_Ignore")
      (set `local.OutPawn` "ECR_Ignore")
      (set `local.OutPhysicsBody` "ECR_Ignore")
      (set `local.OutVehicle` "ECR_Ignore")
      (set `local.OutDestructible` "ECR_Ignore"))
    (:`NewEnumerator1`
      (set `local.OutVisibility` "ECR_Block")
      (set `local.OutCamera` "ECR_Block")
      (set `local.OutWorldStatic` "ECR_Overlap")
      (set `local.OutWorldDynamic` "ECR_Overlap")
      (set `local.OutPawn` "ECR_Overlap")
      (set `local.OutPhysicsBody` "ECR_Overlap")
      (set `local.OutVehicle` "ECR_Overlap")
      (set `local.OutDestructible` "ECR_Overlap")))
  (return "ECR_Ignore" "ECR_Ignore" (`local.OutWorldStatic`) (`local.OutWorldDynamic`) (`local.OutPawn`) (`local.OutPhysicsBody`) (`local.OutVehicle`) (`local.OutDestructible`)))

(fn `ObjectTypeByCollisionPreset`
  (params (CollisionPreset :type "/Game/Blueprints/Enums/EnumCollisionPreset Enum" :default "NewEnumerator0"))
  (returns (ReturnValue :type "ECollisionChannel Enum"))
  (locals (OutType :type "ECollisionChannel Enum"))
  (switch `/Game/Blueprints/Enums/EnumCollisionPreset` CollisionPreset
    (:`NewEnumerator0`
      (set `local.OutType` "ECC_WorldStatic"))
    (:`NewEnumerator1`
      (set `local.OutType` "ECC_WorldDynamic")))
  (return (`local.OutType`)))

(fn `SetComponentCollision`
  (params (PrimitiveComponent :type "PrimitiveComponent Object Reference (by ref)") (CollisionPreset :type "/Game/Blueprints/Enums/EnumCollisionPreset Enum" :default "NewEnumerator0"))
  (bind (_visibility _camera _worldstatic _worlddynamic _pawn _physicsbody _vehicle _destructible) (`self.CollisionResponseByPreset` CollisionPreset))
  (`PrimitiveComponent.SetCollisionEnabled` PrimitiveComponent (`self.CollisionEnabledByPreset` CollisionPreset))
  (`PrimitiveComponent.SetCollisionObjectType` PrimitiveComponent (`self.ObjectTypeByCollisionPreset` CollisionPreset))
  (`PrimitiveComponent.SetCollisionResponseToChannel` PrimitiveComponent "ECC_Visibility" _visibility)
  (`PrimitiveComponent.SetCollisionResponseToChannel` PrimitiveComponent "ECC_Camera" _camera)
  (`PrimitiveComponent.SetCollisionResponseToChannel` PrimitiveComponent "ECC_WorldStatic" _worldstatic)
  (`PrimitiveComponent.SetCollisionResponseToChannel` PrimitiveComponent "ECC_WorldDynamic" _worlddynamic)
  (`PrimitiveComponent.SetCollisionResponseToChannel` PrimitiveComponent "ECC_Pawn" _pawn)
  (`PrimitiveComponent.SetCollisionResponseToChannel` PrimitiveComponent "ECC_PhysicsBody" _physicsbody)
  (`PrimitiveComponent.SetCollisionResponseToChannel` PrimitiveComponent "ECC_Vehicle" _vehicle)
  (`PrimitiveComponent.SetCollisionResponseToChannel` PrimitiveComponent "ECC_Destructible" _destructible))