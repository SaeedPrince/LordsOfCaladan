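; LibBorder is a helper library that generates evenly spaced spawn positions along axis-aligned border edges between vertices.
; ConnectVertices compares two vertices, orders their coordinates and calls ConnectX for equal X, otherwise ConnectY at the second vertex's Y.
; Both helpers step by a spacing parameter, omitting the start point and possibly overshooting the end.
; SumIndicators appears intended to merge arrays, but appends Array2 to itself and returns it.
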(fn `ConnectVertices`
  (params (Vector1 :type "Vector Structure") (Vector2 :type "Vector Structure"))
  (returns (ReturnValue :type "Array of Vector Structure"))
  (locals (SpawnArray :type "Array of Vector Structure"))
  (bind _x (.x Vector1))
  (bind _y (.y Vector1))
  (bind _z (.z Vector1))
  (bind _x_2 (.x Vector2))
  (bind _y_2 (.y Vector2))
  (bind _z_2 (.z Vector2))
  (if (== _x _x_2)
    (if (< _y _y_2)
      (set `local.SpawnArray` (`self.ConnectX` _x _y _y_2 _z))
      (else
        (set `local.SpawnArray` (`self.ConnectX` _x _y_2 _y _z))))
    (elif (< _x _x_2)
      (set `local.SpawnArray` (`self.ConnectY` _x _x_2 _y_2 _z_2))
      (else
        (set `local.SpawnArray` (`self.ConnectY` _x_2 _x _y_2 _z_2)))))
  (return (`local.SpawnArray`)))

(fn `ConnectX`
  (params (X :type "Float (double-precision)") (Y1 :type "Float (double-precision)") (Y2 :type "Float (double-precision)") (Z :type "Float (double-precision)"))
  (returns (ReturnValue :type "Array of Vector Structure"))
  (locals (YAdd :type "Float (double-precision)") (YParam :type "Float (double-precision)" :default 1000.0) (SpawnTransforms :type "Array of Vector Structure"))
  (bind _yadd (`local.YAdd`))
  (set `local.YAdd` Y1)
  (while (< _yadd Y2)
    (set `local.YAdd` (+ (`local.YParam`) _yadd))
    (`KismetArrayLibrary.Array_Add` (`local.SpawnTransforms`) (`KismetMathLibrary.MakeVector` X _yadd Z)))
  (return (`local.SpawnTransforms`)))

(fn `ConnectY`
  (params (X1 :type "Float (double-precision)") (X2 :type "Float (double-precision)") (Y :type "Float (double-precision)") (Z :type "Float (double-precision)"))
  (returns (ReturnValue :type "Array of Vector Structure"))
  (locals (XAdd :type "Float (double-precision)") (XParam :type "Float (double-precision)" :default 1000.0) (SpawnTransforms :type "Array of Vector Structure"))
  (bind _xadd (`local.XAdd`))
  (set `local.XAdd` X1)
  (while (< _xadd X2)
    (set `local.XAdd` (+ (`local.XParam`) _xadd))
    (`KismetArrayLibrary.Array_Add` (`local.SpawnTransforms`) (`KismetMathLibrary.MakeVector` _xadd Y Z)))
  (return (`local.SpawnTransforms`)))

(fn `SumIndicators`
  (params (Array1 :type "Array of /Game/Blueprints/Actors/BP_Box Object Reference") (Array2 :type "Array of /Game/Blueprints/Actors/BP_Box Object Reference"))
  (returns (ReturnValue :type "Array of /Game/Blueprints/Actors/BP_Box Object Reference"))
  (locals (OutArray :type "Array of /Game/Blueprints/Actors/BP_Box Object Reference"))
  (for _array_element Array1
    (`KismetArrayLibrary.Array_Add` (`local.OutArray`) _array_element))
  (for _array_element_2 Array2
    (`KismetArrayLibrary.Array_Add` Array2 _array_element_2))
  (return Array2))