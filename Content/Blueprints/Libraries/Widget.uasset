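; Widget function library that supplies text and data helpers for the game's UI, covering the server browser and inventory screens.
; SessionToText turns a session into row text with truncated name, player counts and ping, matching the SearchHeader columns.
; ItemCategoryList and ItemCategoryCount map a category index to hardcoded weapon, material or food names and the corresponding InventoryData count arrays.
; AllUnchecked scans a checkbox array, stopping at the first checked box.
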(fn `AllUnchecked`
  (params (CheckboxArray :type "Array of CheckBox Object Reference"))
  (returns (ReturnValue :type Boolean))
  (locals (OutBool :type Boolean :default true))
  (for _array_element CheckboxArray
    (if (`|EnumEquality` (`CheckBox.GetCheckedState` _array_element) "Checked")
      (set `local.OutBool` false)
      (break)))
  (return (`local.OutBool`)))

(fn `ItemCategoryCount`
  (params (Category :type Integer) (InventoryData :type "/Game/Blueprints/Structures/Game/StructWidgetInventory Structure"))
  (returns (ReturnValue :type "Array of Integer"))
  (locals (OutArrayInt :type "Array of Integer"))
  (bind ((`NumWeapon_9_2F5BF0634E49915FCF723786EC3925B6` _numweapon) (`NumMaterial_11_AB9C48184D4207E70E5AF0A97C89DBEB` _nummaterial) (`NumFood_13_654ED9244CFCA0EBF1CEF0A62034A18A` _numfood)) (break `/Game/Blueprints/Structures/Game/StructWidgetInventory` InventoryData))
  (switch `int` Category
    (:`0`
      (set `local.OutArrayInt` _numweapon))
    (:`1`
      (set `local.OutArrayInt` _nummaterial))
    (:`2`
      (set `local.OutArrayInt` _numfood)))
  (return (`local.OutArrayInt`)))

(fn `ItemCategoryList`
  (params (Category :type Integer))
  (returns (ReturnValue :type "Array of String"))
  (locals (OutString :type "Array of String"))
  (switch `int` Category
    (:`0`
      (set `local.OutString` (`|MakeArray` "Sword" "Shield" "Copper Armor" "Iron Armor" "Cannon" "Cannon Ball" "Bow" "Light Armor" "Gambeson" "Arrow" "Quiver" "Ball Chest")))
    (:`1`
      (set `local.OutString` (`|MakeArray` "Wood" "Stone" "Planks" "Iron Ore" "Gold Ore" "Copper Ore" "Coal" "Sulfur" "Gunpowder" "Leather" "Wool" "Iron Bar" "Copper Bar" "Gold Bar" "Gold Coin")))
    (:`2`
      (set `local.OutString` (`|MakeArray` "Grain" "Flour" "Honey" "Bread" "Cake" "Fish" "Meat" "Sausage" "Smoked Beef"))))
  (return (`local.OutString`)))

(fn `SearchHeader`
  (returns (ReturnValue :type "Array of Text"))
  (return (`|MakeArray` "Server Name" "Current Players" "Max Players" "Ping" :!type "Text")))

(fn `SessionToText`
  (params (Session :type "BlueprintSessionResult Structure"))
  (returns (ReturnValue :type "Array of Text"))
  (locals (OutText :type "Array of Text"))
  (return (`|MakeArray` (`KismetTextLibrary.Conv_StringToText` (`KismetStringLibrary.Left` (`FindSessionsCallbackProxy.GetServerName` Session) 15)) (`KismetTextLibrary.Conv_IntToText` (`FindSessionsCallbackProxy.GetCurrentPlayers` Session)) (`KismetTextLibrary.Conv_IntToText` (`FindSessionsCallbackProxy.GetMaxPlayers` Session)) (`KismetTextLibrary.Conv_IntToText` (`FindSessionsCallbackProxy.GetPingInMs` Session)))))