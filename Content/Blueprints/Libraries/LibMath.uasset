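; Math function library for box, sphere and circle containment, player border placement checks, random selection, vector angles, melee attack points and quadratic roots.
; Shape tests reduce to axis-aligned min/max comparisons, so circles and spheres act as their bounding squares and cubes.
; 2D position functions classify overlap as named results, which the border functions use to test whether a box extends, sits inside or avoids borders.
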(fn `AngleBetweenVectors2D`
  (params (VectorA :type "Vector Structure") (VectorB :type "Vector Structure"))
  (returns (OutputAngle :type "Float (double-precision)"))
  (return (`KismetMathLibrary.DegAcos` (`KismetMathLibrary.Dot_VectorVector` (`KismetMathLibrary.Normal` (`KismetMathLibrary.MakeVector` (.x VectorA) (.y VectorA))) (`KismetMathLibrary.Normal` (`KismetMathLibrary.MakeVector` (.x VectorB) (.y VectorB)))))))

(fn `AngleBetweenVectors3D`
  (params (VectorA :type "Vector Structure") (VectorB :type "Vector Structure"))
  (returns (OutputAngle :type "Float (double-precision)"))
  (return (`KismetMathLibrary.DegAcos` (`KismetMathLibrary.Dot_VectorVector` (`KismetMathLibrary.Normal` (`KismetMathLibrary.MakeVector` (.x VectorA) (.y VectorA) (.z VectorA))) (`KismetMathLibrary.Normal` (`KismetMathLibrary.MakeVector` (.x VectorB) (.y VectorB) (.z VectorB)))))))

(fn `Box2DOriginAndSide`
  (params (Vertices :type "Array of Vector Structure"))
  (returns (Origin :type "Vector Structure") (Side :type "Float (double-precision)"))
  (locals (Point1 :type "Vector Structure") (Point2 :type "Vector Structure") (Point3 :type "Vector Structure") (Point4 :type "Vector Structure"))
  (bind _returnvalue (/ (+ (.x (`local.Point1`)) (.x (`local.Point2`))) 2.0))
  (set `local.Point1` (`|GetArrayItem` Vertices))
  (set `local.Point2` (`|GetArrayItem` Vertices 1))
  (set `local.Point3` (`|GetArrayItem` Vertices 2))
  (set `local.Point4` (`|GetArrayItem` Vertices 3))
  (return (`KismetMathLibrary.MakeVector` _returnvalue (/ (+ (.y (`local.Point1`)) (.y (`local.Point3`))) 2.0)) (* (- (.x (`local.Point4`)) _returnvalue) 2.0)))

(fn `Box2DVertices`
  (params (Origin :type "Vector Structure") (Side :type "Float (double-precision)"))
  (returns (ReturnValue :type "Array of Vector Structure"))
  (locals (Point1 :type "Vector Structure") (Point2 :type "Vector Structure") (Point3 :type "Vector Structure") (Point4 :type "Vector Structure"))
  (bind _x (.x Origin))
  (bind _y (.y Origin))
  (bind _returnvalue (- _x Side))
  (bind _returnvalue_2 (- _y Side))
  (bind _returnvalue_3 (+ _y Side))
  (bind _returnvalue_4 (+ _x Side))
  (set `local.Point1` (`KismetMathLibrary.MakeVector` _returnvalue _returnvalue_2))
  (set `local.Point2` (`KismetMathLibrary.MakeVector` _returnvalue_4 _returnvalue_2))
  (set `local.Point3` (`KismetMathLibrary.MakeVector` _returnvalue_4 _returnvalue_3))
  (set `local.Point4` (`KismetMathLibrary.MakeVector` _returnvalue _returnvalue_3))
  (return (`|MakeArray` (`local.Point1`) (`local.Point2`) (`local.Point3`) (`local.Point4`))))

(fn `BoxAndBoxPosition2D`
  (params (BoxOrigin1 :type "Vector Structure") (BoxVertices1 :type "Array of Vector Structure") (BoxVertices2 :type "Array of Vector Structure"))
  (returns (ReturnValue :type String))
  (locals (Outside :type Boolean) (Inside :type Boolean) (Result :type String))
  (bind _returnvalue (`self.PointIsInsidePointArray2D` BoxOrigin1 BoxVertices2))
  (for _array_element BoxVertices1
    (if (not (`self.PointIsInsidePointArray2D` _array_element BoxVertices2))
      (set `local.Outside` true) ; At least one point of box1 is outside box2
      (break)))
  (if (`local.Outside`)
    (for _array_element_2 BoxVertices1
      (if (`self.PointIsInsidePointArray2D` _array_element_2 BoxVertices2)
        (set `local.Inside` true) ; At least one point of box1 is inside of box2
        (break)))
    (if (`local.Inside`)
      (if _returnvalue
        (set `local.Result` "OverlappingInside")
        (else
          (set `local.Result` "OverlappingOutside")))
      (elif _returnvalue
        (set `local.Result` "Box2Inside")
        (else
          (set `local.Result` "NotOverlapping"))))
    (else
      (set `local.Result` "Box1Inside")))
  (return (`local.Result`)))

(fn `BoxAndCirclePosition2D`
  (params (CircleOrigin :type "Vector Structure") (CircleRadius :type "Float (double-precision)") (BoxVertices :type "Array of Vector Structure"))
  (returns (ReturnValue :type String))
  (locals (Outside :type Boolean) (Inside :type Boolean) (Result :type String))
  (for _array_element BoxVertices
    (if (not (`self.PointIsInsideCircle2D` _array_element CircleOrigin CircleRadius))
      (set `local.Outside` true)
      (break)))
  (if (`local.Outside`)
    (for _array_element_2 BoxVertices
      (if (`self.PointIsInsideCircle2D` _array_element_2 CircleOrigin CircleRadius)
        (set `local.Inside` true)
        (break)))
    (if (`local.Inside`)
      (set `local.Result` "Overlapping")
      (elif (`self.PointIsInsidePointArray2D` CircleOrigin BoxVertices)
        (set `local.Result` "CircleInside")
        (else
          (set `local.Result` "NotOverlapping"))))
    (else
      (set `local.Result` "BoxInside")))
  (return (`local.Result`)))

(fn `BoxCanMakeBorder`
  (params (BoxOrigin :type "Vector Structure") (Box :type "Array of Vector Structure") (Border :type "Array of /Game/Blueprints/Structures/Object/StructBox Structure"))
  (returns (ReturnVlaue :type Boolean))
  (locals (Positions :type "Array of String") (Break :type Boolean) (Result :type Boolean))
  (bind _positions (`local.Positions`))
  (bind _break (`local.Break`))
  (for _array_element Border
    (bind _returnvalue (`self.BoxAndBoxPosition2D` BoxOrigin Box (`.Vertex_3_DE9B982649CAFFBA127A5285471A28EB` (break `/Game/Blueprints/Structures/Object/StructBox` _array_element))))
    (if (or (`KismetStringLibrary.EqualEqual_StrStr` _returnvalue "Box1Inside") (`KismetStringLibrary.EqualEqual_StrStr` _returnvalue "Box2Inside") (`KismetStringLibrary.EqualEqual_StrStr` _returnvalue "OverlappingInside"))
      (set `local.Break` true)
      (break)
      (else
        (`KismetArrayLibrary.Array_Add` _positions _returnvalue))))
  (if (not _break)
    (for _array_element_2 _positions
      (if (`KismetStringLibrary.EqualEqual_StrStr` _array_element_2 "OverlappingOutside")
        (set `local.Break` true)
        (break)))
    (if _break
      (set `local.Result` true)))
  (return (`local.Result`)))

(fn `BoxDoesntOverlappAnyonesBorder`
  (params (BoxOrigin :type "Vector Structure") (BoxVertices :type "Array of Vector Structure") (Players :type "Array of /Game/Blueprints/Controllers/PlayerController_Game Object Reference"))
  (returns (ReturnValue :type Boolean))
  (locals (Break :type Boolean))
  (bind _break (`local.Break`))
  (for _array_element Players
    (for _array_element_2 (`/Game/Blueprints/Controllers/PlayerController_Game.BorderStructRef` _array_element)
      (if (`KismetStringLibrary.NotEqual_StrStr` (`self.BoxAndBoxPosition2D` BoxOrigin BoxVertices (`.Vertex_3_DE9B982649CAFFBA127A5285471A28EB` (break `/Game/Blueprints/Structures/Object/StructBox` _array_element_2))) "NotOverlapping")
        (set `local.Break` true)
        (break)))
    (if _break
      (break)))
  (return (not _break)))

(fn `BoxIsInsideBorder`
  (params (BoxOrigin :type "Vector Structure") (Box :type "Array of Vector Structure") (Border :type "Array of /Game/Blueprints/Structures/Object/StructBox Structure"))
  (returns (ReturnVlaue :type Boolean))
  (locals (Result :type Boolean))
  (for _array_element Border
    (if (`KismetStringLibrary.EqualEqual_StrStr` (`self.BoxAndBoxPosition2D` BoxOrigin Box (`.Vertex_3_DE9B982649CAFFBA127A5285471A28EB` (break `/Game/Blueprints/Structures/Object/StructBox` _array_element))) "Box1Inside")
      (set `local.Result` true)
      (break)))
  (return (`local.Result`)))

(fn `BoxIsInsideBox`
  (params (OuterOrigin :type "Vector Structure") (OuterExtent :type "Vector Structure") (InnerOrigin :type "Vector Structure") (InnerExtent :type "Vector Structure"))
  (returns (ReturnValue :type Boolean))
  (bind _returnvalue (`self.BoxVertices` InnerOrigin InnerExtent))
  (bind _returnvalue_2 (`self.BoxVertices` OuterOrigin OuterExtent))
  (bind _output (`|GetArrayItem` _returnvalue_2))
  (bind _output_2 (`|GetArrayItem` _returnvalue_2 1))
  (return (and (`self.PointIsBetweenTwoPoints` (`|GetArrayItem` _returnvalue) _output _output_2) (`self.PointIsBetweenTwoPoints` (`|GetArrayItem` _returnvalue 1) _output _output_2))))

(fn `BoxIsInsideSphere`
  (params (OuterOrigin :type "Vector Structure") (OuterRadius :type "Float (double-precision)") (InnerOrigin :type "Vector Structure") (InnerExtent :type "Vector Structure"))
  (returns (ReturnValue :type Boolean))
  (bind _returnvalue (`self.CircleVertices` OuterOrigin OuterRadius))
  (bind _returnvalue_2 (`self.BoxVertices` InnerOrigin InnerExtent))
  (bind _output (`|GetArrayItem` _returnvalue_2 1))
  (bind _output_2 (`|GetArrayItem` _returnvalue_2))
  (bind _output_3 (`|GetArrayItem` _returnvalue))
  (bind _output_4 (`|GetArrayItem` _returnvalue 1))
  (`KismetSystemLibrary.PrintString` null (`KismetStringLibrary.Concat_StrStr` "Circle vertex0:" (`KismetStringLibrary.Conv_VectorToString` _output_3) " Circle vertex1:" (`KismetStringLibrary.Conv_VectorToString` _output_4) " Box Vertex0:" (`KismetStringLibrary.Conv_VectorToString` _output_2) " Box vertex1:" (`KismetStringLibrary.Conv_VectorToString` _output)) true true (struct :`B` 1.0 :`A` 1.0) 20.0)
  (return (and (`self.PointIsBetweenTwoPoints` _output_2 _output_3 _output_4) (`self.PointIsBetweenTwoPoints` _output _output_3 _output_4))))

(fn `BoxIsInsideSphere2D`
  (params (OuterOrigin :type "Vector Structure") (OuterRadius :type "Float (double-precision)") (InnerOrigin :type "Vector Structure") (InnerSide :type "Float (double-precision)"))
  (returns (ReturnValue :type Boolean))
  (bind _returnvalue (`self.Circle2DVertices` OuterOrigin OuterRadius))
  (bind _returnvalue_2 (`self.Box2DVertices` InnerOrigin InnerSide))
  (bind _output (`|GetArrayItem` _returnvalue))
  (bind _output_2 (`|GetArrayItem` _returnvalue 3))
  (return (and (`self.PointIsBetweenTwoPoints2D` (`|GetArrayItem` _returnvalue_2) _output _output_2) (`self.PointIsBetweenTwoPoints2D` (`|GetArrayItem` _returnvalue_2 1) _output _output_2))))

(fn `BoxVertices`
  (params (Origin :type "Vector Structure") (BoxExtent :type "Vector Structure"))
  (returns (ReturnValue :type "Array of Vector Structure"))
  (locals (Point1 :type "Vector Structure") (Point2 :type "Vector Structure") (Point3 :type "Vector Structure") (Point4 :type "Vector Structure") (Point5 :type "Vector Structure") (Point6 :type "Vector Structure") (Point7 :type "Vector Structure") (Point8 :type "Vector Structure"))
  (bind _x (.x Origin))
  (bind _y (.y Origin))
  (bind _z (.z Origin))
  (bind _x_2 (.x BoxExtent))
  (bind _y_2 (.y BoxExtent))
  (bind _z_2 (.z BoxExtent))
  (set `local.Point1` (`KismetMathLibrary.MakeVector` (- _x _x_2) (- _y _y_2) (- _z _z_2)))
  (set `local.Point2` (`KismetMathLibrary.MakeVector` (+ _x _x_2) (+ _y _y_2) (+ _z _z_2)))
  (return (`|MakeArray` (`local.Point1`) (`local.Point2`))))

(fn `Circle2DVertices`
  (params (Origin :type "Vector Structure") (Radius :type "Float (double-precision)"))
  (returns (ReturnValue :type "Array of Vector Structure"))
  (locals (Point1 :type "Vector Structure") (Point2 :type "Vector Structure") (Point3 :type "Vector Structure") (Point4 :type "Vector Structure") (Point5 :type "Vector Structure") (Point6 :type "Vector Structure") (Point7 :type "Vector Structure") (Point8 :type "Vector Structure"))
  (bind _x (.x Origin))
  (bind _y (.y Origin))
  (bind _returnvalue (- _x Radius))
  (bind _returnvalue_2 (- _y Radius))
  (bind _returnvalue_3 (+ _x Radius))
  (bind _returnvalue_4 (+ _y Radius))
  (set `local.Point1` (`KismetMathLibrary.MakeVector` _returnvalue _returnvalue_2))
  (set `local.Point2` (`KismetMathLibrary.MakeVector` _returnvalue _returnvalue_4))
  (set `local.Point3` (`KismetMathLibrary.MakeVector` _returnvalue_3 _returnvalue_2))
  (set `local.Point4` (`KismetMathLibrary.MakeVector` _returnvalue_3 _returnvalue_4))
  (return (`|MakeArray` (`local.Point1`) (`local.Point2`) (`local.Point3`) (`local.Point4`))))

(fn `CircleVertices`
  (params (Origin :type "Vector Structure") (Radius :type "Float (double-precision)"))
  (returns (ReturnValue :type "Array of Vector Structure"))
  (locals (Point1 :type "Vector Structure") (Point2 :type "Vector Structure") (Point3 :type "Vector Structure") (Point4 :type "Vector Structure") (Point5 :type "Vector Structure") (Point6 :type "Vector Structure") (Point7 :type "Vector Structure") (Point8 :type "Vector Structure"))
  (bind _x (.x Origin))
  (bind _y (.y Origin))
  (bind _z (.z Origin))
  (set `local.Point1` (`KismetMathLibrary.MakeVector` (- _x Radius) (- _y Radius) (- _z Radius)))
  (set `local.Point2` (`KismetMathLibrary.MakeVector` (+ _x Radius) (+ _y Radius) (+ _z Radius)))
  (return (`|MakeArray` (`local.Point1`) (`local.Point2`))))

(fn `Delta`
  (params (A :type "Float (double-precision)") (B :type "Float (double-precision)") (C :type "Float (double-precision)"))
  (returns (ReturnValue :type "Float (double-precision)"))
  (return (- (`KismetMathLibrary.Square` B) (* A C 4.0))))

(fn `GetDirectionFromSceneComponent`
  (params (ScenceComponent :type "SceneComponent Object Reference"))
  (returns (Direction :type "Vector Structure"))
  (return (`KismetMathLibrary.Conv_RotatorToVector` (`KismetMathLibrary.MakeRotator` (.roll (`SceneComponent.K2_GetComponentRotation` ScenceComponent)) (.pitch (`SceneComponent.K2_GetComponentRotation` ScenceComponent)) (+ (.yaw (`SceneComponent.K2_GetComponentRotation` ScenceComponent)) 0.0)))))

(fn `MeleeAttackPoint`
  (params (TargetLocation :type "Vector Structure") (CharacterLocation :type "Vector Structure") (WeaponRadius :type "Float (double-precision)"))
  (returns (ReturnValue :type "Vector Structure"))
  (locals (GD :type "Float (double-precision)"))
  (bind _gd (`local.GD`))
  (set `local.GD` (`self.VectorLenghth2D` TargetLocation CharacterLocation))
  (return (`KismetMathLibrary.MakeVector` (`self.ValueFinder` (.x TargetLocation) (.x CharacterLocation) _gd WeaponRadius) (`self.ValueFinder` (.y TargetLocation) (.y CharacterLocation) _gd WeaponRadius) (.z TargetLocation))))

(fn `PointIsBetweenTwoPoints`
  (params (Point :type "Vector Structure") (MinLimit :type "Vector Structure") (MaxLimit :type "Vector Structure"))
  (returns (ReturnValue :type Boolean))
  (bind _x (.x Point))
  (bind _y (.y Point))
  (bind _z (.z Point))
  (return (and (>= _x (.x MinLimit)) (>= _y (.y MinLimit)) (>= _z (.z MinLimit)) (<= _x (.x MaxLimit)) (<= _y (.y MaxLimit)) (<= _z (.z MaxLimit)))))

(fn `PointIsBetweenTwoPoints2D`
  (params (Point :type "Vector Structure") (MinLimit :type "Vector Structure") (MaxLimit :type "Vector Structure"))
  (returns (ReturnValue :type Boolean))
  (bind _x (.x Point))
  (bind _y (.y Point))
  (return (and (>= _x (.x MinLimit)) (>= _y (.y MinLimit)) (<= _x (.x MaxLimit)) (<= _y (.y MaxLimit)))))

(fn `PointIsInsideCircle2D`
  (params (Point :type "Vector Structure") (CircleOrigin :type "Vector Structure") (CircleRadius :type "Float (double-precision)"))
  (returns (ReturnValue :type Boolean))
  (bind _x (.x CircleOrigin))
  (bind _y (.y CircleOrigin))
  (bind _x_2 (.x Point))
  (bind _y_2 (.y Point))
  (return (and (>= _x_2 (- _x CircleRadius)) (<= _x_2 (+ _x CircleRadius)) (>= _y_2 (- _y CircleRadius)) (<= _y_2 (+ _y CircleRadius)))))

(fn `PointIsInsidePointArray2D`
  (params (Point :type "Vector Structure") (PointArray :type "Array of Vector Structure"))
  (returns (ReturnValue :type Boolean))
  (bind _returnvalue (`self.XArrayOfPoints` PointArray))
  (bind _returnvalue_2 (`self.YArrayOfPoints` PointArray))
  (bind _x (.x Point))
  (bind _y (.y Point))
  (return (and (>= _x (`.MinValue` (`KismetMathLibrary.MinOfFloatArray` _returnvalue))) (>= _y (`.MinValue` (`KismetMathLibrary.MinOfFloatArray` _returnvalue_2))) (<= _x (`.MaxValue` (`KismetMathLibrary.MaxOfFloatArray` _returnvalue))) (<= _y (`.MaxValue` (`KismetMathLibrary.MaxOfFloatArray` _returnvalue_2))))))

(fn `QuadraticEquation`
  (params (A :type "Float (double-precision)") (B :type "Float (double-precision)") (C :type "Float (double-precision)"))
  (returns (HasValue :type Boolean) (X1 :type "Float (double-precision)") (X2 :type "Float (double-precision)"))
  (locals (Delt :type "Float (double-precision)") (OutX1 :type "Float (double-precision)") (OutX2 :type "Float (double-precision)"))
  (bind _returnvalue (* B -1.0))
  (bind _returnvalue_2 (* A 2.0))
  (bind _delt (`local.Delt`))
  (bind _returnvalue_3 (>= _delt 0.0))
  (bind _returnvalue_4 (`KismetMathLibrary.Sqrt` _delt))
  (set `local.Delt` (`self.Delta` A B C))
  (if _returnvalue_3
    (set `local.OutX1` (/ (+ _returnvalue _returnvalue_4) _returnvalue_2))
    (set `local.OutX2` (/ (- _returnvalue _returnvalue_4) _returnvalue_2)))
  (return _returnvalue_3 (`local.OutX1`) (`local.OutX2`)))

(fn `RandomArray`
  (params (Total :type Integer) (OccurnessArray :type "Array of Integer"))
  (returns (ReturnValue :type "Array of Integer"))
  (locals (OccurnessCount :type Integer) (SelectionArray :type "Array of Integer") (Occurness :type "Array of Integer") (OutInteger :type "Array of Integer") (OccurenessIndex :type Integer))
  (bind _occurness (`local.Occurness`))
  (bind _selectionarray (`local.SelectionArray`))
  (set `local.SelectionArray` OccurnessArray)
  (set `local.OccurnessCount` (/ Total (`KismetArrayLibrary.Array_Length` OccurnessArray)))
  (for _ (range (`KismetArrayLibrary.Array_Length` _selectionarray))
    (`KismetArrayLibrary.Array_Add` _occurness))
  (while (> (`KismetArrayLibrary.Array_Length` _selectionarray) 0)
    (bind _output_get (set `local.OccurenessIndex` (`KismetMathLibrary.RandomIntegerInRange` 0 (- (`KismetArrayLibrary.Array_Length` _selectionarray) 1))))
    (`KismetArrayLibrary.Array_Add` (`local.OutInteger`) (`|GetArrayItem` _selectionarray _output_get))
    (bind _result (`/Engine/EditorBlueprintResources/StandardMacros.IncrementInt` (`|GetArrayItem` _occurness _output_get))
      (:`  `
        (if (>= _result (`local.OccurnessCount`))
          (`KismetArrayLibrary.Array_Remove` _selectionarray _output_get)
          (`KismetArrayLibrary.Array_Remove` _occurness _output_get)))))
  (return (`local.OutInteger`)))

(fn `RandomIntegerFromOneArray`
  (params (Array :type "Array of Integer"))
  (returns (ReturnValue :type Integer))
  (return (`|GetArrayItem` Array (`KismetMathLibrary.RandomIntegerInRange` 0 (- (`KismetArrayLibrary.Array_Length` Array) 1)))))

(fn `RandomIntegerFromTwoArrays`
  (params (Array1 :type "Array of Integer") (Array2 :type "Array of Integer"))
  (returns (Value1 :type Integer) (Value2 :type Integer) (Index :type Integer))
  (bind _returnvalue (`KismetMathLibrary.RandomIntegerInRange` 0 (- (`KismetArrayLibrary.Array_Length` Array1) 1)))
  (return (`|GetArrayItem` Array1 _returnvalue) (`|GetArrayItem` Array2 _returnvalue) _returnvalue))

(fn `ValueFinder`
  (params (v1 :type "Float (double-precision)") (v2 :type "Float (double-precision)") (GD :type "Float (double-precision)") (SD :type "Float (double-precision)"))
  (returns (v :type "Float (double-precision)"))
  (return (+ v2 (/ (* (- v1 v2) (- GD SD)) GD))))

(fn `VectorLenghth2D`
  (params (Point1 :type "Vector Structure") (Point2 :type "Vector Structure"))
  (returns (ReturnValue :type "Float (double-precision)"))
  (bind _returnvalue (- (.x Point1) (.x Point2)))
  (bind _returnvalue_2 (- (.y Point1) (.y Point2)))
  (return (`KismetMathLibrary.Sqrt` (+ (* _returnvalue _returnvalue) (* _returnvalue_2 _returnvalue_2)))))

(fn `XArrayOfPoints`
  (params (PointArray :type "Array of Vector Structure"))
  (returns (ReturnValue :type "Array of Float (double-precision)"))
  (locals (XArray :type "Array of Float (double-precision)"))
  (for _array_element PointArray
    (`KismetArrayLibrary.Array_Add` (`local.XArray`) (.x _array_element)))
  (return (`local.XArray`)))

(fn `YArrayOfPoints`
  (params (PointArray :type "Array of Vector Structure"))
  (returns (ReturnValue :type "Array of Float (double-precision)"))
  (locals (YArray :type "Array of Float (double-precision)"))
  (for _array_element PointArray
    (`KismetArrayLibrary.Array_Add` (`local.YArray`) (.y _array_element)))
  (return (`local.YArray`)))