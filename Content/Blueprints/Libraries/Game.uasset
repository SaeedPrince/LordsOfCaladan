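; Game-wide helper library of unrelated utility functions for UI, jobs, population and mine flags.
; It creates widgets with their owning player stored as controller reference and builds blank job structs for movement and work IDs.
; It also returns the last true index in a bool array, finds a person by residence or worker index, and maps mine product IDs to flag meshes.
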(fn `BoolMax`
  (params (BoolArray :type "Array of Boolean"))
  (returns (ReturnValue :type Integer))
  (locals (OutMax :type Integer :default -1))
  (for (_array_element _array_index) BoolArray
    (if _array_element
      (set `local.OutMax` _array_index)))
  (return (`local.OutMax`)))

(fn `CreateGameWidget`
  (params (Class :type "/Game/Blueprints/Widgets/Widget_ParentGame Class Reference") (Player :type "/Game/Blueprints/Controllers/PlayerController_Game Object Reference"))
  (returns (ReturnValue :type "/Game/Blueprints/Widgets/Widget_ParentGame Object Reference"))
  (bind _returnvalue (`|CreateWidget` Class Player))
  (set `/Game/Blueprints/Widgets/Widget_ParentGame.ControllerRef` Player _returnvalue)
  (return _returnvalue))

(fn `CreateJob`
  (params (JobID :type Integer))
  (returns (ReturnValue :type "/Game/Blueprints/Structures/Game/StructJob Structure"))
  (locals (OutJob :type "/Game/Blueprints/Structures/Game/StructJob Structure"))
  (switch `int` JobID
    (:`0`
      (set `local.OutJob` (make `/Game/Blueprints/Structures/Game/StructJob` 0)) ; Go to home
    )
    (:`1`
      (set `local.OutJob` (make `/Game/Blueprints/Structures/Game/StructJob` 1)) ; Go to rallypoint
    )
    (:`2`
      (set `local.OutJob` (make `/Game/Blueprints/Structures/Game/StructJob` 2)) ; Go to Destination
    )
    (:`3`
      (set `local.OutJob` (make `/Game/Blueprints/Structures/Game/StructJob` 3)) ; Work as career
    )
    (:`4`
      (set `local.OutJob` (make `/Game/Blueprints/Structures/Game/StructJob` 4)) ; Work as worker
    ))
  (return (`local.OutJob`)))

(fn `FindPersonInPersonArray`
  (params (Index :type Integer) (PersonArray :type "Array of /Game/Blueprints/Controllers/AIController_Game Object Reference") (ArrayName :type String))
  (returns (Found :type Boolean) (Person :type "/Game/Blueprints/Controllers/AIController_Game Object Reference"))
  (locals (OutBool :type Boolean) (OutIndex :type "/Game/Blueprints/Controllers/AIController_Game Object Reference"))
  (for _array_element PersonArray
    (switch `string` ArrayName
      (:`Residence`
        (if (== (`/Game/Blueprints/Controllers/AIController_Game.IndexInResidence` _array_element) Index)
          (set `local.OutBool` true :!label _label)
          (set `local.OutIndex` _array_element)
          (break)))
      (:`Work`
        (if (== Index (`/Game/Blueprints/Controllers/AIController_Game.IndexInWorker` _array_element))
          (goto _label)))))
  (return (`local.OutBool`) (`local.OutIndex`)))

(fn `FlagMesh`
  (params (Product :type Integer))
  (returns (ReturnValue :type "SkeletalMesh Object Reference"))
  (locals (OutMesh :type "SkeletalMesh Object Reference"))
  (switch `int` Product
    (:`19`
      (set `local.OutMesh` "/Game/Assets/SkeletalMeshes/A_Flag_IronMine.A_Flag_IronMine"))
    (:`20`
      (set `local.OutMesh` "/Game/Assets/SkeletalMeshes/A_Flag_GoldMine.A_Flag_GoldMine"))
    (:`21`
      (set `local.OutMesh` "/Game/Assets/SkeletalMeshes/A_Flag_CopperMine.A_Flag_CopperMine"))
    (:`22`
      (set `local.OutMesh` "/Game/Assets/SkeletalMeshes/A_Flag_CoalMine.A_Flag_CoalMine"))
    (:`23`
      (set `local.OutMesh` "/Game/Assets/SkeletalMeshes/A_Flag_SulfurMine.A_Flag_SulfurMine")))
  (return (`local.OutMesh`)))