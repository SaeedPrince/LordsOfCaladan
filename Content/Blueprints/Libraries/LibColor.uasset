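; Blueprint function library of color helpers that convert between color names and linear colors and apply colors to primitive components.
; Name lookup covers primary and secondary colors plus white, while the reverse lookup tests each RGB channel for exactly 1.0 and can also return Black.
; The two setter functions create a dynamic material instance on element 0 and set a named vector parameter, from either a name or a linear color.
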(fn `GetColorByString`
  (params (Color :type String))
  (returns (ReturnValue :type "LinearColor Structure"))
  (locals (OutColor :type "LinearColor Structure"))
  (switch `string` Color
    (:`Red`
      (set `local.OutColor` (make `LinearColor` 1.0 0.0 0.0 1.0)))
    (:`Green`
      (set `local.OutColor` (make `LinearColor` 0.0 1.0 0.0 1.0)))
    (:`Blue`
      (set `local.OutColor` (make `LinearColor` 0.0 0.0 1.0 1.0)))
    (:`Yellow`
      (set `local.OutColor` (make `LinearColor` 1.0 1.0 0.0 1.0)))
    (:`Cyan`
      (set `local.OutColor` (make `LinearColor` 0.0 1.0 1.0 1.0)))
    (:`Purple`
      (set `local.OutColor` (make `LinearColor` 1.0 0.0 1.0 1.0)))
    (:`White`
      (set `local.OutColor` (make `LinearColor` 1.0 1.0 1.0 1.0))))
  (return (`local.OutColor`)))

(fn `GetColorName`
  (params (Color :type "LinearColor Structure"))
  (returns (ReturnValue :type String))
  (locals (OutString :type String))
  (bind (_r _g _b) (break `LinearColor` Color))
  (bind _returnvalue (== _g 1.0))
  (bind _returnvalue_2 (== _b 1.0))
  (if (== _r 1.0)
    (if _returnvalue
      (if _returnvalue_2
        (set `local.OutString` "White")
        (else
          (set `local.OutString` "Yellow")))
      (elif _returnvalue_2
        (set `local.OutString` "Purple")
        (else
          (set `local.OutString` "Red"))))
    (elif _returnvalue
      (if _returnvalue_2
        (set `local.OutString` "Cyan")
        (else
          (set `local.OutString` "Green")))
      (elif _returnvalue_2
        (set `local.OutString` "Blue")
        (else
          (set `local.OutString` "Black")))))
  (return (`local.OutString`)))

(fn `SetComponentColorByLinearColor`
  (params (PrimitiveComponent :type "PrimitiveComponent Object Reference") (Parameter :type Name) (Color :type "LinearColor Structure"))
  (bind _returnvalue (`PrimitiveComponent.CreateDynamicMaterialInstance` PrimitiveComponent 0 null))
  (`MaterialInstanceDynamic.SetVectorParameterValue` _returnvalue Parameter Color))

(fn `SetComponentColorByString`
  (params (PrimitiveComponent :type "PrimitiveComponent Object Reference") (Parameter :type Name) (Color :type String))
  (bind _returnvalue (`PrimitiveComponent.CreateDynamicMaterialInstance` PrimitiveComponent 0 null))
  (`MaterialInstanceDynamic.SetVectorParameterValue` _returnvalue Parameter (`self.GetColorByString` Color)))