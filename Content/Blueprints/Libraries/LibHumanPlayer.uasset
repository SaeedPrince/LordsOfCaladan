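; Blueprint helper library for the human player that resolves camera switching between first-person, third-person and strategy modes.
; ActiveCameraDefine maps the requested mode to the player's camera to activate, the one to deactivate, and an OwnerNoSee flag set only in first person.
; Each mode deactivates just one fixed camera, implying a Strategy, Third Person, First Person cycle.
; It only returns these values, without applying them.
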(fn `ActiveCameraDefine`
  (params (CameraMode :type "/Game/Blueprints/Enums/EnumCameraMode Enum" :default "NewEnumerator0") (HumanPlayer :type "/Game/Blueprints/Characters/HumanPlayer Object Reference"))
  (returns (CamToDeactive :type "SceneComponent Object Reference") (CamToActive :type "SceneComponent Object Reference") (OwnerNoSee :type Boolean))
  (locals (OutBool :type Boolean) (OutScene1 :type "SceneComponent Object Reference") (OutScene2 :type "SceneComponent Object Reference"))
  (bind _camtps (`/Game/Blueprints/Characters/HumanPlayer.CamTps` HumanPlayer))
  (bind _camfps (`/Game/Blueprints/Characters/HumanPlayer.CamFps` HumanPlayer))
  (bind _camrts (`/Game/Blueprints/Characters/HumanPlayer.CamRts` HumanPlayer))
  (switch `/Game/Blueprints/Enums/EnumCameraMode` CameraMode
    (:`NewEnumerator0`
      (set `local.OutScene1` _camtps)
      (set `local.OutScene2` _camfps)
      (set `local.OutBool` true))
    (:`NewEnumerator1`
      (set `local.OutScene1` _camrts)
      (set `local.OutScene2` _camtps)
      (set `local.OutBool` false))
    (:`NewEnumerator2`
      (set `local.OutScene1` _camfps)
      (set `local.OutScene2` _camrts)
      (set `local.OutBool` false)))
  (return (`local.OutScene1`) (`local.OutScene2`) (`local.OutBool`)))