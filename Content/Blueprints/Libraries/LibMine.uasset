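; LibMine is a Blueprint function library of lookup helpers for mines and the resources they produce.
; MineName switches on a production ID for iron, gold, copper, coal or sulfur and appends "Mine" to the resource word to build the mine's name.
; MineIDbyNum maps a contiguous range of numeric production indices to the matching ore item.
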(fn `MineIDbyNum`
  (params (ProductionIndex :type Integer))
  (returns (ReturnValue :type "/Game/Blueprints/Enums/EnumItem Enum"))
  (locals (OutItem :type "/Game/Blueprints/Enums/EnumItem Enum"))
  (switch `int` ProductionIndex
    (:`19`
      (set `local.OutItem` "NewEnumerator19"))
    (:`20`
      (set `local.OutItem` "NewEnumerator34"))
    (:`21`
      (set `local.OutItem` "NewEnumerator35"))
    (:`22`
      (set `local.OutItem` "NewEnumerator20"))
    (:`23`
      (set `local.OutItem` "NewEnumerator21")))
  (return (`local.OutItem`)))

(fn `MineName`
  (params (ProductionID :type "/Game/Blueprints/Enums/EnumItem Enum" :default "NewEnumerator0"))
  (returns (ReturnValue :type String))
  (locals (OutString :type String))
  (switch `/Game/Blueprints/Enums/EnumItem` ProductionID
    (:`NewEnumerator19`
      (set `local.OutString` "Iron"))
    (:`NewEnumerator34`
      (set `local.OutString` "Gold"))
    (:`NewEnumerator35`
      (set `local.OutString` "Copper"))
    (:`NewEnumerator20`
      (set `local.OutString` "Coal"))
    (:`NewEnumerator21`
      (set `local.OutString` "Sulfur")))
  (return (`KismetStringLibrary.Concat_StrStr` (`local.OutString`) " Mine")))