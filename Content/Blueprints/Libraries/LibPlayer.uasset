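; Player helper library for garrison UI, soldier recruitment checks and cursor-driven orders.
; Warrior and archer creation each require a free military place, an idle human and their equipment in stock.
; Garrison slot colors derive from resident occupancy: red empty, yellow assigned but away, green present.
; Cursor helpers trace by object type and turn a given building or human actor into an order struct.
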(fn `BottomButtonColorArray`
  (params (Building :type "/Game/Assets/BP_Meshes/Architecture/BP_House Object Reference"))
  (returns (Military :type "Array of LinearColor Structure") (Civilian :type "Array of LinearColor Structure"))
  (locals (OutColor :type "Array of LinearColor Structure"))
  (bind _outcolor (`local.OutColor`))
  (set `local.OutColor` (`self.MakeColorArray` (* (`/Game/Assets/BP_Meshes/Architecture/BP_House.FlagCount` Building) (`/Game/Assets/BP_Meshes/Architecture/BP_House.MilitPlacePerFlag` Building))))
  (bind (_occupiedarray _isatplacearray) (`self.MilitExistenceArray` Building))
  (for _index (range (`KismetArrayLibrary.Array_Length` _outcolor))
    (if (`|GetArrayItem` _occupiedarray _index)
      (if (`|GetArrayItem` _isatplacearray _index)
        (bind _output (`|GetArrayItem` _outcolor _index))
        (setmembers `LinearColor` :`StructRef` _output :`R` 0.0 :`G` 1.0)
        (else
          (setmembers `LinearColor` :`StructRef` _output :`G` 1.0)))))
  (return (`local.OutColor`)))

(fn `GetUnderCursor`
  (params (PlayerController :type "PlayerController Object Reference") (ObjectTypes :type "Array of EObjectTypeQuery Enum (by ref)" :default _))
  (returns (ReturnValue :type "/Game/Blueprints/Structures/Game/StructUnderCursor Structure"))
  (locals (OutStruct :type "/Game/Blueprints/Structures/Game/StructUnderCursor Structure"))
  (bind (_hitresult _returnvalue) (`PlayerController.GetHitResultUnderCursorForObjects` PlayerController ObjectTypes true))
  (bind (_bblockinghit _binitialoverlap _time _distance _location _impactpoint _normal _impactnormal _physmat _hitactor) (`GameplayStatics.BreakHitResult` _hitresult))
  (if _returnvalue
    (set `local.OutStruct` (make `/Game/Blueprints/Structures/Game/StructUnderCursor` true _location _hitactor)))
  (return (`local.OutStruct`)))

(fn `IsBuilding`
  (params (Actor :type "Actor Object Reference"))
  (returns (Yes :type Boolean) (BuildingRef :type "/Game/Assets/BP_Meshes/Architecture/BP_House Object Reference"))
  (locals (OutBool :type Boolean))
  (bind _asbp_house (cast `/Game/Assets/BP_Meshes/Architecture/BP_House` Actor)
    (:`then`
      (set `local.OutBool` true))
    (:`CastFailed`
      (set `local.OutBool` false)))
  (return (`local.OutBool`) _asbp_house))

(fn `IsHumanCharacter`
  (params (Actor :type "Actor Object Reference"))
  (returns (Yes :type Boolean) (CharacterRef :type "/Game/Blueprints/Characters/HumanBP Object Reference"))
  (locals (OutBool :type Boolean))
  (bind _ashuman_bp (cast `/Game/Blueprints/Characters/HumanBP` Actor)
    (:`then`
      (set `local.OutBool` true))
    (:`CastFailed`
      (set `local.OutBool` false)))
  (return (`local.OutBool`) _ashuman_bp))

(fn `MakeBoolArray`
  (params (ArrayCount :type Integer))
  (returns (ReturnValue :type "Array of Boolean"))
  (locals (OutArray :type "Array of Boolean"))
  (bind _outarray (`local.OutArray`))
  (for _ (range ArrayCount)
    (`KismetArrayLibrary.Array_Add` _outarray))
  (return _outarray))

(fn `MakeColorArray`
  (params (ArrayCount :type Integer))
  (returns (ReturnValue :type "Array of LinearColor Structure"))
  (locals (OutArray :type "Array of LinearColor Structure"))
  (bind _outarray (`local.OutArray`))
  (for _ (range ArrayCount)
    (`KismetArrayLibrary.Array_Add` _outarray (struct :`R` 1.0 :`A` 1.0)))
  (return _outarray))

(fn `MilitExistenceArray`
  (params (Building :type "/Game/Assets/BP_Meshes/Architecture/BP_House Object Reference"))
  (returns (OccupiedArray :type "Array of Boolean") (IsAtPlaceArray :type "Array of Boolean"))
  (locals (IsAtPlace :type "Array of Boolean") (Occupied :type "Array of Boolean"))
  (bind _output_get (set `local.IsAtPlace` (`self.MakeBoolArray` (* (`/Game/Assets/BP_Meshes/Architecture/BP_House.FlagCount` Building) (`/Game/Assets/BP_Meshes/Architecture/BP_House.MilitPlacePerFlag` Building)))))
  (set `local.Occupied` _output_get)
  (for _array_element (`/Game/Assets/BP_Meshes/Architecture/BP_House.MilitResident` Building)
    (bind _indexingarrison (`/Game/Blueprints/Controllers/AIController_Game.IndexInGarrison` _array_element))
    (`|VariableSetRef` (`|GetArrayItem` (`local.Occupied`) _indexingarrison) true)
    (`|VariableSetRef` (`|GetArrayItem` (`local.IsAtPlace`) _indexingarrison) (`/Game/Blueprints/Controllers/AIController_Game.IsAtGarrison` _array_element)))
  (return (`local.Occupied`) (`local.IsAtPlace`)))

(fn `OrderByUnderCursor`
  (params (Actor :type "Actor Object Reference"))
  (returns (ReturnValue :type "/Game/Blueprints/Structures/Game/StructOrder Structure"))
  (locals (OutOrder :type "/Game/Blueprints/Structures/Game/StructOrder Structure"))
  (bind (_yes _buildingref) (`self.IsBuilding` Actor))
  (bind (_yes_2 _characterref) (`self.IsHumanCharacter` Actor))
  (if _yes
    (set `local.OutOrder` (make `/Game/Blueprints/Structures/Game/StructOrder` :`ID` "NewEnumerator2" :`TargetActor` _buildingref))
    (elif _yes_2
      (set `local.OutOrder` (make `/Game/Blueprints/Structures/Game/StructOrder` :`ID` "NewEnumerator1" :`TargetActor` _characterref))))
  (return (`local.OutOrder`)))

(fn `SoldierCreationPossibility`
  (params (BuildingArray :type "Array of /Game/Assets/BP_Meshes/Architecture/BP_House Object Reference") (IdlePool :type "Array of /Game/Blueprints/Controllers/AIController_Game Object Reference"))
  (returns (Warrior :type Boolean) (Archer :type Boolean))
  (locals (BowItemIndex :type Integer :default 18) (QuiverItemIndex :type Integer :default 33) (SwordItemIndex :type Integer :default 12) (ShieldItemIndex :type Integer :default 13))
  (bind _returnvalue (`/Game/Blueprints/Libraries/LibBuilding.MilitaryFreePlaceAvailable` BuildingArray))
  (bind _returnvalue_2 (> (`KismetArrayLibrary.Array_Length` IdlePool) 0))
  (return (and _returnvalue _returnvalue_2 (`/Game/Blueprints/Libraries/LibBuilding.ItemAvailableInStack` (`local.SwordItemIndex`) BuildingArray) (`/Game/Blueprints/Libraries/LibBuilding.ItemAvailableInStack` (`local.ShieldItemIndex`) BuildingArray)) (and _returnvalue _returnvalue_2 (`/Game/Blueprints/Libraries/LibBuilding.ItemAvailableInStack` (`local.BowItemIndex`) BuildingArray) (`/Game/Blueprints/Libraries/LibBuilding.ItemAvailableInStack` (`local.QuiverItemIndex`) BuildingArray))))