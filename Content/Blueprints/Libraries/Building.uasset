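; Blueprint function library that summarizes a building's available items for an inventory widget.
; BuildingInventory loops over the items, tallies each into per-category weapon, material and food count arrays, flags which categories are present, and returns a widget inventory struct.
; ItemIndexInCategory maps global item indices to category-local slots through a hardcoded switch; items matching no category print an on-screen error.
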(fn `BuildingInventory`
  (params (BuildingRef :type "/Game/Assets/BP_Meshes/Architecture/BP_House Object Reference"))
  (returns (ReturnValue :type "/Game/Blueprints/Structures/Game/StructWidgetInventory Structure"))
  (locals (NumWeapon :type "Array of Integer") (NumMaterial :type "Array of Integer") (NumFood :type "Array of Integer") (BoolWeapon :type Boolean) (BoolMatreial :type Boolean) (BoolFood :type Boolean))
  (for _array_element (`/Game/Assets/BP_Meshes/Architecture/BP_House.AvailableItems` BuildingRef)
    (bind (_weapon _material _food) (`self.ItemIndexInCategory` (`/Game/Assets/BP_Meshes/Item/BP_Item.Index` _array_element)))
    (if (!= _weapon -1)
      (`/Engine/EditorBlueprintResources/StandardMacros.IncrementInt` (`|GetArrayItem` (`local.NumWeapon`) _weapon)
        (:`  `
          (set `local.BoolWeapon` true)))
      (elif (!= _material -1)
        (`/Engine/EditorBlueprintResources/StandardMacros.IncrementInt` (`|GetArrayItem` (`local.NumMaterial`) _material)
          (:`  `
            (set `local.BoolMatreial` true)))
        (elif (!= _food -1)
          (`/Engine/EditorBlueprintResources/StandardMacros.IncrementInt` (`|GetArrayItem` (`local.NumFood`) _food)
            (:`  `
              (set `local.BoolFood` true)))
          (else
            (`KismetSystemLibrary.PrintString` null "Error in building inventory" true true (struct :`R` 1.0 :`A` 1.0) 10.0))))))
  (return (make `/Game/Blueprints/Structures/Game/StructWidgetInventory` (`local.BoolWeapon`) (`local.BoolMatreial`) (`local.BoolFood`) (`local.NumWeapon`) (`local.NumMaterial`) (`local.NumFood`))))

(fn `ItemIndexInCategory`
  (params (ItemIndex :type Integer))
  (returns (Weapon :type Integer) (Material :type Integer) (Food :type Integer))
  (locals (OutWeapon :type Integer :default -1) (OutMaterial :type Integer :default -1) (OutFood :type Integer :default -1))
  (switch `int` ItemIndex
    (:`0`
      (set `local.OutMaterial` 0))
    (:`1`
      (set `local.OutMaterial` 1))
    (:`2`
      (set `local.OutMaterial` 2))
    (:`3`
      (set `local.OutFood` 0))
    (:`4`
      (set `local.OutFood` 1))
    (:`5`
      (set `local.OutFood` 2))
    (:`6`
      (set `local.OutFood` 3))
    (:`7`
      (set `local.OutFood` 4))
    (:`8`
      (set `local.OutFood` 5))
    (:`9`
      (set `local.OutFood` 6))
    (:`10`
      (set `local.OutFood` 7))
    (:`11`
      (set `local.OutFood` 8))
    (:`12`
      (set `local.OutWeapon` 0))
    (:`13`
      (set `local.OutWeapon` 1))
    (:`14`
      (set `local.OutWeapon` 2))
    (:`15`
      (set `local.OutWeapon` 3))
    (:`16`
      (set `local.OutWeapon` 4))
    (:`17`
      (set `local.OutWeapon` 5))
    (:`18`
      (set `local.OutWeapon` 6))
    (:`19`
      (set `local.OutMaterial` 3))
    (:`20`
      (set `local.OutMaterial` 4))
    (:`21`
      (set `local.OutMaterial` 5))
    (:`22`
      (set `local.OutMaterial` 6))
    (:`23`
      (set `local.OutMaterial` 7))
    (:`24`
      (set `local.OutMaterial` 8))
    (:`25`
      (set `local.OutWeapon` 7))
    (:`26`
      (set `local.OutWeapon` 8))
    (:`27`
      (set `local.OutWeapon` 9))
    (:`28`
      (set `local.OutMaterial` 9))
    (:`29`
      (set `local.OutMaterial` 10))
    (:`30`
      (set `local.OutMaterial` 11))
    (:`31`
      (set `local.OutMaterial` 12))
    (:`32`
      (set `local.OutMaterial` 13))
    (:`33`
      (set `local.OutWeapon` 10))
    (:`34`
      (set `local.OutMaterial` 14))
    (:`35`
      (set `local.OutWeapon` 11)))
  (return (`local.OutWeapon`) (`local.OutMaterial`) (`local.OutFood`)))