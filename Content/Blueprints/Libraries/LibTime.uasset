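; Time helper library for an in-game clock with separate day and night pacing.
; AddOneScaledSecond advances a DateTime by NightTimeScale or DayTimeScale seconds, depending on whether its hour falls in the night or day window.
; AlphabetMonth converts a month number into its three-letter English abbreviation.
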(fn `AddOneScaledSecond`
  (params (InputTime :type "DateTime Structure"))
  (returns (ReturnValue :type "DateTime Structure"))
  (locals (DayTimeScale :type Integer :default 144) (NightTimeScale :type Integer :default 288) (TimeAdd :type "Timespan Structure"))
  (bind (_year _month _day _hour) (`KismetMathLibrary.BreakDateTime` InputTime))
  (if (or (< _hour 7) (> _hour 17))
    (set `local.TimeAdd` (`KismetMathLibrary.MakeTimespan` 0 0 0 (`local.NightTimeScale`)))
    (else
      (set `local.TimeAdd` (`KismetMathLibrary.MakeTimespan` 0 0 0 (`local.DayTimeScale`)))))
  (return (+ InputTime (`local.TimeAdd`))))

(fn `AlphabetMonth`
  (params (InputMonth :type Integer))
  (returns (ReturnValue :type String))
  (locals (OutString :type String))
  (switch `int` InputMonth
    (:`1`
      (set `local.OutString` "Jan"))
    (:`2`
      (set `local.OutString` "Feb"))
    (:`3`
      (set `local.OutString` "Mar"))
    (:`4`
      (set `local.OutString` "Apr"))
    (:`5`
      (set `local.OutString` "May"))
    (:`6`
      (set `local.OutString` "Jun"))
    (:`7`
      (set `local.OutString` "Jul"))
    (:`8`
      (set `local.OutString` "Aug"))
    (:`9`
      (set `local.OutString` "Sep"))
    (:`10`
      (set `local.OutString` "Oct"))
    (:`11`
      (set `local.OutString` "Nov"))
    (:`12`
      (set `local.OutString` "Dec")))
  (return (`local.OutString`)))