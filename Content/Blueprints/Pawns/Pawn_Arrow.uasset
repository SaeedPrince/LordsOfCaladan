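; Pawn_Arrow is a projectile arrow that flies via its ProjectileMovement component and removes itself shortly after spawning.
; The construction script sets the arrow mesh's world rotation and the projectile's initial speed and velocity from the ArrowRotation, ArrowSpeed and ArrowVelocity variables.
; On BeginPlay, a fixed delay of a few seconds runs before the actor destroys itself, with no hit or damage logic in its graphs.
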(event `self.ReceiveBeginPlay`
  (`KismetSystemLibrary.Delay` 4.0)
  (`self.K2_DestroyActor`))

(fn `UserConstructionScript`
  (bind _projectilemovement (`self.ProjectileMovement`))
  (`SceneComponent.K2_SetWorldRotation` (`self.ArrowMesh`) (`self.ArrowRotation`) false false)
  (set `ProjectileMovementComponent.InitialSpeed` (`self.ArrowSpeed`) _projectilemovement)
  (set `MovementComponent.Velocity` (`self.ArrowVelocity`) _projectilemovement))