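; Server-authoritative flying arrow projectile that sticks into human pawns on hit and despawns after a timeout if it misses.
; Each Tick the server multicasts a velocity-derived rotation correction and red debug trail lines.
; Collider overlap with an attachable HumanBP component spawns a StaticArrow on that component's socket, applies hit effects and destroys the projectile.
; The sphere-trace OverlapSearch duplicates this hit logic, but its timer is never run.
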(event `self.ReceiveBeginPlay`
  ;[1 1 0] Destroy if doesn't hit
  (`/Engine/EditorBlueprintResources/ActorMacros.Switch Has Authority`
    (:`Authority`
      (`KismetSystemLibrary.Delay` 6.0)
      (if (`self.DoOnce`)
        (`self.K2_DestroyActor`)))))

(event `self.ReceiveTick`
  (params (DeltaSeconds :type "Float (single-precision)"))
  (bind _returnvalue (`SceneComponent.K2_GetComponentLocation` (`self.ArrowLocation`)))
  ;[1 1 0] Arrow rotation fix
  (`/Engine/EditorBlueprintResources/ActorMacros.Switch Has Authority`
    (:`Authority`
      (`self.MulticastArrowRotation` (`KismetMathLibrary.MakeRotator` (* (.pitch (`KismetMathLibrary.MakeRotFromX` (`MovementComponent.Velocity` (`self.ProjectileMovement`)))) -1.0) (.pitch (`self.K2_GetActorRotation`)) (.yaw (`self.K2_GetActorRotation`))))
      (if (`self.FirstSet`)
        (set `self.LastPosition` _returnvalue)
        (set `self.FirstSet` false)
        (else
          (`self.MulticastShowDebug` (`self.LastPosition`) _returnvalue)
          (set `self.LastPosition` _returnvalue))))))

(event `MulticastShowDebug`
  (params (Start :type "Vector Structure") (End :type "Vector Structure"))
  ;[1 1 0] Arrow rotation fix
  (`KismetSystemLibrary.DrawDebugLine` Start End (struct :`R` 1.0 :`A` 1.0) 6.0 6.0))

(event `MulticastArrowRotation`
  (params (Rotation :type "Rotator Structure"))
  ;[1 1 0] Arrow rotation fix
  (`self.K2_SetActorRotation` Rotation))

(event `self.ArrowCollider.OnComponentBeginOverlap`
  (params (OverlappedComponent :type "PrimitiveComponent Object Reference") (OtherActor :type "Actor Object Reference") (OtherComp :type "PrimitiveComponent Object Reference") (OtherBodyIndex :type Integer) (bFromSweep :type Boolean) (SweepResult :type "HitResult Structure (by ref)"))
  (bind (_bblockinghit _binitialoverlap _time _distance _location _impactpoint _normal _impactnormal _physmat _hitactor _hitcomponent) (`GameplayStatics.BreakHitResult` SweepResult))
  (bind (_canattach _socketname) (`/Game/Blueprints/Libraries/LibCharacter.SocketByOverlappedComponent` _hitcomponent))
  ;[1 1 0] Overlap
  (if (and (`self.DoOnce`) (`self.HasAuthority`))
    (bind _ashuman_bp (cast `/Game/Blueprints/Characters/HumanBP` _hitactor))
    (if _canattach
      (`KismetSystemLibrary.PrintString` (`KismetStringLibrary.Concat_StrStr` (`KismetSystemLibrary.GetObjectName` _hitactor) (`KismetSystemLibrary.GetObjectName` _hitcomponent)) true true (struct :`B` 1.0 :`A` 1.0) 6.0)
      (set `self.DoOnce` false)
      (`MovementComponent.StopMovementImmediately` (`self.ProjectileMovement`))
      (bind _returnvalue (`|SpawnActorFromClass` "/Game/Blueprints/Pawns/StaticArrow.StaticArrow_C" (`KismetMathLibrary.MakeTransform` _impactpoint (`self.K2_GetActorRotation`)) "AlwaysSpawn" "OverrideRootScale" null null))
      (`SceneComponent.K2_AttachToComponent` (`Actor.RootComponent` _returnvalue) _hitcomponent _socketname "KeepRelative" "KeepWorld" "KeepWorld" false)
      (`KismetSystemLibrary.PrintString` (`KismetStringLibrary.Concat_StrStr` "Actor location: " (`KismetStringLibrary.Conv_VectorToString` (`self.K2_GetActorLocation` _hitactor)) "   Arrow location:  " (`KismetStringLibrary.Conv_VectorToString` (`self.K2_GetActorLocation` _returnvalue))))
      (`/Game/Blueprints/Characters/HumanBP.ServerApplyHitEffects` _ashuman_bp _hitcomponent "NewEnumerator1")
      (`self.K2_DestroyActor`))))

(fn `OverlapSearch`
  (bind _arrowlocation (`self.ArrowLocation`))
  (bind _returnvalue (`SceneComponent.K2_GetComponentLocation` _arrowlocation))
  (bind (_outhit _returnvalue_2) (`KismetSystemLibrary.SphereTraceSingleForObjects` :`Start` _returnvalue :`End` (+ _returnvalue (* (`KismetMathLibrary.GetForwardVector` (`SceneComponent.K2_GetComponentRotation` _arrowlocation)) 200.0)) :`Radius` 200.0 :`ObjectTypes` (`|MakeArray` "ObjectTypeQuery2" :!type "EObjectTypeQuery Enum") :`bTraceComplex` true :`DrawDebugType` "ForDuration"))
  (if (and _returnvalue_2 (`self.DoOnce`))
    (bind (_bblockinghit _binitialoverlap _time _distance _location _impactpoint _normal _impactnormal _physmat _hitactor _hitcomponent) (`GameplayStatics.BreakHitResult` _outhit))
    (bind _ashuman_bp (cast `/Game/Blueprints/Characters/HumanBP` _hitactor))
    (bind (_canattach _socketname) (`/Game/Blueprints/Libraries/LibCharacter.SocketByOverlappedComponent` _hitcomponent))
    (if _canattach
      (`KismetSystemLibrary.PrintString` (`KismetStringLibrary.Concat_StrStr` (`KismetSystemLibrary.GetObjectName` _hitactor) (`KismetSystemLibrary.GetObjectName` _hitcomponent)) true true (struct :`B` 1.0 :`A` 1.0) 6.0)
      (set `self.DoOnce` false)
      (`MovementComponent.StopMovementImmediately` (`self.ProjectileMovement`))
      (bind _returnvalue_3 (`|SpawnActorFromClass` "/Game/Blueprints/Pawns/StaticArrow.StaticArrow_C" (`KismetMathLibrary.MakeTransform` _impactpoint (`self.K2_GetActorRotation`)) "AlwaysSpawn" "OverrideRootScale" null null))
      (`SceneComponent.K2_AttachToComponent` (`Actor.RootComponent` _returnvalue_3) _hitcomponent _socketname "KeepRelative" "KeepWorld" "KeepWorld" false)
      (`KismetSystemLibrary.PrintString` (`KismetStringLibrary.Concat_StrStr` "Actor location: " (`KismetStringLibrary.Conv_VectorToString` (`self.K2_GetActorLocation` _hitactor)) "   Arrow location:  " (`KismetStringLibrary.Conv_VectorToString` (`self.K2_GetActorLocation` _returnvalue_3))))
      (`/Game/Blueprints/Characters/HumanBP.ServerApplyHitEffects` _ashuman_bp _hitcomponent "NewEnumerator1")
      (`self.K2_DestroyActor`))))

(fn `UserConstructionScript`
  (set `ProjectileMovementComponent.InitialSpeed` (`self.ArrowSpeed`) (`self.ProjectileMovement`))
  (`SceneComponent.K2_SetWorldRotation` (`self.ArrowMesh`) (`self.ArrowRotation`) false false)
  (set `MovementComponent.Velocity` (`self.ArrowVelocity`) (`self.ProjectileMovement`))
  (set `self.StartLocation` (`SceneComponent.K2_GetComponentLocation` (`self.ArrowLocation`))))