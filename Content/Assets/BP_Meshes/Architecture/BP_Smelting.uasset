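; BP_Smelting is a smelting building that consumes three item types and produces two others on a timed production period.
; It is a data-only child of a parent building Blueprint, with its construction script setting item indices, a single-worker limit, ownership, and placement sizing after calling the parent.
; It adds no logic of its own, as BeginPlay only forwards to the parent.
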(event `self.ReceiveBeginPlay`
  (`parent.ReceiveBeginPlay`))

(fn `UserConstructionScript`
  (`parent.UserConstructionScript`)
  (set `self.MaxWorker` 1)
  (set `self.IsProductive` true)
  (set `self.Production1ItemIndex` 30)
  (set `self.IsProducing2` true)
  (set `self.Production2ItemIndex` 31)
  (set `self.ProductionPeriod` (+ (`self.DefaultTime`) (`KismetMathLibrary.MakeTimespan` 0 3)))
  (set `self.IsConsumer` true)
  (set `self.Consume1ItemIndex` 19)
  (set `self.IsConsume2` true)
  (set `self.Consume2ItemIndex` 21)
  (set `self.IsConsume3` true)
  (set `self.Consume3ItemIndex` 22)
  (set `self.InnerBorderRadius` 2500.0)
  (set `self.MeshSize` 100.0)
  (set `self.CanBuildScale` (15.5 12.25 28.0))
  (set `self.HasOwner` true))