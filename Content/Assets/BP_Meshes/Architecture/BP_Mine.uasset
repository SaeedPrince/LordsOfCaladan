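; BP_Mine is a productive architecture building that represents a mine, with its product and name derived from a production index.
; The construction script extends the parent's setup by setting worker limit, production period, border radius and mesh size, then assigns the production item and looks up the mine name from it.
; ClientShowFlag swaps the flag's skeletal mesh to the one matching that production item.
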(event `self.ReceiveBeginPlay`
  ;[1 1 0] Begin Play
  (`parent.ReceiveBeginPlay`))

(event `ClientShowFlag`
  ;[1 1 0] Mine flag
  (`SkinnedMeshComponent.SetSkinnedAssetAndUpdate` (`self.FlagPic`) (`/Game/Blueprints/Libraries/LibGame.FlagMesh` (`self.Production1ItemIndex`)) true))

(fn `UserConstructionScript`
  (`parent.UserConstructionScript`)
  (set `self.IsProductive` true)
  (set `self.MaxWorker` 2)
  (set `self.ProductionPeriod` (+ (`self.DefaultTime`) (`KismetMathLibrary.MakeTimespan` 0 3)))
  (set `self.InnerBorderRadius` 2500.0)
  (set `self.MeshSize` 100.0)
  (bind _output_get (set `self.Production1ItemIndex` (`self.ProductionIndex`)))
  (set `self.Name` (`/Game/Blueprints/Libraries/LibMine.MineName` _output_get)))