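; BP_PowderShop is a powder shop building that configures itself as an owned production structure for a single worker.
; Its construction script calls the parent, then sets the production period, two output items and three consumed items, along with border radius, mesh size and build scale.
; The Blueprint only supplies data; BeginPlay just forwards to the parent, and no production logic appears here.
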(event `self.ReceiveBeginPlay`
  (`parent.ReceiveBeginPlay`))

(fn `UserConstructionScript`
  (`parent.UserConstructionScript`)
  (set `self.IsProductive` true)
  (set `self.MaxWorker` 1)
  (set `self.ProductionPeriod` (+ (`self.DefaultTime`) (`KismetMathLibrary.MakeTimespan` 0 4)))
  (set `self.Production1ItemID` "NewEnumerator22")
  (set `self.IsProducing2` true)
  (set `self.Production2ItemID` "NewEnumerator17")
  (set `self.IsConsumer` true)
  (set `self.Consume1ItemID` "NewEnumerator21")
  (set `self.IsConsume2` true)
  (set `self.Consume2ItemID` "NewEnumerator28")
  (set `self.IsConsume3` true)
  (set `self.Consume3ItemID` "NewEnumerator20")
  (set `self.InnerBorderRadius` 2500.0)
  (set `self.MeshSize` 100.0)
  (set `self.CanBuildScale` (15.5 12.25 28.0))
  (set `self.HasOwner` true))