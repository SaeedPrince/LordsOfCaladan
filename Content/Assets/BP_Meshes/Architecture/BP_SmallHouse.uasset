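; BP_SmallHouse is a small residential building Blueprint with an owner that is flagged as a person generator.
; Its construction script runs the parent's, then overrides inherited settings for border radius, mesh size, buildable scale, resident capacity and generation count.
; BeginPlay only calls the parent, so the asset is a data-only specialisation with all behaviour left to its parent class.
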(event `self.ReceiveBeginPlay`
  (`parent.ReceiveBeginPlay`))

(fn `UserConstructionScript`
  (`parent.UserConstructionScript`)
  (set `self.InnerBorderRadius` 2500.0)
  (set `self.MeshSize` 100.0)
  (set `self.CanBuildScale` (15.5 12.25 28.0))
  (set `self.HasOwner` true)
  (set `self.IsPersonGenerator` true)
  (set `self.MaxResident` 6)
  (set `self.GenerationCount` 1)
  (set `self.IsResident` true))