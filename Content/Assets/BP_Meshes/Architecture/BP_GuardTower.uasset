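; Guard tower building Blueprint that acts as an owned border maker and houses military residents.
; Its construction script calls the parent, then sets inherited-style configuration for inner and outer border extents, mesh size, build-check scale, population caps, and ladder and flag counts.
; BeginPlay only forwards to the parent, so the file holds configuration and no behavior of its own.
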(event `self.ReceiveBeginPlay`
  (`parent.ReceiveBeginPlay`))

(fn `UserConstructionScript`
  (`parent.UserConstructionScript`)
  (set `self.IsBorderMaker` true)
  (set `self.InnerBorderRadius` 3500.0)
  (set `self.OuterBorderSide` 12500.0)
  (set `self.MeshSize` 200.0)
  (set `self.CanBuildScale` (30.0 25.0 55.0))
  (set `self.HasOwner` true)
  (set `self.MaxMilitPop` 12)
  (set `self.MaxResident` 12)
  (set `self.IsResident` true)
  (set `self.LadderCount` 3)
  (set `self.FlagCount` 3))