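; BP_Sawmill is the sawmill building, a productive structure that consumes one item type and produces another on a timed period.
; It only configures inherited properties in its Construction Script, after the parent's: worker cap, production timing, item indices, ownership, border radius and build-check dimensions.
; It adds no logic of its own, as BeginPlay just calls the parent, leaving behavior to the base class.
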(event `self.ReceiveBeginPlay`
  (`parent.ReceiveBeginPlay`))

(fn `UserConstructionScript`
  (`parent.UserConstructionScript`)
  (set `self.IsProductive` true)
  (set `self.MaxWorker` 1)
  (set `self.ProductionPeriod` (+ (`self.DefaultTime`) (`KismetMathLibrary.MakeTimespan` 0 2)))
  (set `self.Production1ItemIndex` 2)
  (set `self.IsConsumer` true)
  (set `self.Consume1ItemIndex` 0)
  (set `self.InnerBorderRadius` 2500.0)
  (set `self.MeshSize` 100.0)
  (set `self.CanBuildScale` (15.5 12.25 28.0))
  (set `self.HasOwner` true))