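; BP_SheepFarm is a sheep farm building that serves as an owned, productive structure with a worker slot and two produced items.
; It is a data-only style child: the construction script calls the parent, then overrides production timing, item indices, border radius, mesh size and build-check scale.
; BeginPlay only calls the parent, so the production and placement behavior itself is not defined here.
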(event `self.ReceiveBeginPlay`
  (`parent.ReceiveBeginPlay`))

(fn `UserConstructionScript`
  (`parent.UserConstructionScript`)
  (set `self.IsProductive` true)
  (set `self.MaxWorker` 1)
  (set `self.ProductionPeriod` (+ (`self.DefaultTime`) (`KismetMathLibrary.MakeTimespan` 0 4)))
  (set `self.Production1ItemIndex` 29)
  (set `self.IsProducing2` true)
  (set `self.Production2ItemIndex` 9)
  (set `self.InnerBorderRadius` 2500.0)
  (set `self.MeshSize` 100.0)
  (set `self.CanBuildScale` (15.5 12.25 20.0))
  (set `self.HasOwner` true))