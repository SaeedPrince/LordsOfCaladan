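; Fortress building Blueprint, a border-making, owned structure that houses civilian and military population.
; The construction script runs the parent's, then overrides its settings for stacking, population generation and limits, border radius and side, mesh size and flags.
; On BeginPlay it sets the house mesh collision type and scale, hides the build indicator and border pieces, and starts server activity on authority only.
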(event `self.ReceiveBeginPlay`
  (`PrimitiveComponent.SetCollisionObjectType` (`self.HouseMesh`) (`self.CollisionType`))
  (`SceneComponent.SetWorldScale3D` (`self.HouseMesh`) (`self.FortressMeshScale`))
  (`SceneComponent.SetVisibility` (`self.CanBuild`) false false)
  (for _array_element (`self.Borders`)
    (`/Engine/EditorBlueprintResources/StandardMacros.IsValid` _array_element
      (:`Is Valid`
        (`SceneComponent.SetVisibility` _array_element false false))))
  (`/Engine/EditorBlueprintResources/ActorMacros.Switch Has Authority`
    (:`Authority`
      (`self.ServerStartActivity`))))

(fn `UserConstructionScript`
  (`parent.UserConstructionScript`)
  (set `self.IsStack` true)
  (set `self.MaxItemCount` 32)
  (set `self.CivilGenerationCount` 8)
  (set `self.MilitGenerationCount` 8)
  (set `self.MaxResident` 26)
  (set `self.MaxMilitPop` 26)
  (set `self.IsBorderMaker` true)
  (set `self.InnerBorderRadius` 12200.0)
  (set `self.MeshSize` 1220.0)
  (set `self.OuterBorderSide` (`self.FortressOuterBorderSide`))
  (set `self.IsResident` true)
  (set `self.HasOwner` true)
  (set `self.FlagCount` 5))