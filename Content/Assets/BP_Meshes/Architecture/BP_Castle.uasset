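; BP_Castle is a child building Blueprint that configures the castle, an owned residence that also acts as a border maker.
; Its construction script runs the parent's, then overrides inherited settings for border extents, mesh and build-check scale, military and resident capacity, ladder and flag counts, and a gate.
; BeginPlay only forwards to the parent, so the file itself holds configuration with no behavior of its own.
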(event `self.ReceiveBeginPlay`
  (`parent.ReceiveBeginPlay`))

(fn `UserConstructionScript`
  (`parent.UserConstructionScript`)
  (set `self.IsBorderMaker` true)
  (set `self.InnerBorderRadius` 4000.0)
  (set `self.OuterBorderSide` 20000.0)
  (set `self.MeshSize` 450.0)
  (set `self.CanBuildScale` (48.0 58.0 58.0))
  (set `self.HasOwner` true)
  (set `self.MaxMilitPop` 24)
  (set `self.MaxResident` 24)
  (set `self.IsResident` true)
  (set `self.LadderCount` 14)
  (set `self.FlagCount` 5)
  (set `self.HasGate` true))