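; BP_WoodCuttersHut is a woodcutter's hut building Blueprint, set up as an owned, productive structure.
; Its construction script runs the parent's, then sets worker capacity, an hours-long production period, the produced item index, and sizing values for inner border, mesh and build check.
; BeginPlay only calls the parent, so the file itself holds configuration and no behavior of its own.
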(event `self.ReceiveBeginPlay`
  (`parent.ReceiveBeginPlay`))

(fn `UserConstructionScript`
  (`parent.UserConstructionScript`)
  (set `self.IsProductive` true)
  (set `self.MaxWorker` 2)
  (set `self.ProductionPeriod` (+ (`self.DefaultTime`) (`KismetMathLibrary.MakeTimespan` 0 3)))
  (set `self.Production1ItemIndex` 0)
  (set `self.InnerBorderRadius` 2500.0)
  (set `self.MeshSize` 100.0)
  (set `self.CanBuildScale` (15.5 12.25 20.0))
  (set `self.HasOwner` true))